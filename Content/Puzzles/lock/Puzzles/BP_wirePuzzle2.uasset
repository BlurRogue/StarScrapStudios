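; Wire puzzle actor where the player spins sixteen tagged pieces into alignment.
; UseOpenClose line-traces from the player camera and eases the hit piece a quarter turn in yaw, debounced by DoOnce and Delay.
; A self-rescheduling timer polls six key pieces' yaw; when all match, it plays a success sound, calls AllcoditionsMeet and optionally grants a key ID.
; It also has a custom-depth highlight toggle, while its overlap and Interact events are empty.
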(event OnComponentBeginOverlap(InteractTrigger)
  (params (OverlappedComponent :type Primitive%20Component%20Object%20Reference) (OtherActor :type Actor%20Object%20Reference) (OtherComp :type Primitive%20Component%20Object%20Reference) (OtherBodyIndex :type Integer) (bFromSweep :type Boolean) (SweepResult :type Hit%20Result%20Structure%20%28by%20ref%29))
  ;[1 0.8403 0.1586] User Interface for RE Interaction Wheel
)

(event OnComponentEndOverlap(InteractTrigger)
  (params (OverlappedComponent :type Primitive%20Component%20Object%20Reference) (OtherActor :type Actor%20Object%20Reference) (OtherComp :type Primitive%20Component%20Object%20Reference) (OtherBodyIndex :type Integer))
  ;[1 0.8403 0.1586] User Interface for RE Interaction Wheel
)

(event Custom|GetRotationValues
  ;[1 1 1] Check Rotation Value
  (Utilities|Time|SetTimerbyEvent (delegate Custom|GetRotationValues) 2.0)
  (if (Math|Boolean|ANDBoolean (Math|Float|NearlyEqual(Float) (.yaw (Transformation|GetWorldRotation (Variables|Default|GetBOT))) 9e+01 0.5) (Math|Float|NearlyEqual(Float) (.yaw (Transformation|GetWorldRotation (Variables|Default|GetM))) 9e+01 0.5) (Math|Float|NearlyEqual(Float) (.yaw (Transformation|GetWorldRotation (Variables|Default|GetK))) 9e+01 0.5) (Math|Float|NearlyEqual(Float) (.yaw (Transformation|GetWorldRotation (Variables|Default|GetJ))) 9e+01 0.5) (Math|Float|NearlyEqual(Float) (.yaw (Transformation|GetWorldRotation (Variables|Default|GetB))) 9e+01 0.5) (Math|Float|NearlyEqual(Float) (.yaw (Transformation|GetWorldRotation (Variables|Default|GetTOP))) 9e+01 0.5))
    (Development|PrintString "Hello")
    (Utilities|FlowControl|DoOnce false
      (:Completed
        (Audio|PlaySoundatLocation "/Game/Sound/SoundWaves/Puzzle_Success.Puzzle_Success" "0, 0, 0" "0, 0, 0" 1.0 1.0 0.0 0 0 0 0)
        (Default|CallAllcoditionsmeet)
        (CallFunction|CheckforKey)
        (Development|PrintString "Puzzle Success!!!!")))))

(event Custom|CustomEvent
  (params (toggleEnum :type E_toggle%20Enum :default "NewEnumerator0"))
  ;[1 0.8392 0.4018] Toggle Highlight
  (if (Variables|Default|GetisInteractable)
    (switch Utilities|FlowControl|Switch|SwitchonE_toggle toggleEnum
      (:NewEnumerator0
        (if (not (Variables|Default|GethighlightActive))
          ;;[0.07443 0.15 0.07585 0.5] Turning on Highlight
          (Rendering|SetRenderCustomDepth (Variables|Default|GetStatic_Mesh) true :!label _label)
          (Variables|Default|SethighlightActive true)))
      (:NewEnumerator1
        (goto _label))
      (:NewEnumerator2
        ;;[0.15 0.06655 0.06804 0.5] Turning Off Highlight
        (Rendering|SetRenderCustomDepth (Variables|Default|GetStatic_Mesh) false)
        (Variables|Default|SethighlightActive false)))))

(event Custom|checkForKey
  (if (Variables|Default|GetisKey)
    (Default|AddKeyID (Variables|Default|GetAs%20BP%20First%20Person%20Character) (Variables|Default|GetkeyID))))

(event EventBeginPlay
  (bind _asbp_first_person_character (Utilities|Casting|CastToBP_FirstPersonCharacter (Game|GetPlayerCharacter 0)))
  (Variables|Default|SetCharacterReference _asbp_first_person_character)
  (CallFunction|GetRotationValues))

(event EventUseOpenClose
  (bind _d (Variables|Default|GetD))
  (bind _e (Variables|Default|GetE))
  (bind _g (Variables|Default|GetG))
  (bind _h (Variables|Default|GetH))
  (bind _characterreference (Variables|Default|GetCharacterReference))
  (bind _bot (Variables|Default|GetBOT))
  (bind _mid (Variables|Default|GetMID))
  (bind _top (Variables|Default|GetTOP))
  (bind _i (Variables|Default|GetI))
  (bind _j (Variables|Default|GetJ))
  (bind _k (Variables|Default|GetK))
  (bind _b (Variables|Default|GetB))
  (bind _a (Variables|Default|GetA))
  (bind _c (Variables|Default|GetC))
  (bind _l (Variables|Default|GetL))
  (bind _m (Variables|Default|GetM))
  (bind _f (Variables|Default|GetF))
  (bind _firstpersoncamera (Variables|/Game/FirstPerson/Blueprints/BP_FirstPersonCharacter.BP_FirstPersonCharacter_C|GetFirstPersonCamera _characterreference))
  (bind _returnvalue (Transformation|GetWorldLocation _firstpersoncamera))
  (bind (_outhit _returnvalue_2) (Collision|LineTraceByChannel _returnvalue (+ _returnvalue (* (Math|Vector|GetForwardVector _firstpersoncamera) 2e+02)) "TraceTypeQuery1" false 0 "None" false))
  (if _returnvalue_2
    (if (Components|ComponentHasTag (.HitComponent (Collision|BreakHitResult _outhit)) "TOP")
      ;[1 1 1] Top
      (Utilities|FlowControl|DoOnce false :!label _label
        (:Completed
          (Audio|PlaySoundatLocation "/Game/Sound/SoundWaves/Wire_Spin.Wire_Spin" "0, 0, 0" "0, 0, 0" 1.0 1.0 0.0 0 0 0 0)
          (Components|MoveComponentTo (Variables|Default|GetTOP) (Variables|/Script/Engine.SceneComponent|GetRelativeLocation _top) (Math|Rotator|MakeRotator 0.0 0.0 (.yaw (Math|Rotator|MakeRotator 0.0 0.0 (+ (.yaw (Transformation|GetWorldRotation _top)) 9e+01)))) true true 0.5 false)
          (Utilities|FlowControl|Delay 0.2)
          (goto _label Reset)))
      (elif (Components|ComponentHasTag (.HitComponent (Collision|BreakHitResult _outhit)) "MID")
        ;[1 1 1] middle
        (Utilities|FlowControl|DoOnce false :!label _label_2
          (:Completed
            (Audio|PlaySoundatLocation "/Game/Sound/SoundWaves/Wire_Spin.Wire_Spin" "0, 0, 0" "0, 0, 0" 1.0 1.0 0.0 0 0 0 0)
            (Components|MoveComponentTo (Variables|Default|GetMID) (Variables|/Script/Engine.SceneComponent|GetRelativeLocation _mid) (Math|Rotator|MakeRotator 0.0 0.0 (.yaw (Math|Rotator|MakeRotator 0.0 0.0 (+ (.yaw (Transformation|GetWorldRotation _mid)) 9e+01)))) true true 0.5 false)
            (Utilities|FlowControl|Delay 0.2)
            (goto _label_2 Reset)))
        (elif (Components|ComponentHasTag (.HitComponent (Collision|BreakHitResult _outhit)) "BOT")
          ;[1 1 1] Bot
          (Utilities|FlowControl|DoOnce false :!label _label_3
            (:Completed
              (Audio|PlaySoundatLocation "/Game/Sound/SoundWaves/Wire_Spin.Wire_Spin" "0, 0, 0" "0, 0, 0" 1.0 1.0 0.0 0 0 0 0)
              (Components|MoveComponentTo (Variables|Default|GetBOT) (Variables|/Script/Engine.SceneComponent|GetRelativeLocation _bot) (Math|Rotator|MakeRotator 0.0 0.0 (.yaw (Math|Rotator|MakeRotator 0.0 0.0 (+ (.yaw (Transformation|GetWorldRotation _bot)) 9e+01)))) true true 0.5 false)
              (Utilities|FlowControl|Delay 0.2)
              (goto _label_3 Reset)))
          (elif (Components|ComponentHasTag (.HitComponent (Collision|BreakHitResult _outhit)) "A")
            (Utilities|FlowControl|DoOnce false :!label _label_4
              (:Completed
                (Audio|PlaySoundatLocation "/Game/Sound/SoundWaves/Wire_Spin.Wire_Spin" "0, 0, 0" "0, 0, 0" 1.0 1.0 0.0 0 0 0 0)
                (Components|MoveComponentTo (Variables|Default|GetA) (Variables|/Script/Engine.SceneComponent|GetRelativeLocation _a) (Math|Rotator|MakeRotator 0.0 0.0 (.yaw (Math|Rotator|MakeRotator 0.0 0.0 (+ (.yaw (Transformation|GetWorldRotation _a)) 9e+01)))) true true 0.5 false)
                (Utilities|FlowControl|Delay 0.2)
                (goto _label_4 Reset)))
            (elif (Components|ComponentHasTag (.HitComponent (Collision|BreakHitResult _outhit)) "B")
              ;[1 1 1] middle
              (Utilities|FlowControl|DoOnce false :!label _label_5
                (:Completed
                  (Audio|PlaySoundatLocation "/Game/Sound/SoundWaves/Wire_Spin.Wire_Spin" "0, 0, 0" "0, 0, 0" 1.0 1.0 0.0 0 0 0 0)
                  (Components|MoveComponentTo (Variables|Default|GetB) (Variables|/Script/Engine.SceneComponent|GetRelativeLocation _b) (Math|Rotator|MakeRotator 0.0 0.0 (.yaw (Math|Rotator|MakeRotator 0.0 0.0 (+ (.yaw (Transformation|GetWorldRotation _b)) 9e+01)))) true true 0.5 false)
                  (Utilities|FlowControl|Delay 0.2)
                  (goto _label_5 Reset)))
              (elif (Components|ComponentHasTag (.HitComponent (Collision|BreakHitResult _outhit)) "C")
                ;[1 1 1] Bot
                (Utilities|FlowControl|DoOnce false :!label _label_6
                  (:Completed
                    (Audio|PlaySoundatLocation "/Game/Sound/SoundWaves/Wire_Spin.Wire_Spin" "0, 0, 0" "0, 0, 0" 1.0 1.0 0.0 0 0 0 0)
                    (Components|MoveComponentTo (Variables|Default|GetC) (Variables|/Script/Engine.SceneComponent|GetRelativeLocation _c) (Math|Rotator|MakeRotator 0.0 0.0 (.yaw (Math|Rotator|MakeRotator 0.0 0.0 (+ (.yaw (Transformation|GetWorldRotation _c)) 9e+01)))) true true 0.5 false)
                    (Utilities|FlowControl|Delay 0.2)
                    (goto _label_6 Reset)))
                (elif (Components|ComponentHasTag (.HitComponent (Collision|BreakHitResult _outhit)) "D")
                  (Utilities|FlowControl|DoOnce false :!label _label_7
                    (:Completed
                      (Audio|PlaySoundatLocation "/Game/Sound/SoundWaves/Wire_Spin.Wire_Spin" "0, 0, 0" "0, 0, 0" 1.0 1.0 0.0 0 0 0 0)
                      (Components|MoveComponentTo (Variables|Default|GetD) (Variables|/Script/Engine.SceneComponent|GetRelativeLocation _d) (Math|Rotator|MakeRotator 0.0 0.0 (.yaw (Math|Rotator|MakeRotator 0.0 0.0 (+ (.yaw (Transformation|GetWorldRotation _d)) 9e+01)))) true true 0.5 false)
                      (Utilities|FlowControl|Delay 0.2)
                      (goto _label_7 Reset)))
                  (elif (Components|ComponentHasTag (.HitComponent (Collision|BreakHitResult _outhit)) "E")
                    ;[1 1 1] middle
                    (Utilities|FlowControl|DoOnce false :!label _label_8
                      (:Completed
                        (Audio|PlaySoundatLocation "/Game/Sound/SoundWaves/Wire_Spin.Wire_Spin" "0, 0, 0" "0, 0, 0" 1.0 1.0 0.0 0 0 0 0)
                        (Components|MoveComponentTo (Variables|Default|GetE) (Variables|/Script/Engine.SceneComponent|GetRelativeLocation _e) (Math|Rotator|MakeRotator 0.0 0.0 (.yaw (Math|Rotator|MakeRotator 0.0 0.0 (+ (.yaw (Transformation|GetWorldRotation _e)) 9e+01)))) true true 0.5 false)
                        (Utilities|FlowControl|Delay 0.2)
                        (goto _label_8 Reset)))
                    (elif (Components|ComponentHasTag (.HitComponent (Collision|BreakHitResult _outhit)) "F")
                      ;[1 1 1] Bot
                      (Utilities|FlowControl|DoOnce false :!label _label_9
                        (:Completed
                          (Audio|PlaySoundatLocation "/Game/Sound/SoundWaves/Wire_Spin.Wire_Spin" "0, 0, 0" "0, 0, 0" 1.0 1.0 0.0 0 0 0 0)
                          (Components|MoveComponentTo (Variables|Default|GetF) (Variables|/Script/Engine.SceneComponent|GetRelativeLocation _f) (Math|Rotator|MakeRotator 0.0 0.0 (.yaw (Math|Rotator|MakeRotator 0.0 0.0 (+ (.yaw (Transformation|GetWorldRotation _f)) 9e+01)))) true true 0.5 false)
                          (Utilities|FlowControl|Delay 0.2)
                          (goto _label_9 Reset)))
                      (elif (Components|ComponentHasTag (.HitComponent (Collision|BreakHitResult _outhit)) "G")
                        (Utilities|FlowControl|DoOnce false :!label _label_10
                          (:Completed
                            (Audio|PlaySoundatLocation "/Game/Sound/SoundWaves/Wire_Spin.Wire_Spin" "0, 0, 0" "0, 0, 0" 1.0 1.0 0.0 0 0 0 0)
                            (Components|MoveComponentTo (Variables|Default|GetG) (Variables|/Script/Engine.SceneComponent|GetRelativeLocation _g) (Math|Rotator|MakeRotator 0.0 0.0 (.yaw (Math|Rotator|MakeRotator 0.0 0.0 (+ (.yaw (Transformation|GetWorldRotation _g)) 9e+01)))) true true 0.5 false)
                            (Utilities|FlowControl|Delay 0.2)
                            (goto _label_10 Reset)))
                        (elif (Components|ComponentHasTag (.HitComponent (Collision|BreakHitResult _outhit)) "H")
                          ;[1 1 1] middle
                          (Utilities|FlowControl|DoOnce false :!label _label_11
                            (:Completed
                              (Audio|PlaySoundatLocation "/Game/Sound/SoundWaves/Wire_Spin.Wire_Spin" "0, 0, 0" "0, 0, 0" 1.0 1.0 0.0 0 0 0 0)
                              (Components|MoveComponentTo (Variables|Default|GetH) (Variables|/Script/Engine.SceneComponent|GetRelativeLocation _h) (Math|Rotator|MakeRotator 0.0 0.0 (.yaw (Math|Rotator|MakeRotator 0.0 0.0 (+ (.yaw (Transformation|GetWorldRotation _h)) 9e+01)))) true true 0.5 false)
                              (Utilities|FlowControl|Delay 0.2)
                              (goto _label_11 Reset)))
                          (elif (Components|ComponentHasTag (.HitComponent (Collision|BreakHitResult _outhit)) "I")
                            ;[1 1 1] Bot
                            (Utilities|FlowControl|DoOnce false :!label _label_12
                              (:Completed
                                (Audio|PlaySoundatLocation "/Game/Sound/SoundWaves/Wire_Spin.Wire_Spin" "0, 0, 0" "0, 0, 0" 1.0 1.0 0.0 0 0 0 0)
                                (Components|MoveComponentTo (Variables|Default|GetI) (Variables|/Script/Engine.SceneComponent|GetRelativeLocation _i) (Math|Rotator|MakeRotator 0.0 0.0 (.yaw (Math|Rotator|MakeRotator 0.0 0.0 (+ (.yaw (Transformation|GetWorldRotation _i)) 9e+01)))) true true 0.5 false)
                                (Utilities|FlowControl|Delay 0.2)
                                (goto _label_12 Reset)))
                            (elif (Components|ComponentHasTag (.HitComponent (Collision|BreakHitResult _outhit)) "J")
                              (Utilities|FlowControl|DoOnce false :!label _label_13
                                (:Completed
                                  (Audio|PlaySoundatLocation "/Game/Sound/SoundWaves/Wire_Spin.Wire_Spin" "0, 0, 0" "0, 0, 0" 1.0 1.0 0.0 0 0 0 0)
                                  (Components|MoveComponentTo (Variables|Default|GetJ) (Variables|/Script/Engine.SceneComponent|GetRelativeLocation _j) (Math|Rotator|MakeRotator 0.0 0.0 (.yaw (Math|Rotator|MakeRotator 0.0 0.0 (+ (.yaw (Transformation|GetWorldRotation _j)) 9e+01)))) true true 0.5 false)
                                  (Utilities|FlowControl|Delay 0.2)
                                  (goto _label_13 Reset)))
                              (elif (Components|ComponentHasTag (.HitComponent (Collision|BreakHitResult _outhit)) "K")
                                ;[1 1 1] middle
                                (Utilities|FlowControl|DoOnce false :!label _label_14
                                  (:Completed
                                    (Audio|PlaySoundatLocation "/Game/Sound/SoundWaves/Wire_Spin.Wire_Spin" "0, 0, 0" "0, 0, 0" 1.0 1.0 0.0 0 0 0 0)
                                    (Components|MoveComponentTo (Variables|Default|GetK) (Variables|/Script/Engine.SceneComponent|GetRelativeLocation _k) (Math|Rotator|MakeRotator 0.0 0.0 (.yaw (Math|Rotator|MakeRotator 0.0 0.0 (+ (.yaw (Transformation|GetWorldRotation _k)) 9e+01)))) true true 0.5 false)
                                    (Utilities|FlowControl|Delay 0.2)
                                    (goto _label_14 Reset)))
                                (elif (Components|ComponentHasTag (.HitComponent (Collision|BreakHitResult _outhit)) "L")
                                  ;[1 1 1] Bot
                                  (Utilities|FlowControl|DoOnce false :!label _label_15
                                    (:Completed
                                      (Audio|PlaySoundatLocation "/Game/Sound/SoundWaves/Wire_Spin.Wire_Spin" "0, 0, 0" "0, 0, 0" 1.0 1.0 0.0 0 0 0 0)
                                      (Components|MoveComponentTo (Variables|Default|GetL) (Variables|/Script/Engine.SceneComponent|GetRelativeLocation _l) (Math|Rotator|MakeRotator 0.0 0.0 (.yaw (Math|Rotator|MakeRotator 0.0 0.0 (+ (.yaw (Transformation|GetWorldRotation _l)) 9e+01)))) true true 0.5 false)
                                      (Utilities|FlowControl|Delay 0.2)
                                      (goto _label_15 Reset)))
                                  (elif (Components|ComponentHasTag (.HitComponent (Collision|BreakHitResult _outhit)) "M")
                                    ;[1 1 1] Bot
                                    (Utilities|FlowControl|DoOnce false :!label _label_16
                                      (:Completed
                                        (Audio|PlaySoundatLocation "/Game/Sound/SoundWaves/Wire_Spin.Wire_Spin" "0, 0, 0" "0, 0, 0" 1.0 1.0 0.0 0 0 0 0)
                                        (Components|MoveComponentTo (Variables|Default|GetM) (Variables|/Script/Engine.SceneComponent|GetRelativeLocation _m) (Math|Rotator|MakeRotator 0.0 0.0 (.yaw (Math|Rotator|MakeRotator 0.0 0.0 (+ (.yaw (Transformation|GetWorldRotation _m)) 9e+01)))) true true 0.5 false)
                                        (Utilities|FlowControl|Delay 0.2)
                                        (goto _label_16 Reset)))))))))))))))))))))

(event EventInteract
  (params (Component :type Actor%20Component%20Object%20Reference)))

(fn ConstructionScript)

(fn Inspection
  (return 0))