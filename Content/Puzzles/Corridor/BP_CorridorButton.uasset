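; BP_CorridorButton is an interactable button that runs a one-time, timed door sequence for the corridor puzzle.
; InteractITEM passes through a DoOnce, adds the CorridorPuzzle widget to the viewport, then drives the Door reference through a chain of Delays.
; The front doors open in turn, then both back doors open, and finally two close calls fire, with 2D sounds marking reset, tension and completion.
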(event EventBeginPlay)

(event Collision|EventActorBeginOverlap
  (params (OtherActor :type Actor%20Object%20Reference)))

(event EventTick
  (params (DeltaSeconds :type Float%20%28single-precision%29)))

(event EventInteractITEM
  (Utilities|FlowControl|DoOnce false
    (:Completed
      (bind _returnvalue (UserInterface|CreateWidget "/Game/UI/CorridorPuzzle.CorridorPuzzle_C" (Game|GetPlayerController 0)))
      (UserInterface|Viewport|AddtoViewport _returnvalue 0)
      (Audio|PlaySound2D "/Game/Puzzles/Corridor/sOUND/reset.reset" 1.0 1.0 0.0 0 0)
      (Utilities|FlowControl|Delay 1.0)
      (Default|OpenLeftFDoor (Variables|Default|GetDoor))
      (Audio|PlaySound2D "/Game/Puzzles/Corridor/sOUND/TensionBGM.TensionBGM" 1.0 1.0 0.0 0 0)
      (Utilities|FlowControl|Delay 5.0)
      (Default|OpenRightFDoor (Variables|Default|GetDoor))
      (Utilities|FlowControl|Delay 4.0)
      (Default|OpenLeftBDoor (Variables|Default|GetDoor))
      (Default|OpenRightBDoor (Variables|Default|GetDoor))
      (Audio|PlaySound2D "/Game/Puzzles/Corridor/sOUND/COMPLETESYSTEM.COMPLETESYSTEM" 1.0 1.0 0.0 0 0)
      (Utilities|FlowControl|Delay 3.0)
      (Default|CloseDoor (Variables|Default|GetDoor))
      (Default|CloseDoor1 (Variables|Default|GetDoor)))))

(fn ConstructionScript)

(fn Inspection
  (return 0))