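; Overlap-driven button puzzle for the final puzzle area that opens a glass door when the correct four of eight trigger boxes have been touched.
; Each correct box sets its own flag and checks all four, so order does not matter; the other four boxes clear every flag.
; Every overlap beeps, and completion plays a success sound and calls Opentheglass on GlassDoor through OPG, with debug prints throughout.
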(event OnComponentBeginOverlap(Box2)
  (params (OverlappedComponent :type Primitive%20Component%20Object%20Reference) (OtherActor :type Actor%20Object%20Reference) (OtherComp :type Primitive%20Component%20Object%20Reference) (OtherBodyIndex :type Integer) (bFromSweep :type Boolean) (SweepResult :type Hit%20Result%20Structure%20%28by%20ref%29))
  (CallFunction|ResetButton)
  (Audio|PlaySound2D "/Game/Assets/Audio/Interaction/43400302_beep-short-16.43400302_beep-short-16" 1.0 1.0 0.0 0 0))

(event OnComponentBeginOverlap(Box6)
  (params (OverlappedComponent :type Primitive%20Component%20Object%20Reference) (OtherActor :type Actor%20Object%20Reference) (OtherComp :type Primitive%20Component%20Object%20Reference) (OtherBodyIndex :type Integer) (bFromSweep :type Boolean) (SweepResult :type Hit%20Result%20Structure%20%28by%20ref%29))
  (Variables|Default|SetActive5 true)
  (Audio|PlaySound2D "/Game/Assets/Audio/Interaction/43400302_beep-short-16.43400302_beep-short-16" 1.0 1.0 0.0 0 0)
  (Development|PrintString "Hello")
  (if (Math|Boolean|ANDBoolean (Variables|Default|GetActive5) (Variables|Default|GetActive1) (Variables|Default|GetActive7) (Variables|Default|GetActive2))
    (Development|PrintString "1111111")
    (Audio|PlaySound2D "/Game/Sound/SoundWaves/Puzzle_Success.Puzzle_Success" 1.0 1.0 0.0 0 0)
    (CallFunction|OPG)))

(event OnComponentBeginOverlap(Box3)
  (params (OverlappedComponent :type Primitive%20Component%20Object%20Reference) (OtherActor :type Actor%20Object%20Reference) (OtherComp :type Primitive%20Component%20Object%20Reference) (OtherBodyIndex :type Integer) (bFromSweep :type Boolean) (SweepResult :type Hit%20Result%20Structure%20%28by%20ref%29))
  (Variables|Default|SetActive7 true)
  (Audio|PlaySound2D "/Game/Assets/Audio/Interaction/43400302_beep-short-16.43400302_beep-short-16" 1.0 1.0 0.0 0 0)
  (Development|PrintString "Hello")
  (if (Math|Boolean|ANDBoolean (Variables|Default|GetActive5) (Variables|Default|GetActive1) (Variables|Default|GetActive7) (Variables|Default|GetActive2))
    (Development|PrintString "1111111")
    (Audio|PlaySound2D "/Game/Sound/SoundWaves/Puzzle_Success.Puzzle_Success" 1.0 1.0 0.0 0 0)
    (CallFunction|OPG)))

(event OnComponentBeginOverlap(Box1)
  (params (OverlappedComponent :type Primitive%20Component%20Object%20Reference) (OtherActor :type Actor%20Object%20Reference) (OtherComp :type Primitive%20Component%20Object%20Reference) (OtherBodyIndex :type Integer) (bFromSweep :type Boolean) (SweepResult :type Hit%20Result%20Structure%20%28by%20ref%29))
  (Variables|Default|SetActive2 true)
  (Audio|PlaySound2D "/Game/Assets/Audio/Interaction/43400302_beep-short-16.43400302_beep-short-16" 1.0 1.0 0.0 0 0)
  (Development|PrintString "Hello")
  (if (Math|Boolean|ANDBoolean (Variables|Default|GetActive5) (Variables|Default|GetActive1) (Variables|Default|GetActive7) (Variables|Default|GetActive2))
    (Development|PrintString "1111111")
    (Audio|PlaySound2D "/Game/Sound/SoundWaves/Puzzle_Success.Puzzle_Success" 1.0 1.0 0.0 0 0)
    (CallFunction|OPG)))

(event OnComponentBeginOverlap(Box7)
  (params (OverlappedComponent :type Primitive%20Component%20Object%20Reference) (OtherActor :type Actor%20Object%20Reference) (OtherComp :type Primitive%20Component%20Object%20Reference) (OtherBodyIndex :type Integer) (bFromSweep :type Boolean) (SweepResult :type Hit%20Result%20Structure%20%28by%20ref%29))
  (CallFunction|ResetButton)
  (Audio|PlaySound2D "/Game/Assets/Audio/Interaction/43400302_beep-short-16.43400302_beep-short-16" 1.0 1.0 0.0 0 0))

(event OnComponentBeginOverlap(Box5)
  (params (OverlappedComponent :type Primitive%20Component%20Object%20Reference) (OtherActor :type Actor%20Object%20Reference) (OtherComp :type Primitive%20Component%20Object%20Reference) (OtherBodyIndex :type Integer) (bFromSweep :type Boolean) (SweepResult :type Hit%20Result%20Structure%20%28by%20ref%29))
  (CallFunction|ResetButton)
  (Audio|PlaySound2D "/Game/Assets/Audio/Interaction/43400302_beep-short-16.43400302_beep-short-16" 1.0 1.0 0.0 0 0))

(event OnComponentBeginOverlap(Box4)
  (params (OverlappedComponent :type Primitive%20Component%20Object%20Reference) (OtherActor :type Actor%20Object%20Reference) (OtherComp :type Primitive%20Component%20Object%20Reference) (OtherBodyIndex :type Integer) (bFromSweep :type Boolean) (SweepResult :type Hit%20Result%20Structure%20%28by%20ref%29))
  (CallFunction|ResetButton)
  (Audio|PlaySound2D "/Game/Assets/Audio/Interaction/43400302_beep-short-16.43400302_beep-short-16" 1.0 1.0 0.0 0 0))

(event OnComponentBeginOverlap(Box)
  (params (OverlappedComponent :type Primitive%20Component%20Object%20Reference) (OtherActor :type Actor%20Object%20Reference) (OtherComp :type Primitive%20Component%20Object%20Reference) (OtherBodyIndex :type Integer) (bFromSweep :type Boolean) (SweepResult :type Hit%20Result%20Structure%20%28by%20ref%29))
  (Variables|Default|SetActive1 true)
  (Audio|PlaySound2D "/Game/Assets/Audio/Interaction/43400302_beep-short-16.43400302_beep-short-16" 1.0 1.0 0.0 0 0)
  (Development|PrintString "Hello")
  (if (Math|Boolean|ANDBoolean (Variables|Default|GetActive5) (Variables|Default|GetActive1) (Variables|Default|GetActive7) (Variables|Default|GetActive2))
    (Development|PrintString "1111111")
    (Audio|PlaySound2D "/Game/Sound/SoundWaves/Puzzle_Success.Puzzle_Success" 1.0 1.0 0.0 0 0)
    (CallFunction|OPG)))

(event Custom|ResetButton
  (Variables|Default|SetActive1 false)
  (Variables|Default|SetActive5 false)
  (Variables|Default|SetActive2 false)
  (Variables|Default|SetActive7 false)
  (Development|PrintString "Reset"))

(event Custom|OPG
  (if (Math|Boolean|ANDBoolean (Variables|Default|GetActive5) (Variables|Default|GetActive1) (Variables|Default|GetActive7) (Variables|Default|GetActive2))
    (Default|Opentheglass (Variables|Default|GetGlassDoor))))

(fn ConstructionScript)

(fn Inspection
  (return 0))