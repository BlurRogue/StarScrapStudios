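; BP_Press is a code-entry puzzle actor built from a row of pressure pads, one per character of CorrectCode.
; The construction script spawns flattened meshes with overlap boxes above them.
; When BP_FirstPersonCharacter overlaps a box, its first component tag appends to the input, though the tag-assignment node from RandomCode is unconnected.
; At full length, a matching input plays a sound named as wrong-answer, while a mismatch clears it.
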(event EventBeginPlay)

(event Collision|EventActorBeginOverlap
  (params (OtherActor :type Actor%20Object%20Reference)))

(event EventTick
  (params (DeltaSeconds :type Float%20%28single-precision%29)))

(fn ConstructionScript
  (for _index (range 0 (- (Utilities|String|Len (Variables|Default|GetCorrectCode)) 1))
    (bind _returnvalue (AddComponent|AddStaticMeshComponent false (Math|Transform|MakeTransform (Math|Vector|MakeVector (* _index (Variables|Default|GetSpacing)) 0.0 0.0) "0, 0, 0" "1.000000,1.000000,0.100000")))
    (bind _returnvalue_2 (AddComponent|AddBoxComponent false (Math|Transform|MakeTransform (+ (Variables|/Script/Engine.SceneComponent|GetRelativeLocation _returnvalue) "0.000000,0.000000,50.000000") "0, 0, 0" "1.000000,1.000000,1.000000")))
    (Collision|BindEventtoOnComponentBeginOverlap _returnvalue_2 (EventDispatchers|CreateEvent :!event BPPressAutoGenFunc))))

(fn BPPressAutoGenFunc
  (params (OverlappedComponent :type Primitive%20Component%20Object%20Reference) (OtherActor :type Actor%20Object%20Reference) (OtherComp :type Primitive%20Component%20Object%20Reference) (OtherBodyIndex :type Integer) (bFromSweep :type Boolean) (SweepResult :type Hit%20Result%20Structure%20%28by%20ref%29))
  (Utilities|Casting|CastToBP_FirstPersonCharacter OtherActor)
  (CallFunction|Addcode (Utilities|String|ToString(Name) (Utilities|Array|Get(acopy) (Variables|/Script/Engine.ActorComponent|GetComponentTags OverlappedComponent))))
  (return))

(fn Addcode
  (params (ADD :type String))
  (Variables|Default|SetINPUTE (Utilities|String|Append (Variables|Default|GetINPUTE) ADD))
  (if (== (Utilities|String|Len (Variables|Default|GetCorrectCode)) (Utilities|String|Len (Variables|Default|GetINPUTE)))
    (if (Utilities|Enum|Equal(Enum) (Variables|Default|GetCorrectCode) (Variables|Default|GetINPUTE))
      (Audio|PlaySound2D "/Game/Assets/Audio/Interaction/Door/38806354_wrong-answer-notification-01.38806354_wrong-answer-notification-01" 1.0 1.0 0.0 0 0)
      (else
        (Variables|Default|SetINPUTE "")))))