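; Interactable sliding double door that opens and closes via timeline, can auto-close after a delay, and can load another level.
; Construction script configures meshes, spacing, locks and sounds from DT_DoorIDs presets or custom values.
; Locked doors check the player's KeyIDs before unlocking and recolouring the lock lights.
; Trigger overlaps register it with the GameManager's interaction UI; highlighting uses custom depth, and an older component-tag interaction path remains, marked defunct.
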(event OnComponentBeginOverlap(Box1)
  (params (OverlappedComponent :type Primitive%20Component%20Object%20Reference) (OtherActor :type Actor%20Object%20Reference) (OtherComp :type Primitive%20Component%20Object%20Reference) (OtherBodyIndex :type Integer) (bFromSweep :type Boolean) (SweepResult :type Hit%20Result%20Structure%20%28by%20ref%29))
  ;[1 0.8403 0.1586] User Interface for RE Interaction Wheel
  (if (Variables|Default|GetcanTriggerIntUI?)
    (CallFunction|UIAdjustment OtherActor true)))

(event OnComponentEndOverlap(Box1)
  (params (OverlappedComponent :type Primitive%20Component%20Object%20Reference) (OtherActor :type Actor%20Object%20Reference) (OtherComp :type Primitive%20Component%20Object%20Reference) (OtherBodyIndex :type Integer))
  ;[1 0.8403 0.1586] User Interface for RE Interaction Wheel
  (if (Variables|Default|GetcanTriggerIntUI?)
    (CallFunction|UIAdjustment OtherActor false)))

(event OnComponentBeginOverlap(Box)
  (params (OverlappedComponent :type Primitive%20Component%20Object%20Reference) (OtherActor :type Actor%20Object%20Reference) (OtherComp :type Primitive%20Component%20Object%20Reference) (OtherBodyIndex :type Integer) (bFromSweep :type Boolean) (SweepResult :type Hit%20Result%20Structure%20%28by%20ref%29))
  ;[1 0.8403 0.1586] User Interface for RE Interaction Wheel
  (if (Variables|Default|GetcanTriggerIntUI?)
    (CallFunction|UIAdjustment OtherActor true)))

(event OnComponentEndOverlap(Box)
  (params (OverlappedComponent :type Primitive%20Component%20Object%20Reference) (OtherActor :type Actor%20Object%20Reference) (OtherComp :type Primitive%20Component%20Object%20Reference) (OtherBodyIndex :type Integer))
  ;[1 0.8403 0.1586] User Interface for RE Interaction Wheel
  (if (Variables|Default|GetcanTriggerIntUI?)
    (CallFunction|UIAdjustment OtherActor false)))

(event OnComponentBeginOverlap(InteractTrigger2)
  (params (OverlappedComponent :type Primitive%20Component%20Object%20Reference) (OtherActor :type Actor%20Object%20Reference) (OtherComp :type Primitive%20Component%20Object%20Reference) (OtherBodyIndex :type Integer) (bFromSweep :type Boolean) (SweepResult :type Hit%20Result%20Structure%20%28by%20ref%29))
  ;[1 0.8403 0.1586] User Interface for RE Interaction Wheel
  (CallFunction|UIAdjustment OtherActor true))

(event OnComponentEndOverlap(InteractTrigger2)
  (params (OverlappedComponent :type Primitive%20Component%20Object%20Reference) (OtherActor :type Actor%20Object%20Reference) (OtherComp :type Primitive%20Component%20Object%20Reference) (OtherBodyIndex :type Integer))
  ;[1 0.8403 0.1586] User Interface for RE Interaction Wheel
  (CallFunction|UIAdjustment OtherActor false))

(event Custom|LoadNextLevel
  (if (Variables|Default|GettriggerNextLevel?)
    (Game|OpenLevel(byName) (Variables|Default|GetlevelName))))

(event Custom|UnlockDoor
  ;[0.1788 0.8531 0.4099 0.5] UnlockDoor
  (switch Utilities|FlowControl|Switch|SwitchonE_DoorIDs (Variables|Default|GetDoorID)
    (:NewEnumerator1
      _)
    (:NewEnumerator2
      _)
    (:NewEnumerator3
      (Variables|Default|SetDoorID "NewEnumerator2" :!label _label))
    (:NewEnumerator6
      (goto _label))
    (:NewEnumerator8
      (goto _label))
    (:NewEnumerator4
      (goto _label))
    (:NewEnumerator7
      (goto _label))
    (:NewEnumerator9
      (goto _label)))
  (Variables|DoorLock|SetLockStatus "NewEnumerator2")
  (CallFunction|ChangeLockColor)
  ;;[1 1 1 0.5] Unlock Audio
  (Audio|PlaySoundatLocation (Variables|Audio|GetUnlockIntSound) (Transformation|GetActorLocation self) "0, 0, 0" 1.0 1.0 0.0 0 0 0 0))

(event Custom|ChangeLockColor
  ;[0.1613 0.4615 0.3019 0.5] Change Lock Color
  (switch Utilities|FlowControl|Switch|SwitchonE_DoorLockType (Variables|DoorLock|GetLockStatus)
    (:NewEnumerator0
      (Rendering|Material|SetMaterial (Variables|Default|GetDoorLock1) 2 "/Game/Actors/BuildingBlocks_v2/DoorLock/Door_Lock_Light0.Door_Lock_Light0"))
    (:NewEnumerator1
      (Rendering|Material|SetMaterial (Variables|Default|GetDoorLock1) 2 "/Game/Actors/BuildingBlocks_v2/DoorLock/Door_Lock_Light1.Door_Lock_Light1"))
    (:NewEnumerator2
      (Rendering|Material|SetMaterial (Variables|Default|GetDoorLock1) 2 "/Game/Actors/BuildingBlocks_v2/DoorLock/Door_Lock_Light2.Door_Lock_Light2"))))

(event Custom|DoorIsLocked
  ;[1 1 1 0.5] Door Locked
  ;;[1 1 1 0.5] Locked Jiggle Audio
  (Audio|PlaySound2D (Variables|Audio|GetLockedSound) 1.0 1.0 0.0 0 0))

(event Custom|getPlayerRef
  ;[0.166 0.4456 0.8615] Get Player Ref
  (bind _asbp_first_person_character (Utilities|Casting|CastToBP_FirstPersonCharacter (Game|GetPlayerCharacter 0)))
  (Variables|Default|SetplayerRef _asbp_first_person_character))

(event EventToggleHighlight
  (params (toggleEnum :type E_toggle%20Enum :default "NewEnumerator0"))
  ;[1 0.8392 0.4018] Toggle Highlight
  (if (Variables|Default|GetisInteractable)
    (switch Utilities|FlowControl|Switch|SwitchonE_toggle toggleEnum
      (:NewEnumerator0
        (if (Variables|Default|GethighlightActive)
          ;;[0.15 0.06655 0.06804 0.5] Turning Off Highlight
          (Utilities|FlowControl|Sequence :!label _label
            (:then_0
              (Variables|Default|SethighlightActive false))
            (:then_1
              (bind _array_element (Utilities|Array|ForEachLoopwithBreak (Components|GetChildrenComponents (Variables|Default|Getparent) false))
                (:LoopBody
                  (bind _asprimitive_component (Utilities|Casting|CastToPrimitiveComponent _array_element))
                  (Rendering|SetRenderCustomDepth _asprimitive_component false)))))
          (else
            ;;[0.07443 0.15 0.07585 0.5] Turning on Highlight
            (Utilities|FlowControl|Sequence :!label _label_2
              (:then_0
                (Variables|Default|SethighlightActive true))
              (:then_1
                (bind _array_element_2 (Utilities|Array|ForEachLoopwithBreak (Components|GetChildrenComponents (Variables|Default|Getparent) false))
                  (:LoopBody
                    (bind _asprimitive_component_2 (Utilities|Casting|CastToPrimitiveComponent _array_element_2))
                    (Rendering|SetRenderCustomDepth _asprimitive_component_2 true))))))))
      (:NewEnumerator1
        (goto _label_2))
      (:NewEnumerator2
        (goto _label)))))

(event EventCustomEvent1
  (params (componentHit :type Primitive%20Component%20Object%20Reference))
  (bind _componenttags (Variables|/Script/Engine.ActorComponent|GetComponentTags componentHit))
  (bind _leftdoor (Variables|Default|GetLeftDoor))
  (bind _rightdoor (Variables|Default|GetRightDoor))
  (bind _relativelocation (Variables|/Script/Engine.SceneComponent|GetRelativeLocation _leftdoor))
  (bind _relativelocation_2 (Variables|/Script/Engine.SceneComponent|GetRelativeLocation _rightdoor))
  ;[1 1 1 0.5] Original Functionality (Defunct)
  ;;[1 1 1 0.5] Interaction V2
  (if (Utilities|IsValid componentHit)
    (if (> (Utilities|Array|Length _componenttags) 0)
      (switch Utilities|FlowControl|Switch|SwitchonE_ComponentNum (Utilities|Enum|ByteToEnumE_ComponentNum (Math|Conversions|ToByte(Integer) (- (Math|Conversions|ToInteger(Byte) (Utilities|String|GetSubstring (Utilities|String|ToString(Name) (Utilities|Array|Get(acopy) _componenttags)) 10)) 1)))
        (:NewEnumerator0
          (switch Utilities|FlowControl|Switch|SwitchonE_DoorLockType (Variables|DoorLock|GetLockStatus)
            (:NewEnumerator0
              ;;;[0.15 0.15 0.15 0.5] Interacting with the Door
              (Utilities|FlowControl|FlipFlop :!label _label
                (:A
                  (Audio|PlaySound2D (Variables|Audio|GetDoorOpenIntSound) 1.0 1.0 0.55 0 0)
                  (Variables|Default|SetisOpen? true)
                  (bind (_direction _r_doorslide _l_doorslide) (Timeline|T_Door_Slide PlayFromStart)
                    (:Update
                      (Transformation|SetRelativeLocation _leftdoor (Math|Vector|MakeVector (.x _relativelocation) (* _r_doorslide (Variables|Spacial|GetDoorDistanceTarget)) (.z _relativelocation)) false false)
                      (Transformation|SetRelativeLocation _rightdoor (Math|Vector|MakeVector (.x _relativelocation_2) (* _l_doorslide (Variables|Spacial|GetDoorDistanceTarget)) (.z _relativelocation_2)) false false))
                    (:Finished
                      (if (Variables|Default|GetisOpen?)
                        (if (Variables|Other|GetCloseAfterDelay?)
                          (Utilities|FlowControl|Delay (Variables|Other|GetDelay))
                          (goto _label))))))
                (:B
                  (Audio|PlaySound2D (Variables|Audio|GetDoorCloseIntSound) 1.0 1.0 0.45 0 0)
                  (Variables|Default|SetisOpen? false)
                  (Timeline|T_Door_Slide ReverseFromEnd))))
            (:NewEnumerator1
              (CallFunction|DoorIsLocked))
            (:NewEnumerator2
              (goto _label))))
        (:NewEnumerator1
          (switch Utilities|FlowControl|Switch|SwitchonE_DoorLockType (Variables|DoorLock|GetLockStatus)
            (:NewEnumerator0
              (goto _label))
            (:NewEnumerator1
              (if (Utilities|IsValid (Variables|Default|GetplayerRef))
                (switch Utilities|FlowControl|Switch|SwitchonE_DoorLockType (Variables|DoorLock|GetLockStatus)
                  (:NewEnumerator0
                    (CallFunction|UnlockDoor :!label _label_2))
                  (:NewEnumerator1
                    (bind _array_element (Utilities|Array|ForEachLoopwithBreak (Variables|DoorLock|GetKeyID))
                      (:LoopBody
                        (if (not (Utilities|Array|ContainsItem (Variables|/Game/FirstPerson/Blueprints/BP_FirstPersonCharacter.BP_FirstPersonCharacter_C|GetkeyIDs (Variables|Default|GetplayerRef)) _array_element))
                          (Variables|Default|SetdoorUnlockFailed true)))
                      (:Completed
                        (if (Variables|Default|GetdoorUnlockFailed)
                          (CallFunction|DoorIsLocked)
                          (else
                            (goto _label_2))))))
                  (:NewEnumerator2
                    (goto _label_2)))
                (else
                  (Development|PrintString (Utilities|String|Append "Error: " (Utilities|GetDisplayName self) " failed to find playerRef")))))
            (:NewEnumerator2
              (goto _label))))))))

(event EventBeginPlay
  ;[0.9031 0.6287 0.1025] Event BeginPlay
  (CallFunction|GetPlayerRef)
  (CallFunction|FindGameManager))

(event EventInteract
  (params (Component :type Actor%20Component%20Object%20Reference))
  (bind _rightdoor (Variables|Default|GetRightDoor))
  (bind _leftdoor (Variables|Default|GetLeftDoor))
  (bind _relativelocation (Variables|/Script/Engine.SceneComponent|GetRelativeLocation _rightdoor))
  (bind _relativelocation_2 (Variables|/Script/Engine.SceneComponent|GetRelativeLocation _leftdoor))
  ;[1 0.5111 0] Interact
  (switch Utilities|FlowControl|Switch|SwitchonE_DoorLockType (Variables|DoorLock|GetLockStatus)
    (:NewEnumerator0
      (Utilities|FlowControl|Sequence :!label _label
        (:then_0
          (CallFunction|LoadNextLevel))
        (:then_1
          ;[0.9031 0.7646 0.2373] Opening and Closing the Door
          ;;[0.15 0.15 0.15 0.5] Interacting with the Door
          (Utilities|FlowControl|FlipFlop :!label _label_2
            (:A
              (Audio|PlaySoundatLocation (Variables|Audio|GetDoorOpenIntSound) (Transformation|GetActorLocation self) "0, 0, 0" 2.0 1.0 0.0 0 0 0 0)
              (Variables|Default|SetisOpen? true)
              (Components|Timeline|SetPlayRate (Variables|Default|GetDoorTimeline) (/ 1.0 (Variables|Default|GettimeToOpen)))
              (Utilities|FlowControl|DelayUntilNextTick)
              (bind (_direction _r_doorslide _l_doorslide) (Timeline|DoorTimeline PlayFromStart)
                (:Update
                  (Transformation|SetRelativeLocation _leftdoor (Math|Vector|MakeVector (.x _relativelocation_2) (* _r_doorslide (Variables|Spacial|GetDoorDistanceTarget)) (.z _relativelocation_2)) false false)
                  (Transformation|SetRelativeLocation _rightdoor (Math|Vector|MakeVector (.x _relativelocation) (* _l_doorslide (Variables|Spacial|GetDoorDistanceTarget)) (.z _relativelocation)) false false))
                (:Finished
                  (CallFunction|UpdateDisplayName true)
                  (if (Variables|Default|GetisOpen?)
                    (if (Variables|Other|GetCloseAfterDelay?)
                      (Utilities|FlowControl|Delay (Variables|Other|GetDelay))
                      (goto _label_2))))))
            (:B
              (Audio|PlaySoundatLocation (Variables|Audio|GetDoorCloseIntSound) (Transformation|GetActorLocation self) "0, 0, 0" 2.0 1.0 0.0 0 0 0 0)
              (Variables|Default|SetisOpen? false)
              (Components|Timeline|SetPlayRate (Variables|Default|GetDoorTimeline) (/ 1.0 (Variables|Default|GettimeToOpen)))
              (Utilities|FlowControl|DelayUntilNextTick)
              (Timeline|DoorTimeline ReverseFromEnd))))))
    (:NewEnumerator1
      ;[0.849 0.4128 0.06809] Unlocking the Door
      (if (Utilities|IsValid (Variables|Default|GetplayerRef))
        (Utilities|FlowControl|Sequence
          (:then_0
            (bind _array_element (Utilities|Array|ForEachLoopwithBreak (Variables|DoorLock|GetKeyID))
              (:LoopBody
                (if (not (Utilities|Array|ContainsItem (Variables|/Game/FirstPerson/Blueprints/BP_FirstPersonCharacter.BP_FirstPersonCharacter_C|GetkeyIDs (Variables|Default|GetplayerRef)) _array_element))
                  (Variables|Default|SetdoorUnlockFailed true)))
              (:Completed
                (if (Variables|Default|GetdoorUnlockFailed)
                  (CallFunction|DoorIsLocked)
                  (else
                    (CallFunction|UnlockDoor)))))))))
    (:NewEnumerator2
      (goto _label))))

(fn ConstructionScript
  (bind _leftdoor (Variables|Default|GetLeftDoor))
  (bind _rightdoor (Variables|Default|GetRightDoor))
  (bind _relativelocation (Variables|/Script/Engine.SceneComponent|GetRelativeLocation _rightdoor))
  (bind _relativelocation_2 (Variables|/Script/Engine.SceneComponent|GetRelativeLocation _leftdoor))
  ;[0.15 0.15 0.15 0.5] Begin Construction Script
  (|CallParentFunction)
  (switch Utilities|FlowControl|Switch|SwitchonE_DoorIDs (Variables|Default|GetDoorID)
    (:NewEnumerator0
      (Variables|Default|SetDoorID "NewEnumerator1")
      (Variables|Assets|SethasCasing? false)
      (Variables|Assets|SetLeftDoorAsset "/Game/Actors/BuildingBlocks/Doors/DoorAssets/Door_Narrow_L.Door_Narrow_L")
      (Variables|Spacial|SetL_DoorDistanceInt 0)
      (Variables|Spacial|SetL_DoorDistanceFloat 0.0)
      (Variables|Spacial|SetL_DoorSpacing 0.0)
      (Variables|Assets|SetRightDoorAsset "/Game/Actors/BuildingBlocks/Doors/DoorAssets/Door_Narrow_R.Door_Narrow_R")
      (Variables|Spacial|SetR_DoorDistanceInt 0)
      (Variables|Spacial|SetR_DoorDistanceFloat 0.0)
      (Variables|Spacial|SetR_DoorSpacing 0.0)
      (Variables|Assets|SetDoorCasingAsset "/Game/Actors/BuildingBlocks/Doors/DoorAssets/Door_Frame_Smaller_Door_.Door_Frame_Smaller_Door_")
      (Variables|DoorLock|SetLockStatus "NewEnumerator0")
      (Variables|DoorLock|SetNonNativeLockRef 0)
      (Variables|DoorLock|SethasNativeLock? true)
      (Variables|DoorLock|SetlockAssets "/Game/Actors/BuildingBlocks_v2/DoorLock/Door_Lock.Door_Lock")
      (Variables|DoorLock|Setlock1RelTrans (Variables|Default|Getlock1DefTrans))
      (Variables|DoorLock|Setlock2RelTrans (Variables|Default|Getlock2DefTrans))
      (Variables|DoorLock|SethasLock? false)
      (Variables|Spacial|Setoffset_Height 0.0)
      (Variables|Default|SetHasInitialTransform false)
      (Variables|Default|SetCurrentTransform "")
      (Variables|Default|SetInitialTransform "")
      (Variables|Default|SetLocationLock false)
      (Variables|Spacial|SetDoorDistanceTarget 0.0)
      (Utilities|Array|Clear (Variables|DoorLock|GetKeyID))
      (Variables|Audio|SetuseDefaultIntSounds true)
      (Variables|Audio|SetDoorOpenIntSound "/Game/Assets/Audio/Interaction/Door/SC_DoorOpen.SC_DoorOpen")
      (Variables|Audio|SetDoorCloseIntSound "/Game/Assets/Audio/Interaction/Door/SC_DoorClose.SC_DoorClose")
      (Variables|Audio|SetUnlockIntSound "/Game/Assets/Audio/Interaction/SC_ActionSuccess_Cue.SC_ActionSuccess_Cue")
      (Variables|Audio|SetLockedSound "/Game/Assets/Audio/Interaction/Door/SC_Locked02.SC_Locked02")
      (Variables|Other|SetCloseAfterDelay? false)
      (Variables|Other|SetDelay 5.0))
    (:NewEnumerator1
      _)
    (:NewEnumerator2
      _)
    (:NewEnumerator3
      _)
    (:NewEnumerator6
      _)
    (:NewEnumerator8
      _)
    (:NewEnumerator4
      _)
    (:NewEnumerator7
      _)
    (:NewEnumerator9
      _))
  (if (or (Utilities|Enum|Equal(Enum) (Utilities|String|EnumtoString (Variables|Default|GetDoorID)) "Unassigned") (Utilities|Enum|Equal(Enum) (Utilities|String|EnumtoString (Variables|Default|GetDoorID)) "Custom"))
    _
    (else
      (bind _returnvalue (Utilities|GetDataTableRow "/Game/Actors/BuildingBlocks_v2/DT_DoorIDs.DT_DoorIDs" (Utilities|String|StringToName (Utilities|String|EnumtoString (Variables|Default|GetDoorID))))
        (:then
          (Variables|Assets|SethasCasing? (.hasCasing? (Utilities|Struct|BreakS_DoorIDs _returnvalue)))
          (Variables|Assets|SetLeftDoorAsset (.LeftDoorAsset (Utilities|Struct|BreakS_DoorIDs _returnvalue)))
          (Variables|Spacial|SetL_DoorDistanceInt (.L_DoorDistanceInt (Utilities|Struct|BreakS_DoorIDs _returnvalue)))
          (Variables|Spacial|SetL_DoorDistanceFloat (.L_DoorDistanceFloat (Utilities|Struct|BreakS_DoorIDs _returnvalue)))
          (Variables|Spacial|SetL_DoorSpacing (.L_DoorSpacing (Utilities|Struct|BreakS_DoorIDs _returnvalue)))
          (Variables|Assets|SetRightDoorAsset (.RightDoorAsset (Utilities|Struct|BreakS_DoorIDs _returnvalue)))
          (Variables|Spacial|SetR_DoorDistanceInt (.R_DoorDistanceInt (Utilities|Struct|BreakS_DoorIDs _returnvalue)))
          (Variables|Spacial|SetR_DoorDistanceFloat (.R_DoorDistanceFloat (Utilities|Struct|BreakS_DoorIDs _returnvalue)))
          (Variables|Spacial|SetR_DoorSpacing (.R_DoorSpacing (Utilities|Struct|BreakS_DoorIDs _returnvalue)))
          (Variables|Assets|SetDoorCasingAsset (.DoorCasingAsset (Utilities|Struct|BreakS_DoorIDs _returnvalue)))
          (Variables|DoorLock|SetLockStatus "NewEnumerator0")
          (Variables|DoorLock|SetNonNativeLockRef 0)
          (Variables|DoorLock|SethasNativeLock? (.hasNativeLock? (Utilities|Struct|BreakS_DoorIDs _returnvalue)))
          (Variables|DoorLock|SetlockAssets (.lockAsset (Utilities|Struct|BreakS_DoorIDs _returnvalue)))
          (Variables|DoorLock|Setlock1RelTrans (.lock1RelTrans (Utilities|Struct|BreakS_DoorIDs _returnvalue)))
          (Variables|DoorLock|Setlock2RelTrans (.lock2RelTrans (Utilities|Struct|BreakS_DoorIDs _returnvalue)))
          (Variables|DoorLock|SethasLock? (.hasLock? (Utilities|Struct|BreakS_DoorIDs _returnvalue)))
          (Variables|Spacial|Setoffset_Height (.offset_Height (Utilities|Struct|BreakS_DoorIDs _returnvalue)))
          (Variables|Default|SetHasInitialTransform false)
          (Variables|Default|SetCurrentTransform "")
          (Variables|Default|SetInitialTransform "")
          (Variables|Default|SetLocationLock false)
          (Variables|Spacial|SetDoorDistanceTarget (.DoorDistanceTarget (Utilities|Struct|BreakS_DoorIDs _returnvalue)))
          (Variables|Audio|SetuseDefaultIntSounds (.useDefaultIntSounds (Utilities|Struct|BreakS_DoorIDs _returnvalue)))
          (Variables|Audio|SetDoorOpenIntSound (.DoorOpenIntSound (Utilities|Struct|BreakS_DoorIDs _returnvalue)))
          (Variables|Audio|SetDoorCloseIntSound (.DoorCloseIntSound (Utilities|Struct|BreakS_DoorIDs _returnvalue)))
          (Variables|Audio|SetUnlockIntSound (.UnlockIntSound (Utilities|Struct|BreakS_DoorIDs _returnvalue)))
          (Variables|Audio|SetLockedSound (.LockedSound (Utilities|Struct|BreakS_DoorIDs _returnvalue)))
          (Variables|Other|SetCloseAfterDelay? (.CloseAfterDelay? (Utilities|Struct|BreakS_DoorIDs _returnvalue)))
          (Variables|Other|SetDelay (.Delay (Utilities|Struct|BreakS_DoorIDs _returnvalue)))))))
  (switch Utilities|FlowControl|Switch|SwitchonE_DoorLockType (Variables|DoorLock|GetLockStatus)
    (:NewEnumerator0
      (Rendering|Material|SetMaterial (Variables|Default|GetDoorLock1) 2 "/Game/Actors/BuildingBlocks_v2/DoorLock/Door_Lock_Light0.Door_Lock_Light0"))
    (:NewEnumerator1
      (Rendering|Material|SetMaterial (Variables|Default|GetDoorLock1) 2 "/Game/Actors/BuildingBlocks_v2/DoorLock/Door_Lock_Light1.Door_Lock_Light1"))
    (:NewEnumerator2
      (Rendering|Material|SetMaterial (Variables|Default|GetDoorLock1) 2 "/Game/Actors/BuildingBlocks_v2/DoorLock/Door_Lock_Light2.Door_Lock_Light2")))
  ;[1 1 1 0.5] Location Lock Functionality
  (if (Variables|Default|GetLocationLock)
    ;;[1 1 1 0.5] Enforcing Location Lock
    (if (Variables|Default|GetHasInitialTransform)
      _
      (else
        (Variables|Default|SetInitialTransform (Transformation|GetWorldTransform (Variables|Default|GetDefaultSceneRoot)))
        (Variables|Default|SetHasInitialTransform true)))
    (Transformation|SetWorldLocation (Variables|Default|GetDefaultSceneRoot) (Math|Vector|MakeVector (.x (.location (Variables|Default|GetInitialTransform))) (.y (.location (Variables|Default|GetInitialTransform))) (.z (.location (Variables|Default|GetInitialTransform)))) false false)
    (else
      ;;[1 1 1 0.5] Error Handling for Location Lock
      (if (!= (Variables|Spacial|Getoffset_Height) 0.0)
        (Variables|Spacial|Setoffset_Height 0.0)
        (Development|PrintString "LOCATION LOCK NOT ACTIVE. RESETTING HEIGHT OFFSET"))))
  ;[1 1 1 0.5] Setting the Door Meshes
  (Components|StaticMesh|SetStaticMesh (Variables|Default|GetLeftDoor) (Variables|Assets|GetLeftDoorAsset))
  (Components|StaticMesh|SetStaticMesh (Variables|Default|GetRightDoor) (Variables|Assets|GetRightDoorAsset))
  (if (Variables|Assets|GethasCasing?)
    (Components|StaticMesh|SetStaticMesh (Variables|Default|GetDoor_Casing) (Variables|Assets|GetDoorCasingAsset)))
  (if (Variables|DoorLock|GethasLock?)
    (Components|StaticMesh|SetStaticMesh (Variables|Default|GetDoorLock1) (Variables|DoorLock|GetlockAssets))
    (Components|StaticMesh|SetStaticMesh (Variables|Default|GetDoorLock2) (Variables|DoorLock|GetlockAssets)))
  ;[1 1 1 0.5] Adjusting Door Spacing
  (Transformation|SetRelativeLocation _leftdoor (Math|Vector|MakeVector (+ (.x _relativelocation_2) (Variables|Spacial|GetL_DoorSpacing)) (+ (.y _relativelocation_2) (Variables|Spacial|GetL_DoorDistanceInt) 0.0) (.z _relativelocation_2)) false false)
  (Transformation|SetRelativeLocation _rightdoor (Math|Vector|MakeVector (+ (.x _relativelocation) (Variables|Spacial|GetR_DoorSpacing)) (Utilities|Operators|Subtract (.y _relativelocation) (Variables|Spacial|GetR_DoorDistanceInt) (Variables|Spacial|GetR_DoorDistanceFloat)) (.z _relativelocation)) false false)
  (Transformation|SetRelativeTransform (Variables|Default|GetDoorLock1) (Variables|DoorLock|Getlock1RelTrans) false false)
  (Transformation|SetRelativeTransform (Variables|Default|GetDoorLock2) (Variables|DoorLock|Getlock2RelTrans) false false))

(fn UIAdjustment
  (params (Other%20Actor :type Object%20Object%20Reference) (Add? :type Boolean))
  (LocalVariables|SetF_add? Add?)
  (Utilities|FlowControl|Sequence
    (:then_0
      (bind _asbp_first_person_character (Utilities|Casting|CastToBP_FirstPersonCharacter Other%20Actor))
      (if Add?
        (if (not (Variables|Default|GethasUI))
          (Default|FInteractabletoUI (Variables|Default|GetGameManagerRef) self true)
          (Variables|Default|SetHas%20UI true))
        (else
          (Utilities|FlowControl|Sequence
            (:then_0
              (bind _array_element (Utilities|Array|ForEachLoopwithBreak (Collision|GetOverlappingActors _asbp_first_person_character "/Game/Actors/Interactables/ParentClass/BP_InteractibleParent.BP_InteractibleParent_C" :!class /Script/Engine.Actor))
                (:LoopBody
                  (if (Math|Boolean|ORBoolean (== _array_element (Variables|Default|GetBox)) (== _array_element (Variables|Default|GetBox1)) (== _array_element (Variables|Default|GetInteractTrigger2)))
                    (goto _label Close)))))
            (:then_1
              (Utilities|FlowControl|Gate false :!label _label
                (:Exit
                  (Default|FInteractabletoUI (Variables|Default|GetGameManagerRef) self false)
                  (CallFunction|ToggleHighlight "NewEnumerator2")
                  (Variables|Default|SetHas%20UI false))))))))))

(fn UpdateDisplayName
  (params (Update? :type Boolean))
  (Utilities|FlowControl|Sequence
    (:then_0
      (switch Utilities|FlowControl|Switch|SwitchonE_DoorLockType (Variables|DoorLock|GetLockStatus)
        (:NewEnumerator0
          (if (Variables|Default|GetisOpen?) :!label _label
            (Variables|Default|SetdisplayName "Close Door")
            (else
              (Variables|Default|SetdisplayName "Open Door"))))
        (:NewEnumerator1
          (Variables|Default|SetdisplayName "Unlock Door"))
        (:NewEnumerator2
          (goto _label))))
    (:then_1
      (bind _array_element (Utilities|Array|ForEachLoopwithBreak (Collision|GetOverlappingActors (Variables|Default|GetplayerRef) "/Game/Actors/Interactables/ParentClass/BP_InteractibleParent.BP_InteractibleParent_C" :!class /Script/Engine.Actor))
        (:LoopBody
          (if (Variables|Default|GetcanTriggerIntUI?)
            (if (Math|Boolean|ORBoolean (== _array_element (Variables|Default|GetBox)) (== _array_element (Variables|Default|GetBox1)) (== _array_element (Variables|Default|GetInteractTrigger2)))
              (goto _label_2 Open))
            (elif (== _array_element (Variables|Default|GetInteractTrigger2))
              (goto _label_2 Open))))))
    (:then_2
      (Utilities|FlowControl|Gate true :!label _label_2
        (:Exit
          (Utilities|FlowControl|Sequence
            (:then_0
              (Default|FInteractabletoUI (Variables|Default|GetGameManagerRef) self false)
              (CallFunction|ToggleHighlight "NewEnumerator2")
              (Variables|Default|SetHas%20UI false))
            (:then_1
              (if Update?
                (Default|FInteractabletoUI (Variables|Default|GetGameManagerRef) self true)
                (Variables|Default|SetHas%20UI true)))))))))