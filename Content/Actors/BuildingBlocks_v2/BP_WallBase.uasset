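; Modular wall building actor that lays out child mesh components as a row of walls in its Construction Script.
; Each child takes its mesh and unit length from DT_wallIDs, keyed by wall type and scale.
; An UPDATE flag resizes per-wall arrays and recomputes transforms from cumulative lengths, orientation and junction offsets.
; Transforms are applied before recomputation, so they land on the next construction run; BeginPlay only prints Scale debug text.
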(event EventBeginPlay
  (bind _array_element (Utilities|Array|ForEachLoopwithBreak (Variables|Default|Getscale))
    (:LoopBody
      (Development|PrintString (Utilities|String|Append (Utilities|String|EnumtoString _array_element) " has byte " (Utilities|String|ToString(Integer) (Math|Conversions|ToInteger(Byte) _array_element)) " which could be added to be " (Utilities|String|ToString(Integer) (+ (Math|Conversions|ToInteger(Byte) _array_element) 1))) true true "(R=0.000000,G=0.660000,B=1.000000,A=1.000000)" 6e+01))))

(fn ConstructionScript
  (bind _avgwalldist (Variables|DONOTCHANGE|GetavgWallDist))
  (bind _wallunitdist (Variables|DONOTCHANGE|GetwallUnitDist))
  (bind _array_index_3 (Variables|Default|GetArray%20Index_3))
  (bind _output (Utilities|Array|Get(acopy) _wallunitdist _array_index_3))
  (bind _returnvalue (* _output _avgwalldist))
  ;[0.15 0.15 0.15 0.5] Begin Construction Script
  (|CallParentFunction)
  (Utilities|FlowControl|Sequence
    (:then_0
      (Utilities|FlowControl|Sequence
        (:then_0
          (if (Variables|Default|GetUPDATE)
            (Utilities|Array|Resize (Variables|Custom|GetWallAssets) (Variables|Default|GetnumOfWalls))
            (Utilities|Array|Resize (Variables|Default|GetWallIDs) (Variables|Default|GetnumOfWalls))
            (Utilities|Array|Resize (Variables|Custom|GetnumOfSides) (Variables|Default|GetnumOfWalls))
            (Utilities|Array|Resize (Variables|Default|GetpillarRelations) (Variables|Default|GetnumOfWalls))
            (Utilities|Array|Resize (Variables|DONOTCHANGE|GetwallTransforms) (Variables|Default|GetnumOfWalls))
            (Utilities|Array|Resize (Variables|DONOTCHANGE|GetwallUnitDist) (Variables|Default|GetnumOfWalls))
            (Utilities|Array|Resize (Variables|DONOTCHANGE|GetwallYTransforms) (Variables|Default|GetnumOfWalls))
            (Utilities|Array|Resize (Variables|Default|Getorientation) (Variables|Default|GetnumOfWalls))
            (Utilities|Array|Resize (Variables|Default|Getscale) (Variables|Default|GetnumOfWalls))
            (Variables|Default|SetUPDATE false)
            (Variables|Default|Setresize2 true)))
        (:then_1
          (for (_array_element _array_index) (Components|GetChildrenComponents (Variables|Default|GetStatic_Mesh) false)
            (Transformation|SetRelativeTransform _array_element (Utilities|Array|Get(acopy) (Variables|DONOTCHANGE|GetwallTransforms) _array_index) false false)))))
    (:then_1
      (for (_array_element_2 _array_index_2) (Components|GetChildrenComponents (Variables|Default|GetStatic_Mesh) false)
        (bind _asstatic_mesh_component (Utilities|Casting|CastToStaticMeshComponent _array_element_2))
        (Variables|Default|SetAs%20Static%20Mesh%20Component _asstatic_mesh_component)
        (Variables|Default|SetArray%20Index _array_index_2)
        (switch Utilities|FlowControl|Switch|SwitchonE_WallIDs (Utilities|Array|Get(acopy) (Variables|Default|GetWallIDs) _array_index_2)
          (:NewEnumerator6
            (Components|StaticMesh|SetStaticMesh (Variables|Default|GetAs%20Static%20Mesh%20Component) "/Game/Actors/BuildingBlocks_v2/Walls/StandardWall.StandardWall")
            (Utilities|Array|SetArrayElem (Variables|Default|GetWallIDs) (Variables|Default|GetArray%20Index) "NewEnumerator5")
            (Utilities|Array|SetArrayElem (Variables|DONOTCHANGE|GetwallUnitDist) (Variables|Default|GetArray%20Index) 1.0))
          (:NewEnumerator5
            _)
          (:NewEnumerator12
            _)
          (:NewEnumerator18
            _)
          (:NewEnumerator0
            _)
          (:NewEnumerator7
            _)
          (:NewEnumerator1
            _)
          (:NewEnumerator8
            _)
          (:NewEnumerator2
            _)
          (:NewEnumerator3
            _)
          (:NewEnumerator4
            _)
          (:NewEnumerator9
            _)
          (:NewEnumerator10
            _)
          (:NewEnumerator19
            _))
        (if (not (or (Utilities|Enum|Equal(Enum) (Utilities|String|EnumtoString (Utilities|Array|Get(acopy) (Variables|Default|GetWallIDs) _array_index_2)) "Unassigned") (Utilities|Enum|Equal(Enum) (Utilities|String|EnumtoString (Utilities|Array|Get(acopy) (Variables|Default|GetWallIDs) _array_index_2)) "Custom")))
          (bind _returnvalue_2 (Utilities|GetDataTableRow "/Game/Actors/BuildingBlocks_v2/Walls/DT_wallIDs.DT_wallIDs" (Utilities|String|StringToName (Utilities|String|Append (Utilities|String|EnumtoString (Utilities|Array|Get(acopy) (Variables|Default|GetWallIDs) _array_index_2)) "_" (Utilities|String|ToString(Integer) (+ (Math|Conversions|ToInteger(Byte) (Utilities|Array|Get(acopy) (Variables|Default|Getscale) (Variables|Default|GetArray%20Index))) 1)))))
            (:then
              (Components|StaticMesh|SetStaticMesh (Variables|Default|GetAs%20Static%20Mesh%20Component) (.wallMesh (Utilities|Struct|BreakS_WallIDs _returnvalue_2)))
              (Utilities|Array|SetArrayElem (Variables|DONOTCHANGE|GetwallUnitDist) (Variables|Default|GetArray%20Index) (.wallDist (Utilities|Struct|BreakS_WallIDs _returnvalue_2))))))))
    (:then_2
      (if (Variables|Default|Getresize2)
        (Utilities|FlowControl|Sequence
          (:then_0
            (for (_ _array_index_3) (Components|GetChildrenComponents (Variables|Default|GetStatic_Mesh) false)
              (Utilities|FlowControl|Sequence
                (:then_0
                  (bind (_array_element_3 _array_index_4) (Utilities|Array|ForEachLoopwithBreak (Variables|DONOTCHANGE|GetwallUnitDist) :!label _label)
                    (:LoopBody
                      (if (>= _array_index_4 _array_index_3)
                        (Variables|Default|SetArray%20Index_2 _array_index_4)
                        (Utilities|FlowControl|Sequence
                          (:then_0
                            (switch Utilities|FlowControl|Switch|SwitchonE_Rotation (Utilities|Array|Get(acopy) (Variables|Default|Getorientation) (Variables|Default|GetArray%20Index_2))
                              (:NewEnumerator0
                                (Utilities|Array|SetArrayElem (Variables|DONOTCHANGE|GetwallTransforms) (Variables|Default|GetArray%20Index_2) (Math|Transform|MakeTransform (Math|Vector|MakeVector 0.0 (* (Variables|DONOTCHANGE|GetTotalWallDistance) (Variables|DONOTCHANGE|GetavgWallDist) -1.0) 0.0) (Math|Rotator|MakeRotator 0.0 0.0 0.0) "1.000000,1.000000,1.000000")))
                              (:NewEnumerator1
                                (switch Utilities|FlowControl|Switch|SwitchonE_WallIDs (Utilities|Array|Get(acopy) (Variables|Default|GetWallIDs) (Variables|Default|GetArray%20Index_2))
                                  (:NewEnumerator18
                                    (Utilities|Array|SetArrayElem (Variables|DONOTCHANGE|GetwallTransforms) (Variables|Default|GetArray%20Index_2) (Math|Transform|MakeTransform (Math|Vector|MakeVector (+ (/ (* (Utilities|Array|Get(acopy) (Variables|DONOTCHANGE|GetwallUnitDist) (Variables|Default|GetArray%20Index_2)) (Variables|DONOTCHANGE|GetavgWallDist)) -2.0) 0.0) (+ (* (Variables|DONOTCHANGE|GetTotalWallDistance) (Variables|DONOTCHANGE|GetavgWallDist) -1.0) (/ (* (Utilities|Array|Get(acopy) (Variables|DONOTCHANGE|GetwallUnitDist) (Variables|Default|GetArray%20Index_2)) (Variables|DONOTCHANGE|GetavgWallDist)) -2.0)) 0.0) (Math|Rotator|MakeRotator 0.0 0.0 9e+01) "1.000000,1.000000,1.000000") :!label _label_2))
                                  (:NewEnumerator0
                                    (goto _label_2))
                                  (:NewEnumerator7
                                    (goto _label_2))
                                  (:NewEnumerator1
                                    (goto _label_2))
                                  (:NewEnumerator8
                                    (goto _label_2))
                                  (:NewEnumerator2
                                    (goto _label_2))
                                  (:NewEnumerator3
                                    (goto _label_2))
                                  (:NewEnumerator4
                                    (Utilities|Array|SetArrayElem (Variables|DONOTCHANGE|GetwallTransforms) (Variables|Default|GetArray%20Index_2) (Math|Transform|MakeTransform (Math|Vector|MakeVector (+ (/ (* (Utilities|Array|Get(acopy) (Variables|DONOTCHANGE|GetwallUnitDist) (Variables|Default|GetArray%20Index_2)) (Variables|DONOTCHANGE|GetavgWallDist)) -1.0) 53.0) (+ (+ (* 54.0 (Utilities|Array|Get(acopy) (Variables|DONOTCHANGE|GetwallUnitDist) (Variables|Default|GetArray%20Index_2))) (* -1.0 (Utilities|Array|Get(acopy) (Variables|DONOTCHANGE|GetwallUnitDist) (Variables|Default|GetArray%20Index_2)) 8.1e+02) 0.0) (* (Variables|DONOTCHANGE|GetTotalWallDistance) (Variables|DONOTCHANGE|GetavgWallDist) -1.0)) 0.0) (Math|Rotator|MakeRotator 0.0 0.0 9e+01) "1.000000,1.000000,1.000000") :!label _label_3))
                                  (:NewEnumerator9
                                    (goto _label_3))
                                  (:NewEnumerator10
                                    (goto _label_3))
                                  (:NewEnumerator19
                                    (goto _label_3))))
                              (:NewEnumerator2
                                (Utilities|Array|SetArrayElem (Variables|DONOTCHANGE|GetwallTransforms) (Variables|Default|GetArray%20Index_2) (Math|Transform|MakeTransform (Math|Vector|MakeVector 0.0 (+ (* (Variables|DONOTCHANGE|GetTotalWallDistance) (Variables|DONOTCHANGE|GetavgWallDist) -1.0) (/ (* (Utilities|Array|Get(acopy) (Variables|DONOTCHANGE|GetwallUnitDist) (Variables|Default|GetArray%20Index_2)) (Variables|DONOTCHANGE|GetavgWallDist)) -1.0)) 0.0) (Math|Rotator|MakeRotator 0.0 0.0 1.8e+02) "1.000000,1.000000,1.000000")))
                              (:NewEnumerator3
                                (switch Utilities|FlowControl|Switch|SwitchonE_WallIDs (Utilities|Array|Get(acopy) (Variables|Default|GetWallIDs) (Variables|Default|GetArray%20Index_2))
                                  (:NewEnumerator18
                                    (Utilities|Array|SetArrayElem (Variables|DONOTCHANGE|GetwallTransforms) (Variables|Default|GetArray%20Index_2) (Math|Transform|MakeTransform (Math|Vector|MakeVector (+ (/ _returnvalue 2.0) 0.0) (+ (* (Variables|DONOTCHANGE|GetTotalWallDistance) (Variables|DONOTCHANGE|GetavgWallDist) -1.0) (/ _returnvalue -2.0)) 0.0) (Math|Rotator|MakeRotator 0.0 0.0 2.7e+02) "1.000000,1.000000,1.000000") :!label _label_4))
                                  (:NewEnumerator0
                                    (goto _label_4))
                                  (:NewEnumerator7
                                    (goto _label_4))
                                  (:NewEnumerator1
                                    (goto _label_4))
                                  (:NewEnumerator8
                                    (goto _label_4))
                                  (:NewEnumerator2
                                    (goto _label_4))
                                  (:NewEnumerator3
                                    (goto _label_4))
                                  (:NewEnumerator4
                                    (Utilities|Array|SetArrayElem (Variables|DONOTCHANGE|GetwallTransforms) (Variables|Default|GetArray%20Index_2) (Math|Transform|MakeTransform (Math|Vector|MakeVector (+ (* (Utilities|Array|Get(acopy) (Variables|DONOTCHANGE|GetwallUnitDist) (Variables|Default|GetArray%20Index_2)) (Variables|DONOTCHANGE|GetavgWallDist)) (* 53.0 -1.0 (Utilities|Array|Get(acopy) (Variables|DONOTCHANGE|GetwallUnitDist) (Variables|Default|GetArray%20Index_2)))) (+ (* 54.0 (Utilities|Array|Get(acopy) (Variables|DONOTCHANGE|GetwallUnitDist) (Variables|Default|GetArray%20Index_2)) -1.0) (* (Variables|DONOTCHANGE|GetTotalWallDistance) (Variables|DONOTCHANGE|GetavgWallDist) -1.0)) 0.0) (Math|Rotator|MakeRotator 0.0 0.0 2.7e+02) "1.000000,1.000000,1.000000") :!label _label_5))
                                  (:NewEnumerator9
                                    (goto _label_5))
                                  (:NewEnumerator10
                                    (goto _label_5))
                                  (:NewEnumerator19
                                    (goto _label_5))))))
                          (:then_1
                            (Variables|DONOTCHANGE|SetTotalWallDistance 0.0 :!label _label_6)
                            (goto _label Break)))
                        (else
                          (Variables|DONOTCHANGE|SetTotalWallDistance (+ _array_element_3 (Variables|DONOTCHANGE|GetTotalWallDistance))))))
                    (:Completed
                      (goto _label_6)))))))
          (:then_1
            (Variables|Default|Setresize2 false)))))))