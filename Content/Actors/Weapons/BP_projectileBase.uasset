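; Base projectile actor that plays firing, bounce and impact sounds and triggers interactible objects it hits.
; It counts bounces reported by its ProjectileMovement component.
; On each hit it either plays a bounce sound or, when bouncing is off or the bounce limit is reached, plays the hit sound and destroys itself.
; Any hit BP_InteractibleParent actor also receives a Hit call.
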(event OnProjectileBounce(ProjectileMovement)
  (params (ImpactResult :type Hit%20Result%20Structure%20%28by%20ref%29) (ImpactVelocity :type Vector%20%28by%20ref%29 :default "0, 0, 0"))
  (Math|Integer|IncrementInt (Variables|Default|Getbounces)))

(event EventBeginPlay
  (Audio|PlaySoundatLocation (Variables|Default|GetfireSound) (Transformation|GetActorLocation self) "0, 0, 0" 1.0 1.0 0.0 0 0 0 0))

(event Collision|EventHit
  (params (MyComp :type Primitive%20Component%20Object%20Reference) (Other :type Actor%20Object%20Reference) (OtherComp :type Primitive%20Component%20Object%20Reference) (bSelfMoved :type Boolean) (HitLocation :type Vector :default "0, 0, 0") (HitNormal :type Vector :default "0, 0, 0") (NormalImpulse :type Vector :default "0, 0, 0") (Hit :type Hit%20Result%20Structure%20%28by%20ref%29))
  (Utilities|FlowControl|Sequence
    (:then_0
      (if (Variables|/Script/Engine.ProjectileMovementComponent|GetbShouldBounce (Variables|MyProjectile|GetProjectileMovement))
        (if (>= (Variables|Default|Getbounces) (Variables|Default|GetmaxBounces))
          (Audio|PlaySoundatLocation (Variables|Default|GethitSound) (Transformation|GetActorLocation self) "0, 0, 0" 1.0 1.0 0.0 0 0 0 0 :!label _label)
          (Actor|DestroyActor)
          (else
            (Audio|PlaySoundatLocation (Variables|Default|GetbounceSound) (Transformation|GetActorLocation self) "0, 0, 0" 1.0 1.0 0.0 0 0 0 0)))
        (else
          (goto _label))))
    (:then_1
      (bind _asbp_interactible_parent (Utilities|Casting|CastToBP_InteractibleParent Other))
      (Default|Hit _asbp_interactible_parent))))

(fn ConstructionScript)