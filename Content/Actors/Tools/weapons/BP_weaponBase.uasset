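; Base weapon actor that the player can pick up and fire as either a hitscan or projectile gun.
; Trigger overlaps register it with the game manager's interaction UI, and custom depth on child components provides highlighting.
; Interacting snaps it to the character's gun container and sets GunRef.
; Firing either line-traces from the camera to call Hit on interactibles or spawns a projectile at the Ammo socket with camera rotation.
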(event OnComponentBeginOverlap(InteractTrigger)
  (params (OverlappedComponent :type Primitive%20Component%20Object%20Reference) (OtherActor :type Actor%20Object%20Reference) (OtherComp :type Primitive%20Component%20Object%20Reference) (OtherBodyIndex :type Integer) (bFromSweep :type Boolean) (SweepResult :type Hit%20Result%20Structure%20%28by%20ref%29))
  ;[1 0.8403 0.1586] User Interface for RE Interaction Wheel
  (Utilities|Casting|CastToBP_FirstPersonCharacter OtherActor)
  (Default|FInteractabletoUI (Variables|Default|GetGameManagerRef) self true))

(event OnComponentEndOverlap(InteractTrigger)
  (params (OverlappedComponent :type Primitive%20Component%20Object%20Reference) (OtherActor :type Actor%20Object%20Reference) (OtherComp :type Primitive%20Component%20Object%20Reference) (OtherBodyIndex :type Integer))
  ;[1 0.8403 0.1586] User Interface for RE Interaction Wheel
  (Utilities|Casting|CastToBP_FirstPersonCharacter OtherActor)
  (Default|FInteractabletoUI (Variables|Default|GetGameManagerRef) self false)
  (CallFunction|ToggleHighlight "NewEnumerator2"))

(event Custom|fireHitScan
  (bind _as_bp_first_person_character (Variables|Default|GetAs%20BP%20First%20Person%20Character))
  (bind _firstpersoncamera (Variables|/Game/FirstPerson/Blueprints/BP_FirstPersonCharacter.BP_FirstPersonCharacter_C|GetFirstPersonCamera _as_bp_first_person_character))
  (bind _returnvalue (Transformation|GetWorldLocation _firstpersoncamera))
  ;[0.8448 0.1206 0.1206 0.5] Fire Hit Scan
  (Utilities|FlowControl|Sequence
    (:then_0
      (bind (_outhit _returnvalue_2) (Collision|LineTraceByChannel _returnvalue (+ _returnvalue (* (Math|Vector|GetForwardVector _firstpersoncamera) (Variables|hitscan|GethitScanDistance))) "TraceTypeQuery1" false 0 "ForDuration"))
      (if _returnvalue_2
        (bind _asbp_interactible_parent (Utilities|Casting|CastToBP_InteractibleParent (.HitActor (Collision|BreakHitResult _outhit))))
        (Default|Hit _asbp_interactible_parent)
        (Audio|PlaySoundatLocation (Variables|hitscan|GethitScan_hitSound) (Transformation|GetWorldLocation (.HitComponent (Collision|BreakHitResult _outhit))) "0, 0, 0" 1.0 1.0 0.0 0 0 0 0)))
    (:then_1
      (Audio|PlaySoundatLocation (Variables|hitscan|GetHitScanFireSound) (Transformation|GetActorLocation self) "0, 0, 0" 1.0 1.0 0.0 0 0 0 0))))

(event Custom|fireProjectile
  (bind _returnvalue (Game|GetPlayerCameraManager 0))
  (bind _returnvalue_2 (Camera|GetCameraRotation _returnvalue))
  ;[0.7781 0.2324 0.08092 0.5] Fire Projectile
  (Game|SpawnActorfromClass (Utilities|GetClass (Variables|Default|Getprojectile)) (Math|Transform|MakeTransform (+ (Transformation|GetSocketLocation (Variables|Default|Getgun) "Ammo") (Math|Vector|RotateVector (Variables|Default|GetProjectileOffset) _returnvalue_2)) _returnvalue_2) "Undefined" "OverrideRootScale" 0 0)
  (Development|PrintString "Hello"))

(event Custom|OnFire
  (Utilities|FlowControl|Sequence
    (:then_0
      (if (Variables|hitscan|Gethitscan?)
        (CallFunction|FireHitScan)
        (else
          (CallFunction|FireProjectile))))
    (:then_1
      ;[1 1 1 0.5] Firing Sound
      (Audio|PlaySound2D (Variables|hitscan|GetHitScanFireSound) 1.0 1.0 0.0 0 0))))

(event EventBeginPlay
  ;[1 0.6329 0.2448] Event BeginPlay
  (Utilities|FlowControl|Sequence
    (:then_0
      (bind _asbp_first_person_character (Utilities|Casting|CastToBP_FirstPersonCharacter (Game|GetPlayerCharacter 0)))
      (Variables|Default|SetAs%20BP%20First%20Person%20Character _asbp_first_person_character))
    (:then_1
      (CallFunction|FindGameManager))))

(event EventToggleHighlight
  (params (toggleEnum :type E_toggle%20Enum :default "NewEnumerator0"))
  ;[1 0.8392 0.4018] Toggle Highlight
  (if (Variables|Default|GetisInteractable)
    (switch Utilities|FlowControl|Switch|SwitchonE_toggle toggleEnum
      (:NewEnumerator0
        (if (Variables|Default|GethighlightActive)
          ;;[0.15 0.06655 0.06804 0.5] Turning Off Highlight
          (Utilities|FlowControl|Sequence :!label _label
            (:then_0
              (Variables|Default|SethighlightActive false))
            (:then_1
              (bind _array_element (Utilities|Array|ForEachLoopwithBreak (Components|GetChildrenComponents (Variables|Default|Getparent) false))
                (:LoopBody
                  (bind _asprimitive_component (Utilities|Casting|CastToPrimitiveComponent _array_element))
                  (Rendering|SetRenderCustomDepth _asprimitive_component false)))))
          (else
            ;;[0.07443 0.15 0.07585 0.5] Turning on Highlight
            (Utilities|FlowControl|Sequence :!label _label_2
              (:then_0
                (Variables|Default|SethighlightActive true))
              (:then_1
                (bind _array_element_2 (Utilities|Array|ForEachLoopwithBreak (Components|GetChildrenComponents (Variables|Default|Getparent) false))
                  (:LoopBody
                    (bind _asprimitive_component_2 (Utilities|Casting|CastToPrimitiveComponent _array_element_2))
                    (Rendering|SetRenderCustomDepth _asprimitive_component_2 true))))))))
      (:NewEnumerator1
        (goto _label_2))
      (:NewEnumerator2
        (goto _label)))))

(event EventInteract
  (params (Component :type Actor%20Component%20Object%20Reference))
  ;[1 0.6883 0.114] Interact
  (CallFunction|PlayInteractSound)
  (Default|FInteractabletoUI (Variables|Default|GetGameManagerRef) self false)
  (Collision|SetActorEnableCollision self false)
  (Transformation|AttachComponentToComponent self (Variables|/Game/FirstPerson/Blueprints/BP_FirstPersonCharacter.BP_FirstPersonCharacter_C|GetgunContainer (Variables|Default|GetAs%20BP%20First%20Person%20Character)) "GripPoint" "SnapToTarget" "SnapToTarget" "SnapToTarget" true)
  (Variables|/Game/FirstPerson/Blueprints/BP_FirstPersonCharacter.BP_FirstPersonCharacter_C|SetgunRef (Variables|Default|GetAs%20BP%20First%20Person%20Character) self))

(fn ConstructionScript
  (Components|StaticMesh|SetStaticMesh (Variables|Default|GetStatic_Mesh) 0)
  (Components|StaticMesh|SetStaticMesh (Variables|Default|Getgun) (Variables|Default|GetgunMesh)))