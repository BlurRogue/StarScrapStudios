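; Locker safe puzzle actor with a door and spinnable digit dials.
; InteractV2 reads a number from the hit component's first tag to either play a locked jiggle or spin a digit with sound and MoveComponentTo, deriving roll from relative location X.
; PuzzleSuccess plays a success sound and swings the door open through a timeline.
; No combination check happens in this Blueprint.
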(event Custom|PuzzleSuccess
  (Audio|PlaySoundatLocation (Variables|Audio|GetPuzzleSuccessSound) (Transformation|GetWorldLocation (Variables|Default|GetDefaultSceneRoot self)) "0, 0, 0" 1.0 1.0 0.0 0 0 0 0)
  (CallFunction|RotateDoor))

(event Custom|RotateDoor
  (bind _lockerdoor (Variables|Default|GetLockerDoor))
  (bind _relativerotation (Variables|/Script/Engine.SceneComponent|GetRelativeRotation _lockerdoor))
  (bind _newtrack_0 (Timeline|Timeline Play)
    (:Update
      (Transformation|SetRelativeRotation _lockerdoor (Math|Rotator|MakeRotator (.roll _relativerotation) (.pitch _relativerotation) (* _newtrack_0 -1.3e+02)) false false))))

(event EventBeginPlay)

(event Collision|EventActorBeginOverlap
  (params (OtherActor :type Actor%20Object%20Reference)))

(event EventTick
  (params (DeltaSeconds :type Float%20%28single-precision%29)))

(event EventInteractV2
  (params (componentHit :type Primitive%20Component%20Object%20Reference))
  (bind _componenttags (Variables|/Script/Engine.ActorComponent|GetComponentTags componentHit))
  (Variables|Default|SetcurComponent componentHit)
  (if (Utilities|IsValid componentHit)
    (if (> (Utilities|Array|Length _componenttags) 0)
      (switch Utilities|FlowControl|Switch|SwitchonE_ComponentNum (Utilities|Enum|ByteToEnumE_ComponentNum (Math|Conversions|ToByte(Integer) (- (Math|Conversions|ToInteger(Byte) (Utilities|String|GetSubstring (Utilities|String|ToString(Name) (Utilities|Array|Get(acopy) _componenttags)) 10)) 1)))
        (:NewEnumerator1
          ;[0.15 0.15 0.15 0.5] Play a door locked sound
          (if true
            (Audio|PlaySound2D (Variables|Audio|GetLockedJiggleSound) 1.0 1.0 0.0 0 0)))
        (:NewEnumerator2
          (Audio|PlaySoundatLocation (Variables|Audio|GetDigitSpin) (Variables|/Script/Engine.SceneComponent|GetRelativeLocation (Variables|Default|GetcurComponent)) "0, 0, 0" 1.0 1.0 0.0 0 0 0 0 :!label _label)
          (Components|MoveComponentTo (Variables|Default|GetcurComponent) "0, 0, 0" (Math|Rotator|MakeRotator (.roll (Math|Rotator|MakeRotator (+ (.x (Variables|/Script/Engine.SceneComponent|GetRelativeLocation (Variables|Default|GetcurComponent))) -36.0) 0.0 0.0)) 0.0 0.0) false false 0.2 false))
        (:NewEnumerator3
          (goto _label))
        (:NewEnumerator4
          (goto _label))))))

(fn ConstructionScript)