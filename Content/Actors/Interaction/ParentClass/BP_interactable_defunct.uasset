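; BP_interactable_defunct is an interactable parent class, apparently retired, that holds only grid index helpers and an empty construction script.
; One function flattens one-based X and Y coordinates into a row-major, one-based index using Width.
; The inverse finds Y by repeatedly subtracting Width and X by modulo, so last-column cells return X as 0.
; Both functions take a Height input but never use it.
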(fn ConstructionScript)

(fn ConvertXandYtoArrayValue
  (params (X :type Integer) (Y :type Integer) (Width :type Integer) (Height :type Integer))
  (return (+ (- (Math|Integer|%(Integer) X (+ Width 1)) 1) (+ (* (- Y 1) Width) 1))))

(fn ConvertArrayValuetoXandY
  (params (Array%20Input :type Integer) (Width :type Integer) (Height :type Integer))
  (LocalVariables|SetY%20Output 1)
  (LocalVariables|SetChanging%20Value Array%20Input)
  (while (> (LocalVariables|GetChanging%20Value) Width)
    (LocalVariables|SetChanging%20Value (- (LocalVariables|GetChanging%20Value) Width))
    (LocalVariables|SetY%20Output (+ (LocalVariables|GetY%20Output) 1)))
  (return (Math|Integer|%(Integer) Array%20Input Width) (LocalVariables|GetY%20Output)))