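; Grandfather clock glass piece that swings around its yaw axis when interacted with, like a hinged panel.
; Interact calls Rotate, which plays or reverses the Glass_Rotation timeline depending on the HasRotated flag.
; The timeline scales its track to a yaw of up to 170 degrees on the static mesh.
; HasRotated flips on every timeline update rather than when the timeline finishes.
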(event Custom|Rotate
  (if (Variables|Default|GetHasRotated)
    (bind _newtrack_0 (Timeline|Glass_Rotation Reverse)
      (:Update
        (Transformation|SetRelativeRotation (Variables|Default|GetStatic_Mesh) (Math|Rotator|MakeRotator 0.0 0.0 (* _newtrack_0 1.7e+02)) false false)
        (if (Variables|Default|GetHasRotated)
          (Variables|Default|SetHasRotated false)
          (else
            (Variables|Default|SetHasRotated true)))))
    (else
      (Timeline|Glass_Rotation Play))))

(event EventBeginPlay)

(event Collision|EventActorBeginOverlap
  (params (OtherActor :type Actor%20Object%20Reference)))

(event EventTick
  (params (DeltaSeconds :type Float%20%28single-precision%29)))

(event EventInteract
  (CallFunction|Rotate))

(fn ConstructionScript)