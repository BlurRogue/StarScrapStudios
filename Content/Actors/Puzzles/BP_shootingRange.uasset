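; A shooting range puzzle actor with a sliding target and a configurable clue mesh.
; Construction sets the clue mesh and offsets the target along Y by InitialPosition.
; Hit works only once, easing the target along Y with MoveComponentTo, using MaxDistance, InitialPosition and TimeToSlide.
; ResetTarget slides it along X instead of Y and does not re-arm the DoOnce.
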(event Custom|ResetTarget
  (bind _shooting_range_target (Variables|Default|GetShooting_Range_Target))
  (Variables|Default|SetRelative%20Location (Variables|/Script/Engine.SceneComponent|GetRelativeLocation _shooting_range_target))
  (Components|MoveComponentTo _shooting_range_target (Math|Vector|MakeVector (- (.x (Variables|Default|GetRelative%20Location)) (- (Variables|Default|GetmaxDistance) (Variables|Default|GetinitialPosition))) (.y (Variables|Default|GetRelative%20Location)) (.z (Variables|Default|GetRelative%20Location))) (Variables|/Script/Engine.SceneComponent|GetRelativeRotation _shooting_range_target) false true (Variables|Default|GettimeToSlide) false))

(event EventHit
  (bind _shooting_range_target (Variables|Default|GetShooting_Range_Target))
  (Utilities|FlowControl|DoOnce false
    (:Completed
      (Variables|Default|SetRelative%20Location (Variables|/Script/Engine.SceneComponent|GetRelativeLocation _shooting_range_target))
      (Components|MoveComponentTo _shooting_range_target (Math|Vector|MakeVector (.x (Variables|Default|GetRelative%20Location)) (- (.y (Variables|Default|GetRelative%20Location)) (* (- (* (Variables|Default|GetmaxDistance) -1.0) (Variables|Default|GetinitialPosition)) -1.0)) (.z (Variables|Default|GetRelative%20Location))) (Variables|/Script/Engine.SceneComponent|GetRelativeRotation _shooting_range_target) true false (Variables|Default|GettimeToSlide) false))))

(fn ConstructionScript
  (bind _shooting_range_target (Variables|Default|GetShooting_Range_Target))
  (bind _relativelocation (Variables|/Script/Engine.SceneComponent|GetRelativeLocation _shooting_range_target))
  (Components|StaticMesh|SetStaticMesh (Variables|Default|Getclue) (Variables|Default|GetclueAsset))
  (Transformation|SetRelativeLocation _shooting_range_target (Math|Vector|MakeVector (.x _relativelocation) (+ (.y _relativelocation) (* (Variables|Default|GetinitialPosition) -1.0)) (.z _relativelocation)) false false))