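; Interactable puzzle stand where the player types WASD sequences over several timed rounds.
; Interacting blends the view to the stand and lists the round's required keys in its widget.
; Each input is prefix-checked, coloring characters and flickering key meshes via custom depth; the timer starts on first input through a gate.
; Mistakes or timeouts restart the round, while clearing the last round plays a success sound and restores the player view.
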(event OnComponentBeginOverlap(InteractTrigger)
  (params (OverlappedComponent :type Primitive%20Component%20Object%20Reference) (OtherActor :type Actor%20Object%20Reference) (OtherComp :type Primitive%20Component%20Object%20Reference) (OtherBodyIndex :type Integer) (bFromSweep :type Boolean) (SweepResult :type Hit%20Result%20Structure%20%28by%20ref%29))
  ;[1 0.8403 0.1586] User Interface for RE Interaction Wheel
  (Utilities|Casting|CastToBP_FirstPersonCharacter OtherActor)
  (Default|FInteractabletoUI (Variables|Default|GetGameManagerRef) self true))

(event OnComponentEndOverlap(InteractTrigger)
  (params (OverlappedComponent :type Primitive%20Component%20Object%20Reference) (OtherActor :type Actor%20Object%20Reference) (OtherComp :type Primitive%20Component%20Object%20Reference) (OtherBodyIndex :type Integer))
  ;[1 0.8403 0.1586] User Interface for RE Interaction Wheel
  (Utilities|Casting|CastToBP_FirstPersonCharacter OtherActor)
  (Default|FInteractabletoUI (Variables|Default|GetGameManagerRef) self false)
  (CallFunction|ToggleHighlight "NewEnumerator2"))

(event Custom|flickerKey
  ;[0.15 0.15 0.15 0.5] user timer by event
  ;;[1 0.8392 0.4018] flickerHighlight
  (bind _array_element (Utilities|Array|ForEachLoopwithBreak (Variables|Default|GetFlickeredKeys))
    (:LoopBody
      (Rendering|SetRenderCustomDepth _array_element false))))

(event Custom|triggerTimer
  (params (round :type Integer))
  ;[0.2115 0.1085 0.1233] Round Timer for Timing Out the Puzzle
  (Utilities|FlowControl|Sequence
    (:then_0
      (Utilities|FlowControl|Gate false :!label _label
        (:Exit
          (bind _returnvalue (Utilities|Time|SetTimerbyEvent (delegate Custom|endRound) (Utilities|Array|Get(acopy) (Variables|Default|GetpuzzleInputTimers) round)))
          (Variables|Default|SetendRoundEvent _returnvalue))))
    (:then_1
      (goto _label Close))))

(event Custom|getPlayerCharacter
  ;[0.15 0.15 0.15 0.5] Get Player Character
  (bind _asbp_first_person_character (Utilities|Casting|CastToBP_FirstPersonCharacter (Game|GetPlayerCharacter 0)))
  (Variables|Default|SetPlayerRef _asbp_first_person_character))

(event Custom|takeInput
  (params (input :type String))
  (bind _puzzleinputreqs (Variables|Default|GetpuzzleInputReqs))
  (bind _currentround (Variables|Default|GetcurrentRound))
  (bind _output (Utilities|Array|Get(acopy) _puzzleinputreqs _currentround))
  ;[0.03401 0.424 0.394] Take Input
  (CallFunction|TriggerTimer (Variables|Default|GetcurrentRound))
  (if (Utilities|Enum|Equal(Enum) (Utilities|String|Append (Variables|Default|GetrunningInputs) input) (Utilities|String|GetSubstring _output 0 (Utilities|String|Len (Utilities|String|Append (Variables|Default|GetrunningInputs) input))))
    (CallFunction|InputState (Utilities|Enum|Equal(Enum) (Utilities|String|Append (Variables|Default|GetrunningInputs) input) (Utilities|String|GetSubstring _output 0 (Utilities|String|Len (Utilities|String|Append (Variables|Default|GetrunningInputs) input)))))
    (bind _output_get (Variables|Default|SetrunningInputs (Utilities|String|Append (Variables|Default|GetrunningInputs) input)))
    (if (Utilities|Enum|Equal(Enum) _output_get _output)
      (CallFunction|ResetTimer)
      (CallFunction|FlickerUIState true)
      (if (>= (Variables|Default|GetcurrentRound) (- (Variables|Default|Getrounds) 1))
        (CallFunction|PuzzleSuccess)
        (else
          (bind _result (Math|Integer|IncrementInt (Variables|Default|GetcurrentRound))
            (:%20%20
              (CallFunction|UpdatePuzzleReqs _result))))))
    (else
      (CallFunction|InputState (Utilities|Enum|Equal(Enum) (Utilities|String|Append (Variables|Default|GetrunningInputs) input) (Utilities|String|GetSubstring _output 0 (Utilities|String|Len (Utilities|String|Append (Variables|Default|GetrunningInputs) input)))))
      (CallFunction|ResetTimer)
      (CallFunction|FlickerUIState (Utilities|Enum|Equal(Enum) (Utilities|String|Append (Variables|Default|GetrunningInputs) input) (Utilities|String|GetSubstring _output 0 (Utilities|String|Len (Utilities|String|Append (Variables|Default|GetrunningInputs) input)))))
      (Utilities|Time|SetTimerbyEvent (delegate Custom|restorePuzzle) (Variables|Default|GethighlightTime)))))

(event Custom|UpdatePuzzleReqs
  (params (round :type Integer))
  ;[0.07453 0.3222 0.5406] Update Puzzle Requirements
  (Utilities|FlowControl|Sequence
    (:then_0
      (bind _aswdg_wasd_stand (Utilities|Casting|CastToWDG_wasdStand (UserInterface|GetUserWidgetObject (Variables|Default|GetWidget))))
      (bind _output_get (Variables|Default|SetAs%20WDG%20Wasd%20Stand _aswdg_wasd_stand))
      (Widget|Panel|ClearChildren (Variables|/Game/UI/WDG_wasdStand.WDG_wasdStand_C|GetScrollBox _output_get)))
    (:then_1
      (bind _array_element (Utilities|Array|ForEachLoopwithBreak (Utilities|String|GetCharacterArrayfromString (Utilities|Array|Get(acopy) (Variables|Default|GetpuzzleInputReqs) round)))
        (:LoopBody
          (bind _returnvalue (UserInterface|CreateWidget "/Game/UI/WDG_text.WDG_text_C" 0 _array_element))
          (Widget|Panel|AddChild (Variables|/Game/UI/WDG_wasdStand.WDG_wasdStand_C|GetScrollBox (Variables|Default|GetAs%20WDG%20Wasd%20Stand)) _returnvalue))))
    (:then_2
      (Variables|Default|SetrunningInputs "")
      ;;[0.15 0.15 0.15 0.5] redundancy for safety
      (Variables|Default|SetcurrentRound round)
      ;;[1 1 1 0.5] Timer doesn't start until first input, see TakeInput and StartTimer
      (if true
        _))))

(event Custom|flickerHighlightKey
  (params (mesh :type Primitive%20Component%20Object%20Reference))
  ;[0.15 0.15 0.15 0.5] user timer by event
  ;;[1 0.8392 0.4018] flickerHighlight
  (Utilities|FlowControl|Sequence
    (:then_0
      (bind _array_element (Utilities|Array|ForEachLoopwithBreak (Variables|Default|GetFlickeredKeys))
        (:LoopBody
          (Rendering|SetRenderCustomDepth _array_element false)
          (if (Utilities|Time|IsValidTimerHandle (Variables|Default|GetflickerEvent))
            (Utilities|Time|ClearandInvalidateTimerbyHandle (Variables|Default|GetflickerEvent))))))
    (:then_1
      (Utilities|Array|Add (Variables|Default|GetFlickeredKeys) mesh)
      (Rendering|SetRenderCustomDepth mesh true))
    (:then_2
      (bind _returnvalue (Utilities|Time|SetTimerbyEvent (delegate Custom|flickerKey) (Variables|Default|GethighlightTime)))
      (Variables|Default|SetflickerEvent _returnvalue))))

(event Custom|resetTimer
  ;[0.2115 0.1085 0.1233] Round Timer for Timing Out the Puzzle
  (Utilities|FlowControl|Sequence
    (:then_0
      (Utilities|FlowControl|Gate false) ; enters at Open
    )
    (:then_1
      (if (Utilities|Time|IsValidTimerHandle (Variables|Default|GetendRoundEvent))
        (Utilities|Time|ClearandInvalidateTimerbyHandle (Variables|Default|GetendRoundEvent))))))

(event Custom|flickerUIState
  (params (success? :type Boolean))
  ;[0.15 0.15 0.15 0.5] user timer by event
  ;;[0.9448 0.6878 0.3338] Flicker Stand UI State
  (Utilities|FlowControl|Sequence
    (:then_0
      (bind _aswdg_wasd_stand (Utilities|Casting|CastToWDG_wasdStand (UserInterface|GetUserWidgetObject (Variables|Default|GetWidget)))))
    (:then_1
      (if success?
        (Variables|/Game/UI/WDG_wasdStand.WDG_wasdStand_C|SetslateBrushColor _aswdg_wasd_stand (Utilities|Struct|MakeSlateBrush (Utilities|Struct|MakeSlateColor "(R=0.000000,G=1.000000,B=0.228877,A=1.000000)") "Image" "NoTile" "NoMirror" "(X=32.000000,Y=32.000000)" "(Left=0.000000,Top=0.000000,Right=0.000000,Bottom=0.000000)" 0 "(CornerRadii=(X=0.000000,Y=0.000000,Z=0.000000,W=0.000000),Color=(SpecifiedColor=(R=0.000000,G=0.000000,B=0.000000,A=0.000000),ColorUseRule=UseColor_Specified),Width=0.000000,RoundingType=HalfHeightRadius,bUseBrushTransparency=False)"))
        (else
          (Variables|/Game/UI/WDG_wasdStand.WDG_wasdStand_C|SetslateBrushColor _aswdg_wasd_stand (Utilities|Struct|MakeSlateBrush (Utilities|Struct|MakeSlateColor "(R=1.000000,G=0.000000,B=0.000000,A=1.000000)") "Image" "NoTile" "NoMirror" "(X=32.000000,Y=32.000000)" "(Left=0.000000,Top=0.000000,Right=0.000000,Bottom=0.000000)" 0 "(CornerRadii=(X=0.000000,Y=0.000000,Z=0.000000,W=0.000000),Color=(SpecifiedColor=(R=0.000000,G=0.000000,B=0.000000,A=0.000000),ColorUseRule=UseColor_Specified),Width=0.000000,RoundingType=HalfHeightRadius,bUseBrushTransparency=False)")))))
    (:then_2
      (bind _returnvalue (Utilities|Time|SetTimerbyEvent (delegate Custom|restoreUIHighlight) (Variables|Default|GethighlightTime)))
      (Variables|Default|SetflickerUIEvent _returnvalue))))

(event Custom|endRound
  ;[0.2115 0.1085 0.1233] Round Timer for Timing Out the Puzzle
  ;;[1 0.2129 0.1312] EndRound
  (CallFunction|InputState false)
  (CallFunction|FlickerUIState false)
  (Utilities|FlowControl|Sequence
    (:then_0
      ;;;[1 1 1 0.5] If you want Custom Audio for timing out, put it here
      (if true
        _))
    (:then_1
      (Utilities|Time|SetTimerbyEvent (delegate Custom|restorePuzzle) (Variables|Default|GethighlightTime)))))

(event Custom|InputState
  (params (success :type Boolean))
  ;[0.5063 0.4603 1 0.5] InputState
  (Utilities|FlowControl|Sequence
    (:then_1
      (CallFunction|UpdateCharacter success))
    (:then_2
      (if success
        ;;[1 1 1 0.5] Audio for Inputs
        (Audio|PlaySoundatLocation (Variables|Default|GetSuccessInput) (Transformation|GetWorldLocation (Variables|Default|GetDefaultSceneRoot self)) "0, 0, 0" 1.0 1.0 0.0 0 0 0 0)
        (else
          (Audio|PlaySoundatLocation (Variables|Default|GetFailedInput) (Transformation|GetWorldLocation (Variables|Default|GetDefaultSceneRoot self)) "0, 0, 0" 1.0 1.0 0.0 0 0 0 0))))))

(event Custom|updatePuzzleRequirements
  (params (round :type Integer))
  ;[0.07453 0.3222 0.5406] Update Puzzle Requirements [Defunct]
  (Utilities|FlowControl|Sequence
    (:then_0
      (bind _aswdg_wasd_stand (Utilities|Casting|CastToWDG_wasdStand (UserInterface|GetUserWidgetObject (Variables|Default|GetWidget))))
      (Variables|/Game/UI/WDG_wasdStand.WDG_wasdStand_C|SetWASDCommands _aswdg_wasd_stand (Utilities|Array|Get(acopy) (Variables|Default|GetpuzzleInputReqs) round))
      ;;[0.15 0.15 0.15 0.5] redundancy for safety
      (Variables|Default|SetcurrentRound round)
      ;;[0.15 0.15 0.15 0.5] Timer doesn't start until first input, see TakeInput and StartTimer
      (if true
        _))
    (:then_1
      (Variables|Default|SetrunningInputs ""))))

(event Custom|restoreUIHighlight
  ;[0.15 0.15 0.15 0.5] user timer by event
  ;;[0.9448 0.6878 0.3338] Flicker Stand UI State
  (bind _aswdg_wasd_stand (Utilities|Casting|CastToWDG_wasdStand (UserInterface|GetUserWidgetObject (Variables|Default|GetWidget))))
  (Variables|/Game/UI/WDG_wasdStand.WDG_wasdStand_C|SetslateBrushColor _aswdg_wasd_stand (Utilities|Struct|MakeSlateBrush (Utilities|Struct|MakeSlateColor "(R=0.000000,G=0.000000,B=0.000000,A=1.000000)") "Image" "NoTile" "NoMirror" "(X=32.000000,Y=32.000000)" "(Left=0.000000,Top=0.000000,Right=0.000000,Bottom=0.000000)" 0 "(CornerRadii=(X=0.000000,Y=0.000000,Z=0.000000,W=0.000000),Color=(SpecifiedColor=(R=0.000000,G=0.000000,B=0.000000,A=0.000000),ColorUseRule=UseColor_Specified),Width=0.000000,RoundingType=HalfHeightRadius,bUseBrushTransparency=False)")))

(event Custom|UpdateCharacter
  (params (Success? :type Boolean))
  ;[0.15 0.15 0.15 0.5] user timer by event
  ;;[1 0.591 0.1718] Update Character
  (bind (_array_element _array_index) (Utilities|Array|ForEachLoopwithBreak (Class|PanelWidget|GetAllChildren (Variables|/Game/UI/WDG_wasdStand.WDG_wasdStand_C|GetScrollBox (Variables|Default|GetAs%20WDG%20Wasd%20Stand))))
    (:LoopBody
      (if (== _array_index (Utilities|String|Len (Variables|Default|GetrunningInputs)))
        (bind _aswdg_text (Utilities|Casting|CastToWDG_text _array_element))
        (if Success?
          (Variables|/Script/UMG.TextBlock|SetColorAndOpacity (Variables|/Game/UI/WDG_text.WDG_text_C|GetTextBlock _aswdg_text) (Utilities|Struct|MakeSlateColor "(R=0.000000,G=1.000000,B=0.201411,A=1.000000)"))
          (else
            (Variables|/Script/UMG.TextBlock|SetColorAndOpacity (Variables|/Game/UI/WDG_text.WDG_text_C|GetTextBlock _aswdg_text) (Utilities|Struct|MakeSlateColor "(R=1.000000,G=0.000000,B=0.076898,A=1.000000)"))))))))

(event Custom|playInteractSound
  ;[1 1 1 0.5] PuzzleSuccess
  ;;[1 1 1 0.5] InteractSound
  (Audio|PlaySoundatLocation (Variables|Default|GetinteractSound) (Transformation|GetWorldLocation (Variables|Default|GetDefaultSceneRoot self)) "0, 0, 0" 1.0 1.0 0.0 0 0 0 0))

(event Custom|restorePuzzle
  ;[0.03401 0.424 0.394] Take Input
  (CallFunction|UpdatePuzzleReqs (Variables|Default|GetcurrentRound)))

(event EventToggleHighlight
  (params (toggleEnum :type E_toggle%20Enum :default "NewEnumerator0"))
  ;[1 0.8392 0.4018] Toggle Highlight
  (if (Variables|Default|GetisInteractable)
    (switch Utilities|FlowControl|Switch|SwitchonE_toggle toggleEnum
      (:NewEnumerator0
        (if (Variables|Default|GethighlightActive)
          ;;[0.15 0.06655 0.06804 0.5] Turning Off Highlight
          (Utilities|FlowControl|Sequence :!label _label
            (:then_0
              (Variables|Default|SethighlightActive false))
            (:then_1
              (bind _array_element (Utilities|Array|ForEachLoopwithBreak (Components|GetChildrenComponents (Variables|Default|Getparent) false))
                (:LoopBody
                  (bind _as프리미티브_컴포넌트 (Utilities|Casting|CastToPrimitiveComponent _array_element))
                  (Rendering|SetRenderCustomDepth _as프리미티브_컴포넌트 false)))))
          (else
            ;;[0.07443 0.15 0.07585 0.5] Turning on Highlight
            (Utilities|FlowControl|Sequence :!label _label_2
              (:then_0
                (Variables|Default|SethighlightActive true))
              (:then_1
                (bind _array_element_2 (Utilities|Array|ForEachLoopwithBreak (Components|GetChildrenComponents (Variables|Default|Getparent) false))
                  (:LoopBody
                    (bind _as프리미티브_컴포넌트_2 (Utilities|Casting|CastToPrimitiveComponent _array_element_2))
                    (Rendering|SetRenderCustomDepth _as프리미티브_컴포넌트_2 true))))))))
      (:NewEnumerator1
        (goto _label_2))
      (:NewEnumerator2
        (goto _label)))))

(event EventPuzzleSuccess
  ;[1 1 1 0.5] PuzzleSuccess
  (Utilities|FlowControl|Sequence
    (:then_0
      ;;[1 1 1 0.5] Functionality for success
      (if true
        _))
    (:then_1
      ;;[1 1 1 0.5] Audio For Success
      (Audio|PlaySoundatLocation (Variables|Default|GetPuzzleSuccessSound) (Transformation|GetWorldLocation (Variables|Default|GetDefaultSceneRoot self)) "0, 0, 0" 1.0 1.0 0.0 0 0 0 0)
      ;;[1 1 1 0.5] Returning to Normal View
      (CallFunction|INPUT:Escape)
      ;;[1 1 1 0.5] Cleaning Up
      (Widget|Panel|ClearChildren (Variables|/Game/UI/WDG_wasdStand.WDG_wasdStand_C|GetScrollBox (Variables|Default|GetAs%20WDG%20Wasd%20Stand))))))

(event EventInteract
  (params (Component :type Actor%20Component%20Object%20Reference))
  (bind _playerref (Variables|Default|GetPlayerRef))
  ;[1 1 1] Interact // Setup
  (Utilities|FlowControl|Sequence
    (:then_0
      (CallFunction|PlayInteractSound))
    (:then_1
      (if (Utilities|IsValid _playerref)
        (if (Variables|/Game/FirstPerson/Blueprints/BP_FirstPersonCharacter.BP_FirstPersonCharacter_C|GetisFocusedOnPuzzle? _playerref)
          (CallFunction|INPUT:Escape)
          (else
            (if true :!label _label
              (CallFunction|GetPlayerCharacter)
              (Variables|/Game/FirstPerson/Blueprints/BP_FirstPersonCharacter.BP_FirstPersonCharacter_C|SetpuzzleRef (Variables|Default|GetPlayerRef) self)
              (Variables|/Game/FirstPerson/Blueprints/BP_FirstPersonCharacter.BP_FirstPersonCharacter_C|SetisFocusedOnPuzzle? (Variables|Default|GetPlayerRef) true)
              (Game|Player|SetViewTargetwithBlend (Game|GetPlayerController 0) self (Variables|Default|Getc_InitSwingTime) "VTBlend_Linear" 0.0 false)
              (Default|FInteractabletoUI (Variables|Default|GetGameManagerRef) self false)
              (CallFunction|UpdatePuzzleReqs))))
        (else
          (goto _label))))))

(event EventINPUT:Escape
  (bind _endroundevent (Variables|Default|GetendRoundEvent))
  ;[0.9865 0.3403 0.07518] Escape Inputs
  (CallFunction|OpenFocusGate)
  (Variables|/Game/FirstPerson/Blueprints/BP_FirstPersonCharacter.BP_FirstPersonCharacter_C|SetisFocusedOnPuzzle? (Variables|Default|GetPlayerRef) false)
  (Game|Player|SetViewTargetwithBlend (Game|GetPlayerController 0) (Game|Player|GetPlayerPawn 0) (Variables|Default|Getc_ReturnSwingTime) "VTBlend_Linear" 0.0 false)
  (if (Utilities|Time|IsValidTimerHandle _endroundevent)
    (Utilities|Time|ClearandInvalidateTimerbyHandle _endroundevent)))

(event EventINPUT:Up
  ;[1 0.7569 0.576] WASD Inputs
  (CallFunction|TakeInput "W")
  (CallFunction|FlickerHighlightKey (Variables|Default|GetW_key)))

(event EventINPUT:Down
  ;[1 0.7569 0.576] WASD Inputs
  (CallFunction|TakeInput "S")
  (CallFunction|FlickerHighlightKey (Variables|Default|GetS_key)))

(event EventINPUT:Left
  ;[1 0.7569 0.576] WASD Inputs
  (CallFunction|TakeInput "A")
  (CallFunction|FlickerHighlightKey (Variables|Default|GetA_key)))

(event EventINPUT:Right
  ;[1 0.7569 0.576] WASD Inputs
  (CallFunction|TakeInput "D")
  (CallFunction|FlickerHighlightKey (Variables|Default|GetD_key)))

(fn ConstructionScript
  (Utilities|Array|Resize (Variables|Default|GetpuzzleInputReqs) (Variables|Default|Getrounds))
  (Utilities|Array|Resize (Variables|Default|GetpuzzleInputTimers) (Variables|Default|Getrounds)))