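; Base puzzle actor that the first-person player can focus on, with a camera positioned from a transform variable on construction.
; A gate guards focusing, which registers the puzzle on the player, blends the view to it and removes it from interactable UI.
; Escape reopens the gate and blends back to the pawn.
; Success plays a sound; directional inputs and outline updates are empty stubs, and the gate's Enter trigger is unconnected.
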(event Custom|PuzzleSuccess
  (Audio|PlaySoundatLocation (Variables|Audio|GetPuzzleSuccessSound) (Transformation|GetWorldLocation (Variables|Default|GetDefaultSceneRoot self)) "0, 0, 0" 1.0 1.0 0.0 0 0 0 0))

(event Custom|FindPlayerRef
  (bind _asbp_first_person_character (Utilities|Casting|CastToBP_FirstPersonCharacter (Game|GetPlayerCharacter 0)))
  (Variables|Default|SetAs%20BP%20First%20Person%20Character _asbp_first_person_character))

(event Custom|CloseFocusGate
  (Utilities|FlowControl|Gate false) ; enters at Close
)

(event Custom|OpenFocusGate
  (Utilities|FlowControl|Gate false) ; enters at Open
)

(event Custom|INPUT:%20Up)

(event Custom|INPUT:%20Down)

(event Custom|INPUT:%20Left)

(event Custom|INPUT:%20Right)

(event Custom|INPUT:%20Escape
  (CallFunction|OpenFocusGate)
  (Variables|/Game/FirstPerson/Blueprints/BP_FirstPersonCharacter.BP_FirstPersonCharacter_C|SetisFocusedOnPuzzle? (Variables|Default|GetPlayerRef) false)
  (Game|Player|SetViewTargetwithBlend (Game|GetPlayerController 0) (Game|Player|GetPlayerPawn 0) (Variables|Default|Getc_ReturnSwingTime) "VTBlend_Linear" 0.0 false))

(event EventUpdateOutline)

(fn ConstructionScript
  (Transformation|SetRelativeTransform (Variables|Default|GetCamera) (Variables|Default|GetcameraTransform) false false))