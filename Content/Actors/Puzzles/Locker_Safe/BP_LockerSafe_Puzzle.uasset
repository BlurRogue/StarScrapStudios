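; BP_LockerSafe_Puzzle is an interactable locker safe puzzle whose door swings open when solved.
; Interact calls Gate and blends the player's view to the safe, whose camera transform is set in the construction script.
; PuzzleSuccess plays a sound and runs a timeline that yaws the door open.
; Tag-based logic for locked-jiggle and digit-spin feedback is present but never runs, and InteractV2 is empty.
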(event Custom|PuzzleSuccess
  (Audio|PlaySoundatLocation (Variables|Audio|GetPuzzleSuccessSound_0) (Transformation|GetWorldLocation (Variables|Default|GetDefaultSceneRoot self)) "0, 0, 0" 1.0 1.0 0.0 0 0 0 0)
  (CallFunction|RotateDoor))

(event Custom|RotateDoor
  (bind _lockerdoor (Variables|Default|GetLockerDoor))
  (bind _relativerotation (Variables|/Script/Engine.SceneComponent|GetRelativeRotation _lockerdoor))
  (bind _newtrack_0 (Timeline|Timeline Play)
    (:Update
      (Transformation|SetRelativeRotation _lockerdoor (Math|Rotator|MakeRotator (.roll _relativerotation) (.pitch _relativerotation) (* _newtrack_0 -1.3e+02)) false false))))

(event EventInteractV2
  (params (componentHit :type Primitive%20Component%20Object%20Reference)))

(event EventInteract
  (params (Component :type Actor%20Component%20Object%20Reference))
  (Utilities|FlowControl|Sequence
    (:then_0
      (Utilities|FlowControl|Gate true))
    (:then_1
      (Game|Player|SetViewTargetwithBlend (Game|GetPlayerController 0) self (Variables|Default|GetcameraSwingTime) "VTBlend_Linear" 0.0 false))))

(fn ConstructionScript
  (Transformation|SetRelativeTransform (Variables|Default|GetCamera_0) (Variables|Default|GetcameraTransform_0) false false))