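; BP_Locker is an interactable combination-lock puzzle: the correct code swings the locker door open and enables the item inside.
; Interacting blends the view to the locker, where directional inputs select a digit, highlighted through custom depth, or spin it.
; Each spin updates CurrentState and compares it with SuccessState, with arrays sized from the Digits children in the construction script.
; A trigger overlap registers the locker with the GameManager's interaction UI.
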(event OnComponentBeginOverlap(InteractTrigger)
  (params (OverlappedComponent :type Primitive%20Component%20Object%20Reference) (OtherActor :type Actor%20Object%20Reference) (OtherComp :type Primitive%20Component%20Object%20Reference) (OtherBodyIndex :type Integer) (bFromSweep :type Boolean) (SweepResult :type Hit%20Result%20Structure%20%28by%20ref%29))
  ;[1 0.8403 0.1586] User Interface for RE Interaction Wheel
  (Utilities|Casting|CastToBP_FirstPersonCharacter OtherActor)
  (Default|FInteractabletoUI (Variables|Default|GetGameManagerRef) self true))

(event OnComponentEndOverlap(InteractTrigger)
  (params (OverlappedComponent :type Primitive%20Component%20Object%20Reference) (OtherActor :type Actor%20Object%20Reference) (OtherComp :type Primitive%20Component%20Object%20Reference) (OtherBodyIndex :type Integer))
  ;[1 0.8403 0.1586] User Interface for RE Interaction Wheel
  (Utilities|Casting|CastToBP_FirstPersonCharacter OtherActor)
  (Default|FInteractabletoUI (Variables|Default|GetGameManagerRef) self false)
  (CallFunction|ToggleHighlight "NewEnumerator2")
  (CallFunction|TurnoffDigits))

(event Custom|executeSpin
  (params (component :type Scene%20Component%20Object%20Reference) (keyModifier :type Integer))
  ;[0.04107 0.1188 0.15] defunct
  ;;[1 1 1 0.5] Execute Spin
  (Components|MoveComponentTo component (Variables|/Script/Engine.SceneComponent|GetRelativeLocation component) (Math|Rotator|MakeRotator (+ (.roll (Variables|Default|Getrotation)) (* 36.0 keyModifier)) 0.0 0.0) false false (Variables|Default|GetdigitSpinTime) false))

(event Custom|PuzzleSuccess
  ;[1 1 1 0.5] Puzzle Success
  (Audio|PlaySoundatLocation (Variables|Audio|GetPuzzleSuccessSound_0) (Transformation|GetWorldLocation (Variables|Default|GetDefaultSceneRoot self)) "0, 0, 0" 1.0 1.0 0.0 0 0 0 0)
  (CallFunction|OpenDoor)
  (CallFunction|ToggleHighlight "NewEnumerator2")
  (CallFunction|TurnoffDigits)
  (CallFunction|EnableInternalItem))

(event Custom|sortDigits
  ;[1 1 1 0.5] Sort Digits (defunct
)

(event Custom|updateDigitIndex
  (params (keyModifier :type Integer))
  ;[1 0.8392 0.4018] updateIndex
  (bind _output_get (Variables|Default|SetKey%20Modifier keyModifier))
  (if (>= (+ _output_get (Variables|Default|GethighlightedDigit)) (Utilities|Array|Length (Variables|Default|GetsortedDigits)))
    (Variables|Default|SethighlightedDigit 0)
    (elif (< (+ _output_get (Variables|Default|GethighlightedDigit)) 0)
      (Variables|Default|SethighlightedDigit (- (Utilities|Array|Length (Variables|Default|GetsortedDigits)) 1))
      (else
        (Variables|Default|SethighlightedDigit (+ (Variables|Default|GetKey%20Modifier) (Variables|Default|GethighlightedDigit)))))))

(event Custom|CheckSuccessState
  ;[0 0.02281 0.15] Check Success State
  (Utilities|FlowControl|Sequence
    (:then_0
      (goto _label Open))
    (:then_1
      (bind (_array_element _array_index) (Utilities|Array|ForEachLoopwithBreak (Variables|Default|GetsuccessState))
        (:LoopBody
          (if (not (== _array_element (Utilities|Array|Get(acopy) (Variables|Default|GetcurrentState) _array_index)))
            (goto _label Close)))
        (:Completed
          (Utilities|FlowControl|Gate false :!label _label
            (:Exit
              (CallFunction|PuzzleSuccess))))))))

(event Custom|highlightDigit
  (params (key :type Integer))
  (bind _highlighteddigits (Variables|Default|GethighlightedDigits))
  ;[1 0.8392 0.4018] highlightDigit
  (Utilities|FlowControl|Sequence
    (:then_0
      (bind _array_element (Utilities|Array|ForEachLoopwithBreak _highlighteddigits)
        (:LoopBody
          (bind _asprimitive_component (Utilities|Casting|CastToPrimitiveComponent _array_element))
          (Rendering|SetRenderCustomDepth _asprimitive_component false))
        (:Completed
          (Utilities|Array|Clear _highlighteddigits))))
    (:then_1
      (bind (_array_element_2 _array_index) (Utilities|Array|ForEachLoopwithBreak (Components|GetChildrenComponents (Variables|Default|Getdigits) false))
        (:LoopBody
          (if (== _array_index key)
            (bind _asprimitive_component_2 (Utilities|Casting|CastToPrimitiveComponent _array_element_2))
            (Rendering|SetRenderCustomDepth _asprimitive_component_2 true)
            (Utilities|Array|Add (Variables|Default|GethighlightedDigits) _array_element_2)))))))

(event Custom|UpdateCurrentState
  (params (key%20Modifier :type Integer) (digitIndex :type Integer))
  ;[0.02779 0.06552 0.15] Update Success State
  (Utilities|FlowControl|Sequence
    (:then_0
      (Variables|Default|SetDigit%20Index digitIndex)
      (bind _output_get (Variables|Default|SetKey%20Modifier key%20Modifier))
      (if (>= (+ _output_get (Utilities|Array|Get(acopy) (Variables|Default|GetcurrentState) digitIndex)) (Variables|Default|GetmaxIndexOnDigit))
        (Utilities|Array|SetArrayElem (Variables|Default|GetcurrentState) (Variables|Default|GetDigit%20Index) 0)
        (elif (< (+ _output_get (Utilities|Array|Get(acopy) (Variables|Default|GetcurrentState) digitIndex)) 0)
          (Utilities|Array|SetArrayElem (Variables|Default|GetcurrentState) (Variables|Default|GetDigit%20Index) (- (Variables|Default|GetmaxIndexOnDigit) 1))
          (else
            (Utilities|Array|SetArrayElem (Variables|Default|GetcurrentState) (Variables|Default|GetDigit%20Index) (+ (Variables|Default|GetKey%20Modifier) (Utilities|Array|Get(acopy) (Variables|Default|GetcurrentState) (Variables|Default|GetDigit%20Index))))))))
    (:then_1
      (CallFunction|CheckSuccessState))))

(event Custom|OpenDoor
  (bind _lockerdoor (Variables|Default|GetlockerDoor))
  (bind _relativerotation (Variables|/Script/Engine.SceneComponent|GetRelativeRotation _lockerdoor))
  (Variables|Default|Setrotation (Variables|/Script/Engine.SceneComponent|GetRelativeRotation _lockerdoor))
  (Collision|SetCollisionEnabled _lockerdoor "NoCollision")
  (bind _newtrack_0 (Timeline|Timeline PlayFromStart)
    (:Update
      (Transformation|SetRelativeRotation _lockerdoor (Math|Rotator|MakeRotator (.roll _relativerotation) (.pitch _relativerotation) (+ (* (/ _newtrack_0 1e+02) (* (Variables|Default|GetDoorSwingAngle) -1.0)) (.yaw _relativerotation))) false false))))

(event Custom|turnoffDigits
  (bind _array_element (Utilities|Array|ForEachLoopwithBreak (Components|GetChildrenComponents (Variables|Default|Getdigits) false))
    (:LoopBody
      (bind _asprimitive_component (Utilities|Casting|CastToPrimitiveComponent _array_element))
      (Rendering|SetRenderCustomDepth _asprimitive_component false))))

(event Custom|CustomEvent
  ;[0.04107 0.1188 0.15] defunct
  (bind (_array_element _array_index) (Utilities|Array|ForEachLoopwithBreak (Components|GetChildrenComponents (Variables|Default|Getdigits) false))
    (:LoopBody
      (if (== _array_index (Variables|Default|GethighlightedDigit))
        ;;[1 1 1 0.5] Audio for Spinning Digit
        (Audio|PlaySoundatLocation (Variables|Audio|GetdigitSpinAudio) (Variables|/Script/Engine.SceneComponent|GetRelativeLocation _array_element) "0, 0, 0" 1.0 1.0 0.0 0 0 0 0)
        (Transformation|SetRelativeRotation _array_element (Math|Rotator|MakeRotator (.roll (Math|Rotator|MakeRotator (* (+ (.x (Variables|/Script/Engine.SceneComponent|GetRelativeLocation _array_element)) 36.0) 0.0) (.y (Variables|/Script/Engine.SceneComponent|GetRelativeLocation _array_element)) (.z (Variables|/Script/Engine.SceneComponent|GetRelativeLocation _array_element)))) (.pitch (Math|Rotator|MakeRotator (* (+ (.x (Variables|/Script/Engine.SceneComponent|GetRelativeLocation _array_element)) 36.0) 0.0) (.y (Variables|/Script/Engine.SceneComponent|GetRelativeLocation _array_element)) (.z (Variables|/Script/Engine.SceneComponent|GetRelativeLocation _array_element)))) (.yaw (Math|Rotator|MakeRotator (* (+ (.x (Variables|/Script/Engine.SceneComponent|GetRelativeLocation _array_element)) 36.0) 0.0) (.y (Variables|/Script/Engine.SceneComponent|GetRelativeLocation _array_element)) (.z (Variables|/Script/Engine.SceneComponent|GetRelativeLocation _array_element))))) false false)))))

(event Custom|spinDigit
  (params (key%20modifier :type Integer))
  ;[0.04107 0.1188 0.15] defunct
  (bind (_array_element _array_index) (Utilities|Array|ForEachLoopwithBreak (Components|GetChildrenComponents (Variables|Default|Getdigits) false) :!label _label)
    (:LoopBody
      (if (== _array_index (Variables|Default|GethighlightedDigit))
        ;;[1 1 1 0.5] Audio for Spinning Digit
        (Audio|PlaySoundatLocation (Variables|Audio|GetdigitSpinAudio) (Transformation|GetWorldLocation _array_element) "0, 0, 0" 1.0 1.0 0.0 0 0 0 0)
        (Variables|Default|Setrotation (Variables|/Script/Engine.SceneComponent|GetRelativeRotation _array_element))
        (CallFunction|ExecuteSpin _array_element key%20modifier)
        (goto _label Break)))))

(event Custom|playInteractSound
  ;[1 1 1 0.5] InteractSound
  (Audio|PlaySoundatLocation (Variables|Audio|GetinteractSound) (Transformation|GetWorldLocation (Variables|Default|GetDefaultSceneRoot self)) "0, 0, 0" 1.0 1.0 0.0 0 0 0 0))

(event EventToggleHighlight
  (params (toggleEnum :type E_toggle%20Enum :default "NewEnumerator0"))
  ;[1 0.8392 0.4018] Toggle Highlight
  (if (Variables|Default|GetisInteractable)
    (switch Utilities|FlowControl|Switch|SwitchonE_toggle toggleEnum
      (:NewEnumerator0
        (if (Variables|Default|GethighlightActive)
          ;;[0.15 0.06655 0.06804 0.5] Turning Off Highlight
          (Utilities|FlowControl|Sequence :!label _label
            (:then_0
              (Variables|Default|SethighlightActive false))
            (:then_1
              (bind _array_element (Utilities|Array|ForEachLoopwithBreak (Components|GetChildrenComponents (Variables|Default|Getparent) false))
                (:LoopBody
                  (bind _asprimitive_component (Utilities|Casting|CastToPrimitiveComponent _array_element))
                  (Rendering|SetRenderCustomDepth _asprimitive_component false)))))
          (else
            ;;[0.07443 0.15 0.07585 0.5] Turning on Highlight
            (Utilities|FlowControl|Sequence :!label _label_2
              (:then_0
                (Variables|Default|SethighlightActive true))
              (:then_1
                (bind _array_element_2 (Utilities|Array|ForEachLoopwithBreak (Components|GetChildrenComponents (Variables|Default|Getparent) false))
                  (:LoopBody
                    (bind _asprimitive_component_2 (Utilities|Casting|CastToPrimitiveComponent _array_element_2))
                    (Rendering|SetRenderCustomDepth _asprimitive_component_2 true))))))))
      (:NewEnumerator1
        (goto _label_2))
      (:NewEnumerator2
        (goto _label)))))

(event EventInteract
  (params (Component :type Actor%20Component%20Object%20Reference))
  (bind _as_bp_first_person_character (Variables|Default|GetAs%20BP%20First%20Person%20Character))
  (bind _as_bp_first_person_character_2 (Variables|Default|GetAs%20BP%20First%20Person%20Character))
  ;[1 1 1] Interact // Setup
  (Utilities|FlowControl|Sequence
    (:then_0
      (CallFunction|PlayInteractSound))
    (:then_1
      (if (Utilities|IsValid _as_bp_first_person_character)
        (if (Variables|/Game/FirstPerson/Blueprints/BP_FirstPersonCharacter.BP_FirstPersonCharacter_C|GetisFocusedOnPuzzle? _as_bp_first_person_character)
          (CallFunction|INPUT:Escape)
          (else
            (if true :!label _label
              (Variables|/Game/FirstPerson/Blueprints/BP_FirstPersonCharacter.BP_FirstPersonCharacter_C|SetpuzzleRef _as_bp_first_person_character_2 self)
              (Variables|/Game/FirstPerson/Blueprints/BP_FirstPersonCharacter.BP_FirstPersonCharacter_C|SetisFocusedOnPuzzle? _as_bp_first_person_character_2 true)
              (Game|Player|SetViewTargetwithBlend (Game|GetPlayerController 0) self (Variables|Default|GetDoorSwingTime) "VTBlend_Linear" 0.0 false)
              (Default|FInteractabletoUI (Variables|Default|GetGameManagerRef) self false)
              (CallFunction|HighlightDigit (Variables|Default|GethighlightedDigit)))))
        (else
          (goto _label))))))

(event EventBeginPlay
  ;[0.9115 0.6659 0.3276] Event BeginPlay
  (CallFunction|SortDigits)
  (CallFunction|FindGameManager)
  (CallFunction|FindPlayerRef)
  (CallFunction|DisableInternalItem))

(event EventINPUT:Left
  ;[1 0.7569 0.576] WASD Inputs
  (CallFunction|UpdateDigitIndex -1)
  (CallFunction|HighlightDigit (Variables|Default|GethighlightedDigit)))

(event EventINPUT:Right
  ;[1 0.7569 0.576] WASD Inputs
  (CallFunction|UpdateDigitIndex 1)
  (CallFunction|HighlightDigit (Variables|Default|GethighlightedDigit)))

(event EventINPUT:Up
  ;[1 0.7569 0.576] WASD Inputs
  (CallFunction|SpinDigit 1)
  (CallFunction|UpdateCurrentState -1 (Variables|Default|GethighlightedDigit)))

(event EventINPUT:Down
  ;[1 0.7569 0.576] WASD Inputs
  (CallFunction|SpinDigit -1)
  (CallFunction|UpdateCurrentState 1 (Variables|Default|GethighlightedDigit)))

(event EventINPUT:Escape
  ;[0.9865 0.3403 0.07518] Escape Inputs
  (CallFunction|OpenFocusGate)
  (Variables|/Game/FirstPerson/Blueprints/BP_FirstPersonCharacter.BP_FirstPersonCharacter_C|SetisFocusedOnPuzzle? (Variables|Default|GetAs%20BP%20First%20Person%20Character) false)
  (Game|Player|SetViewTargetwithBlend (Game|GetPlayerController 0) (Game|Player|GetPlayerPawn 0) (Variables|Default|Getc_ReturnSwingTime_0) "VTBlend_Linear" 0.0 false))

(fn ConstructionScript
  (bind _digits (Variables|Default|Getdigits))
  (bind _children (Components|GetChildrenComponents _digits false))
  (bind _returnvalue (Utilities|Array|Length _children))
  (Utilities|Array|Resize (Variables|Default|GetsortedDigits) _returnvalue)
  (Utilities|Array|Resize (Variables|Default|GetsuccessState) _returnvalue)
  (Utilities|Array|Resize (Variables|Default|GetcurrentState) _returnvalue))