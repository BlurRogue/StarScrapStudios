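; Level sound manager that starts and stops sounds as the player overlaps its tagged trigger boxes.
; "soundN" component tags index parallel per-sound setting arrays, which the construction script sizes to NumOfSounds.
; On overlap, it stops interruptible sounds, then plays cues in 2D, at the player, or attached to initial/final triggers or another actor.
; Trigger limits replays for most placements, while ActiveSounds tracks audio components for stopping on later triggers or exit.
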(event Custom|GetPlayerRef
  (bind _asbp_first_person_character (Utilities|Casting|CastToBP_FirstPersonCharacter (Game|GetPlayerCharacter 0)))
  (Variables|Default|SetPlayerRef _asbp_first_person_character))

(event Custom|StoptheStoppableSounds
  (for (_array_element _array_index) (Variables|Default|GetActiveSounds)
    (if (Utilities|Array|Get(acopy) (Variables|Conditions|GetstopWithOtherTriggers) _array_index)
      (Audio|Components|Audio|Stop _array_element))))

(event Custom|loop
  (params (Sound :type Integer))
  (if (!= (Utilities|Array|Get(acopy) (Variables|Conditions|GetloopAfter) Sound) 0.0)
    _
    (else
      _))
  (Utilities|FlowControl|Delay (+ (Variables|/Script/Engine.SoundBase|GetDuration (Utilities|Array|Get(acopy) (Variables|General|GetsoundCues) Sound)) 0.01))
  (bind (_array_element _array_index) (Utilities|Array|ForEachLoopwithBreak (Variables|Default|GetActiveSounds))
    (:LoopBody
      (if (== _array_index Sound)
        (if (not (Audio|Components|Audio|IsPlaying _array_element))
          (Audio|CreateSound2D "/Game/Sound/SoundWaves/Bruin_Boot.Bruin_Boot" 1.0 1.0 0.0 0))))))

(event Custom|CloseGate
  (bind _soundindex (Variables|Default|GetSoundIndex))
  (bind _soundindex_2 (Variables|Default|GetSoundIndex))
  (bind _soundindex_3 (Variables|Default|GetSoundIndex))
  (bind _soundindex_4 (Variables|Default|GetSoundIndex))
  (bind _soundindex_5 (Variables|Default|GetSoundIndex))
  (bind _soundindex_6 (Variables|Default|GetSoundIndex))
  (bind _returnvalue (- _soundindex_6 1))
  (bind _returnvalue_2 (- _soundindex 1))
  (bind _returnvalue_3 (- _soundindex_2 1))
  (bind _returnvalue_4 (- _soundindex_3 1))
  (bind _returnvalue_5 (- _soundindex_4 1))
  (bind _returnvalue_6 (- _soundindex_5 1))
  (Utilities|FlowControl|Gate false) ; enters at Close
)

(event Collision|EventActorBeginOverlap
  (params (OtherActor :type Actor%20Object%20Reference))
  (switch Utilities|FlowControl|Switch|SwitchonE_ActorType (Variables|Other|GetTriggerType)
    (:NewEnumerator1
      (bind _asbp_first_person_character (Utilities|Casting|CastToBP_FirstPersonCharacter OtherActor))
      (Variables|Default|SetPlayerRef _asbp_first_person_character)
      (Variables|Default|SetOverlapping%20Components (Class|Actor|GetOverlappingComponents _asbp_first_person_character))
      (bind _array_element (Utilities|Array|ForEachLoopwithBreak (Class|Actor|GetOverlappingComponents _asbp_first_person_character))
        (:LoopBody
          (Variables|Default|SetcomponentRef _array_element)
          (Utilities|Casting|CastToBP_SoundManager (Components|GetOwner _array_element))
          (Utilities|FlowControl|Sequence
            (:then_0
              (if (> (Utilities|Array|Length (Variables|/Script/Engine.ActorComponent|GetComponentTags _array_element)) 0)
                (CallFunction|StoptheStoppableSounds)))
            (:then_1
              (bind _array_element_2 (Utilities|Array|ForEachLoopwithBreak (Variables|/Script/Engine.ActorComponent|GetComponentTags _array_element))
                (:LoopBody
                  (Variables|Default|SetSoundIndex (Math|Conversions|ToInteger(Byte) (Utilities|String|RightChop (Utilities|String|ToString(Name) _array_element_2) 5)))
                  (Utilities|FlowControl|Gate false
                    (:Exit
                      (Utilities|FlowControl|Sequence
                        (:then_0
                          (bind (_array_element_3 _array_index) (Utilities|Array|ForEachLoopwithBreak (Variables|Default|GetActiveSounds))
                            (:LoopBody
                              (if (== _array_index (- (Variables|Default|GetSoundIndex) 1))
                                (Utilities|FlowControl|Sequence
                                  (:then_1
                                    (if (Components|ComponentHasTag (Variables|Default|GetcomponentRef) "final")
                                      (if (Audio|Components|Audio|IsPlaying _array_element_3)
                                        (if (Utilities|Array|Get(acopy) (Variables|Conditions|GetstopAtFinalTrigger) (- (Variables|Default|GetSoundIndex) 1))
                                          (Audio|Components|Audio|Stop _array_element_3)
                                          (CallFunction|CloseGate))))))))))
                        (:then_1
                          (switch Utilities|FlowControl|Switch|SwitchonE_SoundLocation (Utilities|Array|Get(acopy) (Variables|Conditions|GetsoundLocation) (Math|Conversions|ToInteger(Byte) (Utilities|String|RightChop (Utilities|String|ToString(Name) _array_element_2) 5)))
                            (:NewEnumerator0
                              (bind _trigger_ (CallFunction|Trigger?))
                              (if _trigger_
                                (bind _returnvalue (Audio|CreateSound2D (Utilities|Array|Get(acopy) (Variables|General|GetsoundCues) (- (Variables|Default|GetSoundIndex) 1)) 1.0 1.0 0.0 0 false false))
                                (Utilities|Array|SetArrayElem (Variables|Default|GetActiveSounds) (- (Variables|Default|GetSoundIndex) 1) _returnvalue)
                                (Audio|Components|Audio|Play _returnvalue (Utilities|Array|Get(acopy) (Variables|General|GetstartTime) (- (Variables|Default|GetSoundIndex) 1)))
                                (if (Utilities|Array|Get(acopy) (Variables|Conditions|Getloop?) (- (Variables|Default|GetSoundIndex) 1))
                                  (CallFunction|Loop (- (Variables|Default|GetSoundIndex) 1)))))
                            (:NewEnumerator1
                              (Audio|PlaySoundatLocation (Utilities|Array|Get(acopy) (Variables|General|GetsoundCues) (- (Variables|Default|GetSoundIndex) 1)) (Transformation|GetActorLocation (Variables|Default|GetPlayerRef)) "0, 0, 0" 1.0 1.0 (Utilities|Array|Get(acopy) (Variables|General|GetstartTime) (- (Variables|Default|GetSoundIndex) 1)) 0 0 0 0))
                            (:NewEnumerator2
                              (bind _array_element_4 (Utilities|Array|ForEachLoopwithBreak (Actor|GetComponentsbyTag self "/Script/Engine.BoxComponent" "initial") :!label _label)
                                (:LoopBody
                                  (if (Components|ComponentHasTag _array_element_4 (Utilities|String|StringToName (Utilities|String|Append "sound" (Utilities|String|ToString(Integer) (Variables|Default|GetSoundIndex)))))
                                    (bind _trigger__2 (CallFunction|Trigger?))
                                    (if _trigger__2
                                      (bind _returnvalue_2 (Audio|SpawnSoundAttached (Utilities|Array|Get(acopy) (Variables|General|GetsoundCues) (- (Variables|Default|GetSoundIndex) 1)) _array_element_4 "None" "0, 0, 0" "0, 0, 0" "KeepRelativeOffset" false 1.0 1.0 (Utilities|Array|Get(acopy) (Variables|General|GetstartTime) (- (Variables|Default|GetSoundIndex) 1)) 0 0 false))
                                      (Utilities|Array|SetArrayElem (Variables|Default|GetActiveSounds) (- (Variables|Default|GetSoundIndex) 1) _returnvalue_2)
                                      (goto _label Break))))))
                            (:NewEnumerator3
                              (bind _array_element_5 (Utilities|Array|ForEachLoopwithBreak (Actor|GetComponentsbyTag self "/Script/Engine.BoxComponent" "final") :!label _label_2)
                                (:LoopBody
                                  (if (Components|ComponentHasTag _array_element_5 (Utilities|String|StringToName (Utilities|String|Append "sound" (Utilities|String|ToString(Integer) (Variables|Default|GetSoundIndex)))))
                                    (bind _trigger__3 (CallFunction|Trigger?))
                                    (if _trigger__3
                                      (bind _returnvalue_3 (Audio|SpawnSoundAttached (Utilities|Array|Get(acopy) (Variables|General|GetsoundCues) (- (Variables|Default|GetSoundIndex) 1)) _array_element_5 "None" "0, 0, 0" "0, 0, 0" "KeepRelativeOffset" false 1.0 1.0 (Utilities|Array|Get(acopy) (Variables|General|GetstartTime) (- (Variables|Default|GetSoundIndex) 1)) 0 0 false))
                                      (Utilities|Array|SetArrayElem (Variables|Default|GetActiveSounds) (- (Variables|Default|GetSoundIndex) 1) _returnvalue_3)
                                      (goto _label_2 Break))))))
                            (:NewEnumerator4
                              (bind _trigger__4 (CallFunction|Trigger?))
                              (if _trigger__4
                                (bind _returnvalue_4 (Audio|SpawnSoundAttached (Utilities|Array|Get(acopy) (Variables|General|GetsoundCues) (- (Variables|Default|GetSoundIndex) 1)) (Variables|/Game/Actors/Interactables/ParentClass/BP_InteractibleParent.BP_InteractibleParent_C|GetStatic_Mesh (Utilities|Array|Get(acopy) (Variables|Conditions|GetactorToPlayAt))) "None" "0, 0, 0" "0, 0, 0" "KeepRelativeOffset" false 1.0 1.0 (Utilities|Array|Get(acopy) (Variables|General|GetstartTime) (- (Variables|Default|GetSoundIndex) 1)) 0 0 false))
                                (Utilities|Array|SetArrayElem (Variables|Default|GetActiveSounds) (- (Variables|Default|GetSoundIndex) 1) _returnvalue_4)))))))))))))))))

(event EventBeginPlay
  (CallFunction|GetPlayerRef))

(event Collision|EventActorEndOverlap
  (params (OtherActor :type Actor%20Object%20Reference))
  (switch Utilities|FlowControl|Switch|SwitchonE_ActorType (Variables|Other|GetTriggerType)
    (:NewEnumerator1
      (bind _array_element (Utilities|Array|ForEachLoopwithBreak (Variables|Default|GetOverlapping%20Components))
        (:LoopBody
          (Variables|Default|SetcomponentRef _array_element)
          (Utilities|Casting|CastToBP_SoundManager (Components|GetOwner _array_element))
          (Utilities|FlowControl|Sequence
            (:then_0
              (if (> (Utilities|Array|Length (Variables|/Script/Engine.ActorComponent|GetComponentTags _array_element)) 0)
                (CallFunction|StoptheStoppableSounds)))
            (:then_1
              (bind _array_element_2 (Utilities|Array|ForEachLoopwithBreak (Variables|/Script/Engine.ActorComponent|GetComponentTags _array_element))
                (:LoopBody
                  (bind _output_get (Variables|Default|SetSoundIndex (Math|Conversions|ToInteger(Byte) (Utilities|String|RightChop (Utilities|String|ToString(Name) _array_element_2) 5))))
                  (if (Utilities|Array|Get(acopy) (Variables|Conditions|GetstopWLeavingCollision?) _output_get)
                    (bind (_array_element_3 _array_index) (Utilities|Array|ForEachLoopwithBreak (Variables|Default|GetActiveSounds) :!label _label)
                      (:LoopBody
                        (if (== _array_index (Variables|Default|GetSound%20Index2))
                          (Audio|Components|Audio|Stop _array_element_3)
                          (goto _label Break))))))))))))))

(fn ConstructionScript
  (bind _numofsounds (Variables|Other|GetNumOfSounds))
  (bind _numofsounds_2 (Variables|Other|GetNumOfSounds))
  (bind _componenttags (Variables|Default|GetComponentTags))
  (Utilities|Array|Resize (Variables|General|GetSoundName) (Variables|Other|GetNumOfSounds))
  (Utilities|Array|Resize (Variables|Conditions|Getloop?) (Variables|Other|GetNumOfSounds))
  (Utilities|Array|Resize (Variables|Conditions|GetstopWLeavingCollision?) (Variables|Other|GetNumOfSounds))
  (Utilities|Array|Resize (Variables|Conditions|GetsoundLocation) (Variables|Other|GetNumOfSounds))
  (Utilities|Array|Resize (Variables|Default|GetActiveSounds) (Variables|Other|GetNumOfSounds))
  (Utilities|Array|Resize (Variables|General|GetstartTime) (Variables|Other|GetNumOfSounds))
  (Utilities|Array|Resize (Variables|Conditions|GetactorToPlayAt) (Variables|Other|GetNumOfSounds))
  (Utilities|Array|Resize (Variables|Conditions|GetstopAtFinalTrigger) (Variables|Other|GetNumOfSounds))
  (Utilities|Array|Resize (Variables|Conditions|GetstopWithOtherTriggers) (Variables|Other|GetNumOfSounds))
  (Utilities|Array|Resize (Variables|Conditions|GetisRetriggerable?) (Variables|Other|GetNumOfSounds))
  (Utilities|Array|Resize (Variables|General|GetsoundCues) _numofsounds_2)
  (Utilities|Array|Resize (Variables|General|GetsoundCue) _numofsounds_2)
  (Utilities|Array|Resize (Variables|General|GetinitialTrigger) (Variables|Other|GetNumOfSounds))
  (Utilities|Array|Resize (Variables|General|GetfinalTrigger) (Variables|Other|GetNumOfSounds))
  (Utilities|Array|Resize _componenttags (Variables|Other|GetNumOfSounds))
  (Utilities|FlowControl|Sequence
    (:then_0
      (Utilities|Array|Resize (Variables|Default|Gettriggered?) _numofsounds)
      (Utilities|Array|Resize (Variables|Conditions|GetloopAfter) _numofsounds))
    (:then_1
      (for (_ _array_index) _componenttags
        (Utilities|Array|SetArrayElem _componenttags _array_index (Utilities|String|StringToName (Utilities|String|Append "sound" (Utilities|String|ToString(Integer) (+ _array_index 1)))))))))

(fn Trigger?
  (bind _triggered_ (Variables|Default|Gettriggered?))
  (bind _soundindex (Variables|Default|GetSoundIndex))
  (bind _returnvalue (- _soundindex 1))
  (if (< _returnvalue 0)
    (return false)
    (elif (Utilities|Array|Get(acopy) _triggered_ _returnvalue)
      (if (Utilities|Array|Get(acopy) (Variables|Conditions|GetisRetriggerable?) (- _soundindex 1))
        (return true)
        (else
          (return false)))
      (else
        (Utilities|Array|SetArrayElem _triggered_ 0 true)
        (return true)))))