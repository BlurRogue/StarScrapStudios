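; Base class for interactable actors that feed the player's interaction wheel UI and can be highlighted.
; A looping timer finds BP_gameManager, which is told to add the actor when the player enters InteractTrigger and remove it on exit or interaction.
; ToggleHighlight drives the mesh's custom depth rendering while IsInteractable is set, and leaving the trigger switches it off.
; Helper functions convert between grid X/Y coordinates and array indices.
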(event OnComponentBeginOverlap(InteractTrigger)
  (params (OverlappedComponent :type Primitive%20Component%20Object%20Reference) (OtherActor :type Actor%20Object%20Reference) (OtherComp :type Primitive%20Component%20Object%20Reference) (OtherBodyIndex :type Integer) (bFromSweep :type Boolean) (SweepResult :type Hit%20Result%20Structure%20%28by%20ref%29))
  ;[1 0.8403 0.1586] User Interface for RE Interaction Wheel
  (Utilities|Casting|CastToBP_FirstPersonCharacter OtherActor)
  (Default|FInteractabletoUI (Variables|Default|GetGameManagerRef) self true))

(event OnComponentEndOverlap(InteractTrigger)
  (params (OverlappedComponent :type Primitive%20Component%20Object%20Reference) (OtherActor :type Actor%20Object%20Reference) (OtherComp :type Primitive%20Component%20Object%20Reference) (OtherBodyIndex :type Integer))
  ;[1 0.8403 0.1586] User Interface for RE Interaction Wheel
  (Utilities|Casting|CastToBP_FirstPersonCharacter OtherActor)
  (Default|FInteractabletoUI (Variables|Default|GetGameManagerRef) self false)
  (CallFunction|ToggleHighlight "NewEnumerator2"))

(event Custom|Interact
  (params (Component :type Actor%20Component%20Object%20Reference))
  ;[0 0.2959 0.5365] Interact
  (Default|FInteractabletoUI (Variables|Default|GetGameManagerRef) self false))

(event Custom|ToggleHighlight
  (params (toggleEnum :type E_toggle%20Enum :default "NewEnumerator0"))
  ;[1 0.8392 0.4018] Toggle Highlight
  (if (Variables|Default|GetisInteractable)
    (switch Utilities|FlowControl|Switch|SwitchonE_toggle toggleEnum
      (:NewEnumerator0
        (if (not (Variables|Default|GethighlightActive))
          ;;[0.07443 0.15 0.07585 0.5] Turning on Highlight
          (Rendering|SetRenderCustomDepth (Variables|Default|GetStatic_Mesh) true :!label _label)
          (Variables|Default|SethighlightActive true)))
      (:NewEnumerator1
        (goto _label))
      (:NewEnumerator2
        ;;[0.15 0.06655 0.06804 0.5] Turning Off Highlight
        (Rendering|SetRenderCustomDepth (Variables|Default|GetStatic_Mesh) false)
        (Variables|Default|SethighlightActive false)))))

(event Custom|FindGameManager
  ;[1 0.6329 0.2448] Event BeginPlay
  ;;[1 0.8828 0.5312] Find the Game Manager
  (bind _returnvalue (Utilities|Time|SetTimerbyEvent (delegate Custom|getGameManager) (Variables|Default|GeteventTimer) true true 0.1))
  (Variables|Default|SetgetGameManagerEvent _returnvalue))

(event Custom|getGameManager
  (bind _getgamemanagerevent (Variables|Default|GetgetGameManagerEvent))
  ;[1 0.6329 0.2448] Event BeginPlay
  ;;[1 0.8828 0.5312] Find the Game Manager
  (bind _outactors (Actor|GetAllActorsOfClass "/Game/SaveGame/BP_gameManager.BP_gameManager_C"))
  (bind _array_element (Utilities|Array|ForEachLoopwithBreak _outactors :!label _label)
    (:LoopBody
      (Variables|Default|SetGameManagerRef _array_element)
      (if (Utilities|Time|IsValidTimerHandle _getgamemanagerevent)
        (Utilities|Time|ClearandInvalidateTimerbyHandle _getgamemanagerevent)
        (goto _label Break)))))

(event Custom|debugTags
  (Variables|Default|SetdebugString "")
  (bind _array_element (Utilities|Array|ForEachLoopwithBreak (Variables|Actor|GetTags))
    (:LoopBody
      (Development|PrintString (Utilities|String|Append (Variables|Default|GetdebugString) ", " (Utilities|String|ToString(Name) _array_element))))))

(event EventBeginPlay
  ;[1 0.6329 0.2448] Event BeginPlay
  (Utilities|FlowControl|Sequence
    (:then_0
      (bind _asbp_first_person_character (Utilities|Casting|CastToBP_FirstPersonCharacter (Game|GetPlayerCharacter 0)))
      (Variables|Other|SetAs%20BP%20First%20Person%20Character _asbp_first_person_character))
    (:then_1
      (CallFunction|FindGameManager))))

(fn ConstructionScript)

(fn ConvertXandYtoArrayValue
  (params (X :type Integer) (Y :type Integer) (Width :type Integer) (Height :type Integer))
  (return (+ (- (Math|Integer|%(Integer) X (+ Width 1)) 1) (+ (* (- Y 1) Width) 1))))

(fn ConvertArrayValuetoXandY
  (params (Array%20Input :type Integer) (Width :type Integer) (Height :type Integer))
  (LocalVariables|SetY%20Output 1)
  (LocalVariables|SetChanging%20Value Array%20Input)
  (while (> (LocalVariables|GetChanging%20Value) Width)
    (LocalVariables|SetChanging%20Value (- (LocalVariables|GetChanging%20Value) Width))
    (LocalVariables|SetY%20Output (+ (LocalVariables|GetY%20Output) 1)))
  (return (Math|Integer|%(Integer) Array%20Input Width) (LocalVariables|GetY%20Output)))