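; Base actor for interactable objects, providing empty Interact, Shot and InteractV2 (with hit component) events, presumably for child Blueprints to override.
; On BeginPlay it caches the player's BP_FirstPersonCharacter.
; It also carries helper functions that convert between 1-based X/Y grid coordinates and a flat array value for a given width.
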(event Custom|Interact)

(event Custom|Shot)

(event Custom|InteractV2
  (params (componentHit :type Primitive%20Component%20Object%20Reference)))

(event EventBeginPlay
  (bind _asbp_first_person_character (Utilities|Casting|CastToBP_FirstPersonCharacter (Game|GetPlayerCharacter 0)))
  (Variables|Default|SetAs%20BP%20First%20Person%20Character _asbp_first_person_character))

(event Collision|EventActorBeginOverlap
  (params (OtherActor :type Actor%20Object%20Reference)))

(event EventTick
  (params (DeltaSeconds :type Float%20%28single-precision%29)))

(fn ConstructionScript)

(fn ConvertXandYtoArrayValue
  (params (X :type Integer) (Y :type Integer) (Width :type Integer) (Height :type Integer))
  (return (+ (- (Math|Integer|%(Integer) X (+ Width 1)) 1) (+ (* (- Y 1) Width) 1))))

(fn ConvertArrayValuetoXandY
  (params (Array%20Input :type Integer) (Width :type Integer) (Height :type Integer))
  (LocalVariables|SetY%20Output 1)
  (LocalVariables|SetChanging%20Value Array%20Input)
  (while (> (LocalVariables|GetChanging%20Value) Width)
    (LocalVariables|SetChanging%20Value (- (LocalVariables|GetChanging%20Value) Width))
    (LocalVariables|SetY%20Output (+ (LocalVariables|GetY%20Output) 1)))
  (return (Math|Integer|%(Integer) Array%20Input Width) (LocalVariables|GetY%20Output)))