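; BP_Item is an interactable pickup actor for items and clues, configured in the editor by an item type enum.
; The construction script resets fields or imports them from the DT_itemID data table using the enum name as row name, then applies the DefaultSounds choice.
; Interacting plays a default or custom sound, records entries flagged both item and clue on the player, and removes items or clues via the GameManager UI call and destruction.
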(event Custom|PlayInteractSound
  ;[0.04436 1 0.3933] Play Interact Sound
  (if (Variables|ItemIdentification|GetisItem)
    (if (Variables|ItemIdentification|GetisClue)
      (Utilities|Array|Add (Variables|/Game/FirstPerson/Blueprints/BP_FirstPersonCharacter.BP_FirstPersonCharacter_C|GetClues (Variables|Default|GetAs%20BP%20First%20Person%20Character)) 0)))
  (if (Variables|Default|GetuseDefaultInteractionSounds)
    (if (Variables|ItemIdentification|GetisItem)
      (Audio|PlaySoundatLocation "/Game/Assets/Audio/Interaction/SC_itemPickup1.SC_itemPickup1" (Transformation|GetActorLocation self) "0, 0, 0" 1.0 1.0 0.0 0 0 0 0)
      (else
        (Audio|PlaySoundatLocation "/Game/Assets/Audio/Interaction/SC_ActionSuccess.SC_ActionSuccess" (Transformation|GetActorLocation self) "0, 0, 0" 1.0 1.0 0.0 0 0 0 0)))
    (elif (Utilities|IsValid (Variables|Default|GetinteractSound))
      (Audio|PlaySoundatLocation (Variables|Default|GetinteractSound) (Transformation|GetActorLocation self) "0, 0, 0" 1.0 1.0 0.0 0 0 0 0)
      (elif (Variables|/Game/FirstPerson/Blueprints/BP_FirstPersonCharacter.BP_FirstPersonCharacter_C|GetDebugMode (Variables|Default|GetAs%20BP%20First%20Person%20Character))
        (Development|PrintString "Error: Sound Cue Not Valid")))))

(event EventInteract
  (params (Component :type Actor%20Component%20Object%20Reference))
  ;[1 0.6883 0.114] Interact
  (CallFunction|PlayInteractSound)
  (if (or (Variables|ItemIdentification|GetisItem) (Variables|ItemIdentification|GetisClue))
    (Default|FInteractabletoUI (Variables|Default|GetGameManagerRef) self false)
    (Actor|DestroyActor)))

(fn ConstructionScript
  (|CallParentFunction)
  (Transformation|SetWorldScale3D (Variables|Default|GetStaticMesh) (Variables|Default|GetMeshScale))
  (Components|StaticMesh|SetStaticMesh (Variables|Default|GetStaticMesh) (Variables|Default|GetitemMesh))
  (Utilities|FlowControl|Sequence
    (:then_0
      (switch Utilities|FlowControl|Switch|SwitchonE_itemID (Variables|ItemIdentification|GetitemTypes)
        (:NewEnumerator4
          (Variables|Default|SetdisplayName "")
          (Variables|Default|SetdisplayDescription "")
          (Variables|Default|SetisInteractable true)
          ;[0.15 0.15 0.15 0.5] Resetting Values to Defaults
          (Variables|ItemIdentification|SetisItem false)
          (Variables|ItemIdentification|SetisClue false)
          (Variables|Default|SetItemValue 0)
          (Variables|Default|SetItemCount 1)
          (Variables|Default|SetuseDefaultInteractionSounds true)
          (Variables|Default|SetitemMesh (Variables|Default|GetdefaultMesh))
          (Variables|Default|SetItemWidget 0)
          (Variables|Default|SetinteractSound "/Game/Assets/Audio/Interaction/SC_itemPickup1.SC_itemPickup1")
          (Variables|Default|SetInvUseAudio 0)
          (Variables|Default|SetCanUseFromInventory false)
          (Variables|Default|SetMeshScale (Math|Vector|MakeVector 1.0 1.0 1.0))
          (Variables|ItemIdentification|SetitemTypes "NewEnumerator0"))
        (:NewEnumerator0
          _)
        (:NewEnumerator3
          _)
        (:NewEnumerator1
          _)
        (:NewEnumerator2
          _))
      (if (not (or (Utilities|Enum|Equal(Enum) (Utilities|String|EnumtoString (Variables|ItemIdentification|GetitemTypes)) "Unassigned") (Utilities|Enum|Equal(Enum) (Utilities|String|EnumtoString (Variables|ItemIdentification|GetitemTypes)) "Custom")))
        ;[0.15 0.15 0.15 0.5] Importing Data
        (bind _returnvalue (Utilities|GetDataTableRow "/Game/Actors/Interactables/Background/DT_itemID.DT_itemID" (Utilities|String|StringToName (Utilities|String|EnumtoString (Variables|ItemIdentification|GetitemTypes))))
          (:then
            ;[0.15 0.15 0.15 0.5] Setting Default Values
            (Variables|Default|SetdisplayName (.displayName (Utilities|Struct|BreakS_itemIDs _returnvalue)))
            (Variables|Default|SetdisplayDescription (.displayDescription (Utilities|Struct|BreakS_itemIDs _returnvalue)))
            (Variables|Default|SetisInteractable (.isInteractable (Utilities|Struct|BreakS_itemIDs _returnvalue)))
            (Variables|ItemIdentification|SetisItem (.isItem (Utilities|Struct|BreakS_itemIDs _returnvalue)))
            (Variables|ItemIdentification|SetisClue (.isClue (Utilities|Struct|BreakS_itemIDs _returnvalue)))
            (Variables|Default|SetItemValue (.ScrapValue (Utilities|Struct|BreakS_itemIDs _returnvalue)))
            (Variables|Default|SetItemCount (.ItemCount (Utilities|Struct|BreakS_itemIDs _returnvalue)))
            (Variables|Default|SetuseDefaultInteractionSounds (.useDefaultInteractionAudio (Utilities|Struct|BreakS_itemIDs _returnvalue)))
            (Variables|Default|SetitemMesh (.BaseMesh (Utilities|Struct|BreakS_itemIDs _returnvalue)))
            (Variables|Default|SetItemWidget (.itemWidget (Utilities|Struct|BreakS_itemIDs _returnvalue)))
            (Variables|Default|SetinteractSound (.interactAudio (Utilities|Struct|BreakS_itemIDs _returnvalue)))
            (Variables|Default|SetInvUseAudio (.InvUseAudio (Utilities|Struct|BreakS_itemIDs _returnvalue)))
            (Variables|Default|SetCanUseFromInventory (.canUseFromInventory (Utilities|Struct|BreakS_itemIDs _returnvalue)))
            (Variables|Default|SetMeshScale (.Scale (Utilities|Struct|BreakS_itemIDs _returnvalue)))))))
    (:then_1
      ;[0.15 0.15 0.15 0.5] Comment
      ;;[0.15 0.15 0.15 0.5] Setting Sounds
      (switch Utilities|FlowControl|Switch|SwitchonE_DefaultInteractSounds (Variables|Default|GetDefaultSounds)
        (:NewEnumerator0
          (Variables|Default|SetinteractSound "/Game/Assets/Audio/Interaction/SC_itemPickup1.SC_itemPickup1"))
        (:NewEnumerator1
          (Variables|Default|SetinteractSound "/Game/Assets/Audio/Interaction/SC_itemPickup2.SC_itemPickup2"))
        (:NewEnumerator2
          (Variables|Default|SetinteractSound "/Game/Assets/Audio/Interaction/SC_ActionSuccess.SC_ActionSuccess"))
        (:NewEnumerator3
          (Variables|Default|SetinteractSound "/Game/Assets/Audio/Interaction/SC_PlugInsert.SC_PlugInsert"))))))

(fn RunConstructionErrorChecker)