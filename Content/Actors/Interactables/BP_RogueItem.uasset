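; Interactable item actor for pickups and clues, configured in the editor from an item-type preset.
; The Construction Script applies mesh and scale, picks a sound preset, then imports item data from DT_itemID using the enum name as row name, with a RESET VALUES option restoring defaults.
; Interact records clues on the player character, plays a sound and destroys items or clues.
; A debug checker for missing item data exists but is unwired.
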(event Custom|PlayInteractSound
  (if (Variables|General|GetisItem)
    (if (Variables|General|GetisClue)
      (Utilities|Array|Add (Variables|/Game/FirstPerson/Blueprints/BP_FirstPersonCharacter.BP_FirstPersonCharacter_C|GetClues (Variables|Default|GetAs%20BP%20First%20Person%20Character)) 0)))
  (if (Variables|Audio|GetuseDefaultInteractionSounds)
    (if (Variables|General|GetisItem)
      (Audio|PlaySoundatLocation "/Game/Assets/Audio/Interaction/SC_itemPickup1.SC_itemPickup1" (Transformation|GetActorLocation self) "0, 0, 0" 1.0 1.0 0.0 0 0 0 0)
      (else
        (Audio|PlaySoundatLocation "/Game/Assets/Audio/Interaction/SC_ActionSuccess.SC_ActionSuccess" (Transformation|GetActorLocation self) "0, 0, 0" 1.0 1.0 0.0 0 0 0 0)))
    (elif (Utilities|IsValid (Variables|Audio|GetinteractSound))
      (Audio|PlaySoundatLocation (Variables|Audio|GetinteractSound) (Transformation|GetActorLocation self) "0, 0, 0" 1.0 1.0 0.0 0 0 0 0)
      (elif (Variables|/Game/FirstPerson/Blueprints/BP_FirstPersonCharacter.BP_FirstPersonCharacter_C|GetDebugMode (Variables|Default|GetAs%20BP%20First%20Person%20Character))
        (Development|PrintString "Error: Sound Cue Not Valid")))))

(event Collision|EventActorBeginOverlap
  (params (OtherActor :type Actor%20Object%20Reference)))

(event EventTick
  (params (DeltaSeconds :type Float%20%28single-precision%29)))

(event EventInteract
  (CallFunction|PlayInteractSound)
  (if (or (Variables|General|GetisItem) (Variables|General|GetisClue))
    (Actor|DestroyActor)))

(event EventBeginPlay)

(fn ConstructionScript
  (|CallParentFunction)
  (Transformation|SetWorldScale3D (Variables|Default|GetStaticMesh) (Variables|Default|GetMeshScale))
  (Components|StaticMesh|SetStaticMesh (Variables|Default|GetStaticMesh) (Variables|General|GetBaseMesh))
  ;[0.15 0.15 0.15 0.5] Comment
  ;;[0.15 0.15 0.15 0.5] Setting Sounds
  (switch Utilities|FlowControl|Switch|SwitchonE_DefaultInteractSounds (Variables|Audio|GetDefaultSounds)
    (:NewEnumerator4
      _)
    (:NewEnumerator0
      (Variables|Audio|SetinteractSound "/Game/Assets/Audio/Interaction/SC_itemPickup1.SC_itemPickup1"))
    (:NewEnumerator1
      (Variables|Audio|SetinteractSound "/Game/Assets/Audio/Interaction/SC_itemPickup2.SC_itemPickup2"))
    (:NewEnumerator2
      (Variables|Audio|SetinteractSound "/Game/Assets/Audio/Interaction/SC_ActionSuccess.SC_ActionSuccess"))
    (:NewEnumerator3
      (Variables|Audio|SetinteractSound "/Game/Assets/Audio/Interaction/SC_PlugInsert.SC_PlugInsert")))
  (switch Utilities|FlowControl|Switch|SwitchonE_itemID (Variables|ItemIdentification|GetitemTypes)
    (:NewEnumerator4
      (Variables|ItemIdentification|SetclearItemData true)
      (if (Variables|ItemIdentification|GetclearItemData)
        ;[0.15 0.15 0.15 0.5] Resetting Values to Defaults
        (Variables|ItemIdentification|SetItem_ID "")
        (Variables|General|SetisItem false)
        (Variables|General|SetisClue false)
        (Variables|itemInfo|SetScrapValue 0)
        (Variables|itemInfo|SetItemCount 1)
        (Variables|Audio|SetuseDefaultInteractionSounds true)
        (Variables|General|SetBaseMesh (Variables|Default|GetdefaultMesh))
        (Variables|General|SetItemWidget 0)
        (Variables|itemInfo|SetItemDescription (Utilities|Text|ToText(String) "This is a description of the item or clue"))
        (Variables|Audio|SetinteractSound "/Game/Assets/Audio/Interaction/SC_itemPickup1.SC_itemPickup1")
        (Variables|Audio|SetInvUseAudio 0)
        (Variables|itemInfo|SetCanUseFromInventory false)
        (Variables|Default|SetMeshScale (Math|Vector|MakeVector 1.0 1.0 1.0))
        (Variables|ItemIdentification|SetclearItemData false)
        (Variables|ItemIdentification|SetitemTypes "NewEnumerator0")
        (if (not (or (Utilities|Enum|Equal(Enum) (Utilities|String|EnumtoString (Variables|ItemIdentification|GetitemTypes)) "Unassigned") (Utilities|Enum|Equal(Enum) (Utilities|String|EnumtoString (Variables|ItemIdentification|GetitemTypes)) "Custom"))) :!label _label
          ;[0.15 0.15 0.15 0.5] Importing Data
          (bind _returnvalue (Utilities|GetDataTableRow "/Game/DT_itemID.DT_itemID" (Utilities|String|StringToName (Utilities|String|EnumtoString (Variables|ItemIdentification|GetitemTypes))))
            (:then
              ;[0.15 0.15 0.15 0.5] Setting Default Values
              (Variables|ItemIdentification|SetItem_ID (.itemID (Utilities|Struct|BreakS_itemIDs _returnvalue)))
              (Variables|General|SetisItem (.isItem (Utilities|Struct|BreakS_itemIDs _returnvalue)))
              (Variables|General|SetisClue (.isClue (Utilities|Struct|BreakS_itemIDs _returnvalue)))
              (Variables|itemInfo|SetScrapValue (.ScrapValue (Utilities|Struct|BreakS_itemIDs _returnvalue)))
              (Variables|itemInfo|SetItemCount (.ItemCount (Utilities|Struct|BreakS_itemIDs _returnvalue)))
              (Variables|Audio|SetuseDefaultInteractionSounds (.useDefaultInteractionAudio (Utilities|Struct|BreakS_itemIDs _returnvalue)))
              (Variables|General|SetBaseMesh (.BaseMesh (Utilities|Struct|BreakS_itemIDs _returnvalue)))
              (Variables|General|SetItemWidget (.itemWidget (Utilities|Struct|BreakS_itemIDs _returnvalue)))
              (Variables|itemInfo|SetItemDescription (Utilities|Text|ToText(String) (.ItemDescription (Utilities|Struct|BreakS_itemIDs _returnvalue))))
              (Variables|Audio|SetinteractSound (.interactAudio (Utilities|Struct|BreakS_itemIDs _returnvalue)))
              (Variables|Audio|SetInvUseAudio (.InvUseAudio (Utilities|Struct|BreakS_itemIDs _returnvalue)))
              (Variables|itemInfo|SetCanUseFromInventory (.canUseFromInventory (Utilities|Struct|BreakS_itemIDs _returnvalue)))
              (Variables|Default|SetMeshScale (.Scale (Utilities|Struct|BreakS_itemIDs _returnvalue))))))))
    (:NewEnumerator0
      (goto _label))
    (:NewEnumerator3
      (goto _label))
    (:NewEnumerator1
      (goto _label))
    (:NewEnumerator2
      (goto _label))))

(fn RunConstructionErrorChecker
  (if (Variables|/Game/FirstPerson/Blueprints/BP_FirstPersonCharacter.BP_FirstPersonCharacter_C|GetDebugMode (Variables|Default|GetAs%20BP%20First%20Person%20Character))
    (if (Variables|General|GetisItem)
      (if (Utilities|Enum|Equal(Enum) (Variables|itemInfo|GetItemDescription) (Utilities|Text|ToText(String) (Utilities|String|Append "This is a description of the item or clue" "")))
        (Development|PrintString (Utilities|String|Append "Error: Item [" (Utilities|GetObjectName self) "] is missing it's item description")))
      (if (not (Variables|General|GetisClue))
        (if (<= (Variables|itemInfo|GetScrapValue) 0)
          (Development|PrintString (Utilities|String|Append "Error: Item [" (Utilities|GetObjectName self) "has an unassigned or invalid scrap value [" (Utilities|String|ToString(Integer) (Variables|itemInfo|GetScrapValue)) "].")))))))