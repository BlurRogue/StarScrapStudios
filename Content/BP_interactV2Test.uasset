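; BP_interactV2Test is a test actor for the InteractV2 interaction event, printing which of its components was hit.
; InteractV2 takes the hit component and parses a one-character number at index 10 of its first component tag.
; That number, minus one, picks a MultiGate output that prints a Sphere or Cube message, and the gate resets after each print.
; The older Interact event is left empty.
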(event EventBeginPlay
  (|CallParentFunction) ; This node is disabled and will not be called.\nDrag off pins to build functionality.
)

(event Collision|EventActorBeginOverlap
  (params (OtherActor :type Actor%20Object%20Reference))
  (|CallParentFunction OtherActor) ; This node is disabled and will not be called.\nDrag off pins to build functionality.
)

(event EventTick
  (params (DeltaSeconds :type Float%20%28single-precision%29))
  (|CallParentFunction DeltaSeconds) ; This node is disabled and will not be called.\nDrag off pins to build functionality.
)

(event EventInteract)

(event EventInteractV2
  (params (componentHit :type Primitive%20Component%20Object%20Reference))
  (bind _componenttags (Variables|/Script/Engine.ActorComponent|GetComponentTags componentHit))
  ;[1 1 1 0.5] Interaction V2
  (if (Utilities|IsValid componentHit)
    (if (> (Utilities|Array|Length _componenttags) 0)
      (Utilities|FlowControl|MultiGate false false (- (Math|Conversions|ToInteger(Byte) (Utilities|String|GetSubstring (Utilities|String|ToString(Name) (Utilities|Array|Get(acopy) _componenttags)) 10)) 1) :!label _label
        (:Out%200
          (Development|PrintString "Hit the Sphere!")
          (goto _label Reset))
        (:Out%201
          (Development|PrintString "Hit the Cube!")
          (goto _label Reset))))))

(fn ConstructionScript
  (|CallParentFunction))