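; BP_DoorBase is a configurable double-door actor with optional casing and locks, built in the construction script with no runtime logic.
; DoorID selects a preset row from DT_DoorIDs, keeps values as set for Unassigned or Custom, or resets them via RESET VALUES.
; These values drive meshes, door spacing, lock transforms and the lock-light material per LockStatus.
; LocationLock pins the root to its stored location, while the height-offset move is disconnected.
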(event Collision|EventActorBeginOverlap
  (params (OtherActor :type Actor%20Object%20Reference))
  (|CallParentFunction OtherActor) ; This node is disabled and will not be called.\nDrag off pins to build functionality.
)

(event EventTick
  (params (DeltaSeconds :type Float%20%28single-precision%29))
  (|CallParentFunction DeltaSeconds) ; This node is disabled and will not be called.\nDrag off pins to build functionality.
)

(event EventBeginPlay)

(fn ConstructionScript
  (bind _leftdoor (Variables|Default|GetLeftDoor))
  (bind _rightdoor (Variables|Default|GetRightDoor))
  (bind _relativelocation (Variables|/Script/Engine.SceneComponent|GetRelativeLocation _rightdoor))
  (bind _relativelocation_2 (Variables|/Script/Engine.SceneComponent|GetRelativeLocation _leftdoor))
  ;[0.15 0.15 0.15 0.5] Begin Construction Script
  (|CallParentFunction)
  (switch Utilities|FlowControl|Switch|SwitchonE_DoorIDs (Variables|Default|GetDoorID)
    (:NewEnumerator0
      (Variables|Default|SetDoorID "NewEnumerator1")
      (Variables|Assets|SethasCasing? false)
      (Variables|Assets|SetLeftDoorAsset "/Game/Assets/TutorialLevel/Doors/Narrow/Assets/Door_Narrow_L.Door_Narrow_L")
      (Variables|Spacial|SetL_DoorDistanceInt 0)
      (Variables|Spacial|SetL_DoorDistanceFloat 0.0)
      (Variables|Spacial|SetL_DoorSpacing 0.0)
      (Variables|Assets|SetRightDoorAsset "/Game/Assets/TutorialLevel/Doors/Narrow/Assets/Door_Narrow_R.Door_Narrow_R")
      (Variables|Spacial|SetR_DoorDistanceInt 0)
      (Variables|Spacial|SetR_DoorDistanceFloat 0.0)
      (Variables|Spacial|SetR_DoorSpacing 0.0)
      (Variables|Assets|SetDoorCasingAsset 0)
      (Variables|DoorLock|SetLockStatus "NewEnumerator0")
      (Variables|DoorLock|SetNonNativeLockRef 0)
      (Variables|DoorLock|SethasNativeLock? true)
      (Variables|DoorLock|SetlockAssets "/Game/Actors/DoorLock/Door_Lock.Door_Lock")
      (Variables|DoorLock|Setlock1RelTrans (Variables|Default|Getlock1DefTrans))
      (Variables|DoorLock|Setlock2RelTrans (Variables|Default|Getlock2DefTrans))
      (Variables|DoorLock|SethasLock? false)
      (Variables|Default|Setoffset_Height 0.0)
      (Variables|Default|SetHasInitialTransform false)
      (Variables|Default|SetCurrentTransform "")
      (Variables|Default|SetInitialTransform "")
      (Variables|Default|SetLocationLock false))
    (:NewEnumerator1
      _)
    (:NewEnumerator2
      _)
    (:NewEnumerator3
      _)
    (:NewEnumerator6
      _)
    (:NewEnumerator4
      _)
    (:NewEnumerator7
      _))
  (if (or (Utilities|Enum|Equal(Enum) (Utilities|String|EnumtoString (Variables|Default|GetDoorID)) "Unassigned") (Utilities|Enum|Equal(Enum) (Utilities|String|EnumtoString (Variables|Default|GetDoorID)) "Custom"))
    _
    (else
      (bind _returnvalue (Utilities|GetDataTableRow "/Game/DT_DoorIDs.DT_DoorIDs" (Utilities|String|StringToName (Utilities|String|EnumtoString (Variables|Default|GetDoorID))))
        (:then
          (Variables|Assets|SethasCasing? (.hasCasing? (Utilities|Struct|BreakS_DoorIDs _returnvalue)))
          (Variables|Assets|SetLeftDoorAsset (.LeftDoorAsset (Utilities|Struct|BreakS_DoorIDs _returnvalue)))
          (Variables|Spacial|SetL_DoorDistanceInt (.L_DoorDistanceInt (Utilities|Struct|BreakS_DoorIDs _returnvalue)))
          (Variables|Spacial|SetL_DoorDistanceFloat (.L_DoorDistanceFloat (Utilities|Struct|BreakS_DoorIDs _returnvalue)))
          (Variables|Spacial|SetL_DoorSpacing (.L_DoorSpacing (Utilities|Struct|BreakS_DoorIDs _returnvalue)))
          (Variables|Assets|SetRightDoorAsset (.RightDoorAsset (Utilities|Struct|BreakS_DoorIDs _returnvalue)))
          (Variables|Spacial|SetR_DoorDistanceInt (.R_DoorDistanceInt (Utilities|Struct|BreakS_DoorIDs _returnvalue)))
          (Variables|Spacial|SetR_DoorDistanceFloat (.R_DoorDistanceFloat (Utilities|Struct|BreakS_DoorIDs _returnvalue)))
          (Variables|Spacial|SetR_DoorSpacing (.R_DoorSpacing (Utilities|Struct|BreakS_DoorIDs _returnvalue)))
          (Variables|Assets|SetDoorCasingAsset (.DoorCasingAsset (Utilities|Struct|BreakS_DoorIDs _returnvalue)))
          (Variables|DoorLock|SetLockStatus "NewEnumerator0")
          (Variables|DoorLock|SetNonNativeLockRef 0)
          (Variables|DoorLock|SethasNativeLock? (.hasNativeLock? (Utilities|Struct|BreakS_DoorIDs _returnvalue)))
          (Variables|DoorLock|SetlockAssets (.lockAsset (Utilities|Struct|BreakS_DoorIDs _returnvalue)))
          (Variables|DoorLock|Setlock1RelTrans (.lock1RelTrans (Utilities|Struct|BreakS_DoorIDs _returnvalue)))
          (Variables|DoorLock|Setlock2RelTrans (.lock2RelTrans (Utilities|Struct|BreakS_DoorIDs _returnvalue)))
          (Variables|DoorLock|SethasLock? (.hasLock? (Utilities|Struct|BreakS_DoorIDs _returnvalue)))
          (Variables|Default|Setoffset_Height (.offset_Height (Utilities|Struct|BreakS_DoorIDs _returnvalue)))
          (Variables|Default|SetHasInitialTransform false)
          (Variables|Default|SetCurrentTransform "")
          (Variables|Default|SetInitialTransform "")
          (Variables|Default|SetLocationLock false)))))
  (switch Utilities|FlowControl|Switch|SwitchonE_DoorLockType (Variables|DoorLock|GetLockStatus)
    (:NewEnumerator0
      (Rendering|Material|SetMaterial (Variables|Default|GetDoorLock1) 2 "/Game/Actors/DoorLock/Door_Lock_Light0.Door_Lock_Light0"))
    (:NewEnumerator1
      (Rendering|Material|SetMaterial (Variables|Default|GetDoorLock1) 2 "/Game/Actors/DoorLock/Door_Lock_Light1.Door_Lock_Light1"))
    (:NewEnumerator2
      (Rendering|Material|SetMaterial (Variables|Default|GetDoorLock1) 2 "/Game/Actors/DoorLock/Door_Lock_Light2.Door_Lock_Light2")))
  ;[1 1 1 0.5] Location Lock Functionality
  (if (Variables|Default|GetLocationLock)
    ;;[1 1 1 0.5] Enforcing Location Lock
    (if (Variables|Default|GetHasInitialTransform)
      _
      (else
        (Variables|Default|SetInitialTransform (Transformation|GetWorldTransform (Variables|Default|GetDefaultSceneRoot)))
        (Variables|Default|SetHasInitialTransform true)))
    (Transformation|SetWorldLocation (Variables|Default|GetDefaultSceneRoot) (Math|Vector|MakeVector (.x (.location (Variables|Default|GetInitialTransform))) (.y (.location (Variables|Default|GetInitialTransform))) (.z (.location (Variables|Default|GetInitialTransform)))) false false)
    (else
      ;;[1 1 1 0.5] Error Handling for Location Lock
      (if (!= (Variables|Default|Getoffset_Height) 0.0)
        (Variables|Default|Setoffset_Height 0.0)
        (Development|PrintString "LOCATION LOCK NOT ACTIVE. RESETTING HEIGHT OFFSET"))))
  ;[1 1 1 0.5] Setting the Door Meshes
  (Components|StaticMesh|SetStaticMesh (Variables|Default|GetLeftDoor) (Variables|Assets|GetLeftDoorAsset))
  (Components|StaticMesh|SetStaticMesh (Variables|Default|GetRightDoor) (Variables|Assets|GetRightDoorAsset))
  (if (Variables|Assets|GethasCasing?)
    (Components|StaticMesh|SetStaticMesh (Variables|Default|GetDoor_Casing) (Variables|Assets|GetDoorCasingAsset)))
  (if (Variables|DoorLock|GethasLock?)
    (Components|StaticMesh|SetStaticMesh (Variables|Default|GetDoorLock1) (Variables|DoorLock|GetlockAssets))
    (Components|StaticMesh|SetStaticMesh (Variables|Default|GetDoorLock2) (Variables|DoorLock|GetlockAssets)))
  ;[1 1 1 0.5] Adjusting Door Spacing
  (Transformation|SetRelativeLocation _leftdoor (Math|Vector|MakeVector (+ (.x _relativelocation_2) (Variables|Spacial|GetL_DoorSpacing)) (+ (.y _relativelocation_2) (Variables|Spacial|GetL_DoorDistanceInt) 0.0) (.z _relativelocation_2)) false false)
  (Transformation|SetRelativeLocation _rightdoor (Math|Vector|MakeVector (+ (.x _relativelocation) (Variables|Spacial|GetR_DoorSpacing)) (Utilities|Operators|Subtract (.y _relativelocation) (Variables|Spacial|GetR_DoorDistanceInt) (Variables|Spacial|GetR_DoorDistanceFloat)) (.z _relativelocation)) false false)
  (Transformation|SetRelativeTransform (Variables|Default|GetDoorLock1) (Variables|DoorLock|Getlock1RelTrans) false false)
  (Transformation|SetRelativeTransform (Variables|Default|GetDoorLock2) (Variables|DoorLock|Getlock2RelTrans) false false))