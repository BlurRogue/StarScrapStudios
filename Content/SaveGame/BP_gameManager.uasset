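; Game manager that creates the main GameUI, caches the player character and tracks interactable objects shown on screen.
; Adding an interactable gives it a unique "int_N" tag, reusing free numbers, and creates its UI widget; removal clears both and adjusts the highlight.
; Highlighting steps through the tag array with wraparound, finds actors by tag and toggles both actor and widget.
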(event EventBeginPlay
  (Utilities|FlowControl|Sequence
    (:then_0
      (bind _returnvalue (UserInterface|CreateWidget "/Game/UI/gameUI.gameUI_C" 0 self))
      (bind _output_get (Variables|Default|SetGameUI _returnvalue))
      (UserInterface|Viewport|AddtoViewport _output_get 0))
    (:then_1
      (bind _asbp_first_person_character (Utilities|Casting|CastToBP_FirstPersonCharacter (Game|GetPlayerCharacter 0)))
      (Variables|Default|SetplayerRef _asbp_first_person_character))))

(fn ConstructionScript)

(fn FInteractabletoUI
  (params (Interactable :type BP%20Interactible%20Parent%20Object%20Reference) (Add? :type Boolean))
  (bind _intactortags (Variables|Default|GetIntActorTags))
  (bind _intactortags_2 (Variables|Default|GetIntActorTags))
  (bind _f_interactable (LocalVariables|Getf_interactable))
  (bind _returnvalue (Utilities|Array|Length _intactortags))
  (bind _returnvalue_2 (Utilities|String|ToString(Integer) _returnvalue))
  (bind _returnvalue_3 (Utilities|String|Append "int_" _returnvalue_2))
  (bind _returnvalue_4 (Utilities|String|StringToName _returnvalue_3))
  (LocalVariables|SetF_interactable Interactable)
  (if Add?
    ;[1 1 1] Keep Track of Interactable & it's widget
    (Utilities|FlowControl|Sequence
      (:then_0
        (LocalVariables|SetF_gateOpen? true))
      (:then_1
        (bind _array_index (Utilities|Array|ForEachLoopwithBreak (Variables|Default|GetIntActorTags) :!label _label)
          (:LoopBody
            (if (not (Utilities|Array|ContainsItem (Variables|Default|GetIntActorTags) (Utilities|String|StringToName (Utilities|String|Append "int_" (Utilities|String|ToString(Integer) _array_index)))))
              (Variables|/Script/Engine.Actor|SetTags (LocalVariables|Getf_interactable) (Utilities|Array|MakeArray (Utilities|String|StringToName (Utilities|String|Append "int_" (Utilities|String|ToString(Integer) _array_index)))))
              (Utilities|Array|Add (Variables|Default|GetIntActorTags) (Utilities|String|StringToName (Utilities|String|Append "int_" (Utilities|String|ToString(Integer) _array_index))))
              (LocalVariables|SetF_gateOpen? false)
              (goto _label Break)))))
      (:then_2
        (if (LocalVariables|GetF_gateOpen?)
          (Variables|/Script/Engine.Actor|SetTags (LocalVariables|GetF_interactable) (Utilities|Array|MakeArray _returnvalue_4))
          (Utilities|Array|Add (Variables|Default|GetIntActorTags) _returnvalue_4)))
      (:then_3
        (bind _returnvalue_5 (UserInterface|CreateWidget "/Game/UI/WDG_InteractableObject.WDG_InteractableObject_C" 0 (LocalVariables|Getf_interactable)))
        (Variables|/Game/Actors/Interactables/ParentClass/BP_InteractibleParent.BP_InteractibleParent_C|SetWDG_Ref (LocalVariables|Getf_interactable) _returnvalue_5)
        (Default|AddInteractableChild (Variables|Default|GetGameUI) _returnvalue_5 true)))
    (else
      (bind (_array_element _array_index_2) (Utilities|Array|ForEachLoopwithBreak _intactortags_2 :!label _label_2)
        (:LoopBody
          (if (== _array_element (Utilities|Array|Get(acopy) (Variables|/Script/Engine.Actor|GetTags (LocalVariables|Getf_interactable))))
            (Utilities|FlowControl|Sequence
              (:then_0
                (if (Variables|/Game/Actors/Interactables/ParentClass/BP_InteractibleParent.BP_InteractibleParent_C|GethighlightActive _f_interactable)
                  (if (> (Utilities|Array|Length _intactortags_2) 1)
                    (CallFunction|FHighlightInt 0 "NewEnumerator2" "NewEnumerator1")
                    (else
                      (CallFunction|FHighlightInt _array_index_2 "NewEnumerator1" "NewEnumerator2" :!label _label_3)))
                  (else
                    (goto _label_3))))
              (:then_1
                (Utilities|Array|RemoveIndex _intactortags_2 _array_index_2)
                (Default|AddInteractableChild (Variables|Default|GetGameUI) (Variables|/Game/Actors/Interactables/ParentClass/BP_InteractibleParent.BP_InteractibleParent_C|GetWDG_Ref _f_interactable) false)
                (Utilities|Array|Clear (Variables|/Script/Engine.Actor|GetTags _f_interactable))
                (goto _label_2 Break)))))))))

(fn FHighlightInt
  (params (Array%20Ind :type Integer) (Highlight%20Target :type E_Progression%20Enum :default "NewEnumerator0") (Toggle%20Enum :type E_toggle%20Enum :default "NewEnumerator0"))
  (LocalVariables|SetF_ArrayInd Array%20Ind)
  (LocalVariables|SetF_toggleEnum Toggle%20Enum)
  (Utilities|FlowControl|Sequence
    (:then_0
      (switch Utilities|FlowControl|Switch|SwitchonE_Progression Highlight%20Target
        (:NewEnumerator0
          (LocalVariables|SetF_keyModifier -1)
          (LocalVariables|SetF_ArrayInd (Variables|Default|GethighlightedInt) :!label _label)
          (bind _outactors (Actor|GetAllActorsOfClasswithTag "/Game/Actors/Interactables/ParentClass/BP_InteractibleParent.BP_InteractibleParent_C" (Utilities|Array|Get(acopy) (Variables|Default|GetIntActorTags) (LocalVariables|GetF_ArrayInd))))
          (if (> (Utilities|Array|Length _outactors) 1)
            (Development|PrintString "Error ID01: Multiple Actors with same tag")
            (else
              (bind _array_element (Utilities|Array|ForEachLoopwithBreak _outactors)
                (:LoopBody
                  (Default|ToggleHighlight _array_element "NewEnumerator2")
                  (Default|ToggleHighlight (Variables|/Game/Actors/Interactables/ParentClass/BP_InteractibleParent.BP_InteractibleParent_C|GetWDG_Ref _array_element) "NewEnumerator2"))))))
        (:NewEnumerator1
          (LocalVariables|SetF_keyModifier 0))
        (:NewEnumerator2
          (LocalVariables|SetF_keyModifier 1)
          (goto _label))))
    (:then_2
      (if (>= (+ (LocalVariables|GetF_keyModifier) (LocalVariables|GetF_ArrayInd)) (Utilities|Array|Length (Variables|Default|GetIntActorTags)))
        (LocalVariables|SetF_ArrayInd 0)
        (elif (< (+ (LocalVariables|GetF_keyModifier) (LocalVariables|GetF_ArrayInd)) 0)
          (LocalVariables|SetF_ArrayInd (- (Utilities|Array|Length (Variables|Default|GetIntActorTags)) 1))
          (else
            (LocalVariables|SetF_ArrayInd (+ (LocalVariables|GetF_keyModifier) (LocalVariables|GetF_ArrayInd)))))))
    (:then_3
      (bind _outactors_2 (Actor|GetAllActorsOfClasswithTag "/Game/Actors/Interactables/ParentClass/BP_InteractibleParent.BP_InteractibleParent_C" (Utilities|Array|Get(acopy) (Variables|Default|GetIntActorTags) (LocalVariables|GetF_ArrayInd))))
      (if (> (Utilities|Array|Length _outactors_2) 1)
        (Development|PrintString "Error ID02: Multiple Actors with same tag")
        (else
          (bind _array_element_2 (Utilities|Array|ForEachLoopwithBreak _outactors_2)
            (:LoopBody
              (if (Variables|/Game/Actors/Interactables/ParentClass/BP_InteractibleParent.BP_InteractibleParent_C|GetisInteractable _array_element_2)
                (Default|ToggleHighlight _array_element_2 (LocalVariables|GetF_toggleEnum))
                (Default|ToggleHighlight (Variables|/Game/Actors/Interactables/ParentClass/BP_InteractibleParent.BP_InteractibleParent_C|GetWDG_Ref _array_element_2) (LocalVariables|GetF_toggleEnum))))))))
    (:then_4
      (Variables|Default|SethighlightedInt (LocalVariables|GetF_ArrayInd)))))