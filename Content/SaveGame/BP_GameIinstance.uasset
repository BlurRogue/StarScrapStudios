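; Game instance that owns the game's save data, keeping one BP_SaveGame object in memory and persisting it to a save slot.
; On Init it synchronously loads the slot, or creates a fresh save object if none exists.
; Saving and loading each support sync or async modes, but only a completed async load fires OnGameLoaded.
; SavePlayer writes player data into the cached object and saves it, while GetGameData exposes that object.
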(event EventInit
  (CallFunction|LoadGameData false))

(event EventSaveGameData
  (params (Async :type Boolean))
  (bind _saveddata (Variables|Default|GetSavedData))
  (bind _slotname (Variables|Default|GetSlotName))
  ;[1 1 1] Save Game
  (if Async
    (|AsyncSaveGametoSlot _saveddata _slotname)
    (else
      (SaveGame|SaveGametoSlot _saveddata _slotname))))

(event EventLoadGameData
  (params (Async :type Boolean))
  (bind _slotname (Variables|Default|GetSlotName))
  ;[1 1 1] Load Game
  (bind _returnvalue (SaveGame|DoesSaveGameExist (Variables|Default|GetSlotName)))
  (if _returnvalue
    (if Async
      (bind _savegame (|AsyncLoadGamefromSlot _slotname)
        (:Completed
          (bind _asbp_save (Utilities|Casting|CastToBP_SaveGame _savegame))
          (Variables|Default|SetSavedData _asbp_save)
          (Default|CallOnGameLoaded)))
      (else
        (bind _returnvalue_2 (SaveGame|LoadGamefromSlot _slotname))
        (bind _asbp_save_2 (Utilities|Casting|CastToBP_SaveGame _returnvalue_2))
        (Variables|Default|SetSavedData _asbp_save_2)))
    (else
      (bind _returnvalue_3 (SaveGame|CreateSaveGameObject "/Game/SaveGame/BP_SaveGame.BP_SaveGame_C"))
      (Variables|Default|SetSavedData _returnvalue_3))))

(event EventSavePlayer
  (params (PlayerSave :type S%20Player%20Save%20Structure) (Async :type Boolean))
  (Variables|/Game/SaveGame/BP_SaveGame.BP_SaveGame_C|SetPlayerSave (Variables|Default|GetSavedData) PlayerSave)
  (CallFunction|SaveGameData Async))

(fn GetGameData
  (return (Variables|Default|GetSavedData)))