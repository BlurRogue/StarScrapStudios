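; Spaceship Blueprint whose Interact event plays a door sound at world origin and toggles two sliding doors.
; Separate FlipFlops drive each door's timelines, which only act as tickers, nudging relative X one unit per update, so travel depends on update count.
; The left door reverses one timeline and takes direction from IsOpen, flipped on finish.
; The right door uses a separate timeline for each direction.
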(event Custom|ShiftLeftDoor
  (bind _leftdoor (Variables|Default|GetLeftDoor))
  (bind _relativelocation (Variables|/Script/Engine.SceneComponent|GetRelativeLocation _leftdoor))
  (Utilities|FlowControl|FlipFlop
    (:A
      (Timeline|Timeline PlayFromStart
        (:Update
          (if (Variables|Default|GetIsOpen)
            (Transformation|SetRelativeLocation _leftdoor (Math|Vector|MakeVector (- (.x _relativelocation) -1.0) 0.0 0.0) false false)
            (else
              (Transformation|SetRelativeLocation _leftdoor (Math|Vector|MakeVector (- (.x _relativelocation) 1.0) 0.0 0.0) false false))))
        (:Finished
          (if (Variables|Default|GetIsOpen)
            (Variables|Default|SetIsOpen false)
            (else
              (Variables|Default|SetIsOpen true))))))
    (:B
      (Timeline|Timeline ReverseFromEnd))))

(event Custom|ShiftRightDoor
  (bind _rightdoor (Variables|Default|GetRightDoor))
  (bind _rightdoor_2 (Variables|Default|GetRightDoor))
  (Utilities|FlowControl|FlipFlop
    (:A
      (Timeline|Timeline_1 Play
        (:Update
          (Transformation|SetRelativeLocation _rightdoor_2 (Math|Vector|MakeVector (+ (.x (Variables|/Script/Engine.SceneComponent|GetRelativeLocation _rightdoor_2)) 1.0) 0.0 0.0) false false))))
    (:B
      (Timeline|Timeline_2 Play
        (:Update
          (Transformation|SetRelativeLocation _rightdoor (Math|Vector|MakeVector (- (.x (Variables|/Script/Engine.SceneComponent|GetRelativeLocation _rightdoor)) 1.0) 0.0 0.0) false false))))))

(event EventBeginPlay)

(event Collision|EventActorBeginOverlap
  (params (OtherActor :type Actor%20Object%20Reference)))

(event EventTick
  (params (DeltaSeconds :type Float%20%28single-precision%29)))

(event EventInteract
  (Audio|PlaySoundatLocation "/Game/Assets/Audio/Interaction/Door_Open.Door_Open" "0, 0, 0" "0, 0, 0" 1.0 1.0 0.0 0 0 0 0)
  (CallFunction|ShiftLeftDoor)
  (CallFunction|ShiftRightDoor))

(fn ConstructionScript)