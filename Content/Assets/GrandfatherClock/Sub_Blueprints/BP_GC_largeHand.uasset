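; Interactable large hand of a grandfather clock puzzle, stepped around the dial by the player.
; Interact plays a tick sound and eases the mesh through a -30 degree roll step via MoveComponentTo.
; It then advances RotationPosition, which wraps to 0 only after 12, giving 13 states per cycle.
; Each step reports the position to the parent's CheckSolution, passing 13 as the small-hand value.
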(event Custom|Rotate
  (bind _static_mesh (Variables|Default|GetStatic_Mesh))
  (Audio|PlaySoundatLocation "/Game/Assets/Audio/Interaction/Clock/Clock_Ticking_Once.Clock_Ticking_Once" (Transformation|GetWorldLocation (Variables|Default|GetStatic_Mesh)) "0, 0, 0" 1.0 1.0 0.0 0 0 0 0)
  (Components|MoveComponentTo (Variables|Default|GetStatic_Mesh) (Variables|/Script/Engine.SceneComponent|GetRelativeLocation _static_mesh) (Math|Rotator|MakeRotator (.roll (Math|Rotator|MakeRotator (+ (.roll (Transformation|GetWorldRotation _static_mesh)) -3e+01) 0.0 0.0)) 0.0 0.0) true true 0.2 false)
  (Utilities|FlowControl|Delay 0.2))

(event Custom|Update%20Rotation%20Position
  (bind _parent (Variables|Default|GetParent))
  (if (> (+ (Variables|Default|GetRotation_Position) 1) 12)
    (bind _output_get (Variables|Default|SetRotation_Position 0))
    (Default|CheckSolution _parent 13 _output_get)
    (else
      (bind _output_get_2 (Variables|Default|SetRotation_Position (Math|Integer|Clamp(Integer) (+ (Variables|Default|GetRotation_Position) 1) 0 12)))
      (Default|CheckSolution _parent 13 _output_get_2))))

(event EventBeginPlay)

(event Collision|EventActorBeginOverlap
  (params (OtherActor :type Actor%20Object%20Reference)))

(event EventTick
  (params (DeltaSeconds :type Float%20%28single-precision%29)))

(event EventInteract
  (CallFunction|Rotate)
  (CallFunction|UpdateRotationPosition))

(fn ConstructionScript)