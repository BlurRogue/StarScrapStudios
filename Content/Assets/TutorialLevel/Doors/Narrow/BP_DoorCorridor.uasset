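; Narrow corridor double sliding door that toggles open and closed through its Interact event.
; Interact plays a sound at world origin, then drives each leaf through its own FlipFlop, alternately playing and reversing a timeline.
; Timeline updates add scaled, opposite-signed local Y offsets cumulatively to the leaves, rather than setting absolute positions.
; A trigger overlap shows a message widget while the first-person character is nearby.
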(event OnComponentBeginOverlap(WigitTrigger)
  (params (OverlappedComponent :type Primitive%20Component%20Object%20Reference) (OtherActor :type Actor%20Object%20Reference) (OtherComp :type Primitive%20Component%20Object%20Reference) (OtherBodyIndex :type Integer) (bFromSweep :type Boolean) (SweepResult :type Hit%20Result%20Structure%20%28by%20ref%29))
  (Utilities|Casting|CastToBP_FirstPersonCharacter OtherActor)
  (Rendering|SetVisibility (Variables|Default|Getmessagewiget) true false))

(event OnComponentEndOverlap(WigitTrigger)
  (params (OverlappedComponent :type Primitive%20Component%20Object%20Reference) (OtherActor :type Actor%20Object%20Reference) (OtherComp :type Primitive%20Component%20Object%20Reference) (OtherBodyIndex :type Integer))
  (Utilities|Casting|CastToBP_FirstPersonCharacter OtherActor)
  (Rendering|SetVisibility (Variables|Default|Getmessagewiget) false false))

(event Custom|OpenLeftDoor
  (Utilities|FlowControl|FlipFlop
    (:A
      (bind _leftdoor (Timeline|Timeline Play)
        (:Update
          (Transformation|AddLocalOffset (Variables|Default|GetLeftDoor) (Math|Vector|MakeVector 0.0 (+ 0.0 (* (* _leftdoor -1.0) 0.6)) 0.0) false false))
        (:Finished)))
    (:B
      (Timeline|Timeline Reverse))))

(event Custom|OpenDoors
  (Audio|PlaySoundatLocation "/Game/Sound/SoundWaves/Door_Open.Door_Open" "0, 0, 0" "0, 0, 0" 1.0 1.0 0.0 0 0 0 0)
  (CallFunction|OpenLeftDoor)
  (CallFunction|OpenRightDoor))

(event Custom|OpenRightDoor
  (Utilities|FlowControl|FlipFlop
    (:A
      (bind _leftdoor (Timeline|Timeline_0 Play)
        (:Update
          (Transformation|AddLocalOffset (Variables|Default|GetRightDoor) (Math|Vector|MakeVector 0.0 (+ 0.0 (* (* _leftdoor 1.0) 0.6)) 0.0) false false))))
    (:B
      (Timeline|Timeline_0 Reverse))))

(event EventInteract
  (CallFunction|OpenDoors))

(fn ConstructionScript)

(fn FOpenLeftDoor)

(fn FOpenRightDoor)