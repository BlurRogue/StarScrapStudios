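; BP_Light is a configurable light fixture actor that combines a spot light and a rect light.
; Its construction script copies per-instance variables onto both components, covering visibility, color temperature, intensity, attenuation, shape and indirect lighting, plus volumetric scattering.
; Each light has its own set of variables and visibility toggle.
; A single scale value drives both the rect light's source width and height, keeping it square.
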(fn ConstructionScript
  (bind _rl_sourcescale (Variables|RectLight|GetRL_sourceScale))
  (bind _rectlight (Variables|Default|GetRectLight))
  (bind _spotlight (Variables|Default|GetSpotLight))
  (bind _rectlight_2 (Variables|Default|GetRectLight))
  (bind _rectlight_3 (Variables|Default|GetRectLight))
  (Rendering|SetVisibility _spotlight (Variables|Spot_Light|GetSL_isVis) false)
  (Class|LightComponent|SetTemperature _spotlight (Variables|Spot_Light|GetSL_temp))
  (Rendering|Components|Light|SetIntensity _spotlight (Variables|Spot_Light|GetSL_intensity))
  (Rendering|Lighting|SetAttenuationRadius (Variables|Default|GetSpotLight) (Variables|Spot_Light|GetSL_attenRadius))
  (Rendering|Lighting|SetInnerConeAngle (Variables|Default|GetSpotLight) (Variables|Spot_Light|GetSL_innConAng))
  (Rendering|Lighting|SetOuterConeAngle (Variables|Default|GetSpotLight) (Variables|Spot_Light|GetSL_outConAng))
  (Class|LightComponent|SetIndirectLightingIntensity (Variables|Default|GetSpotLight) (Variables|Spot_Light|GetSL_indLightInt))
  (Class|LightComponent|SetVolumetricScatteringIntensity (Variables|Default|GetSpotLight) (Variables|Spot_Light|GetSL_volScaInt))
  (Class|PointLightComponent|SetLightFalloffExponent (Variables|Default|GetSpotLight) (Variables|Spot_Light|GetSL_lighFallExpo))
  (Class|PointLightComponent|SetSourceRadius (Variables|Default|GetSpotLight) (Variables|Spot_Light|GetSL_souRad))
  (Class|PointLightComponent|SetSoftSourceRadius (Variables|Default|GetSpotLight) (Variables|Spot_Light|GetSL_sofSouRad))
  (Class|PointLightComponent|SetSourceLength (Variables|Default|GetSpotLight) (Variables|Spot_Light|GetSL_souLen))
  (Rendering|SetVisibility _rectlight_3 (Variables|RectLight|GetRL_isVis) false)
  (Class|LightComponent|SetTemperature _rectlight_3 (Variables|RectLight|GetRL_temp))
  (Rendering|Components|Light|SetIntensity (Variables|Default|GetRectLight) (Variables|RectLight|GetRL_intensity))
  (Class|LightComponent|SetVolumetricScatteringIntensity (Variables|Default|GetRectLight) (Variables|RectLight|GetRL_volScaInt))
  (Class|RectLightComponent|SetSourceHeight _rectlight_2 _rl_sourcescale)
  (Class|RectLightComponent|SetSourceWidth _rectlight_2 _rl_sourcescale)
  (Rendering|Lighting|SetAttenuationRadius _rectlight (Variables|RectLight|GetRL_attenRadius))
  (Class|RectLightComponent|SetBarnDoorAngle _rectlight (Variables|RectLight|GetRL_barnDoorAng))
  (Class|RectLightComponent|SetBarnDoorLength _rectlight (Variables|RectLight|GetRL_barnDoorLen))
  (Class|LightComponent|SetIndirectLightingIntensity _rectlight (Variables|RectLight|GetRL_indLightInt)))